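; Base gun pickup for the 2D platformer that the player attaches and fires.
; Overlapping its trigger attaches the sprite to the player's Gun socket, enables input on the gun for player 0 and switches the player's animation state.
; The Shoot input spawns a Bullet_Master at the Bullet component's transform, passing damage and despawn delay, unless the player is dead.
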(event OnComponentBeginOverlap(Trigger)
  (params (OverlappedComponent :type Primitive%20Component%20Object%20Reference) (OtherActor :type Actor%20Object%20Reference) (OtherComp :type Primitive%20Component%20Object%20Reference) (OtherBodyIndex :type Integer) (bFromSweep :type Boolean) (SweepResult :type Hit%20Result%20Structure%20%28by%20ref%29))
  ;[1 1 1] Attaching gun to player/Enable Input
  (bind _asplayer_character (Utilities|Casting|CastToPlayer_Character OtherActor))
  (bind _output_get (Variables|Default|SetPlayer _asplayer_character))
  (Default|AttachItem _output_get (Variables|Default|GetPaperSprite) (Variables|Default|GetGun))
  (Input|EnableInput (Game|GetPlayerController 0))
  (bind _output_get_2 (Variables|Default|Sethas%20gun true))
  (if _output_get_2
    (Variables|/Game/2DPlatformingKit/Blueprints/Player/Player_Character.Player_Character_C|SetplayerAnimState (Variables|Default|GetPlayer) "NewEnumerator31")))

(event Input|ActionEvents|InputActionShoot
  (params (Key :type Key%20Structure))
  ;[1 1 1] Shoot when left mouse is clicked if dead does not fire
  (:Pressed
    (if (not (Variables|/Game/2DPlatformingKit/Blueprints/Player/Player_Character.Player_Character_C|GetIs%20Dead (stale OnComponentBeginOverlap(Trigger) _asplayer_character)))
      (Game|SpawnActorfromClass "/Game/2DPlatformingKit/Blueprints/Player/Bullet_Master.Bullet_Master_C" (Transformation|GetWorldTransform (Variables|Default|GetBullet)) "Undefined" 0 (Variables|Default|GetDamage) (Variables|Default|GetBullet%20Despawn) 0))))

(fn ConstructionScript)