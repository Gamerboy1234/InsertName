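; Cyborg_Bullet is a projectile Blueprint, filed with the player assets of the 2D platforming kit, for a bullet moved by a ProjectileMovement component.
; On BeginPlay it runs the parent logic, then copies its StartingSpeed, MaxSpeed and Gravity variables into that component's initial speed, max speed and gravity scale.
; Tick and the construction script only call their parent versions.
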(event EventBeginPlay
  (bind _projectilemovement (Variables|Default|GetProjectileMovement))
  (|CallParentFunction)
  (Variables|/Script/Engine.ProjectileMovementComponent|SetInitialSpeed _projectilemovement (Variables|Default|GetStarting%20Speed))
  (Variables|/Script/Engine.ProjectileMovementComponent|SetMaxSpeed _projectilemovement (Variables|Default|GetMax%20Speed))
  (Variables|/Script/Engine.ProjectileMovementComponent|SetProjectileGravityScale _projectilemovement (Variables|Default|GetGravity)))

(event EventTick
  (params (DeltaSeconds :type Float%20%28single-precision%29))
  (|CallParentFunction DeltaSeconds))

(fn ConstructionScript
  (|CallParentFunction))