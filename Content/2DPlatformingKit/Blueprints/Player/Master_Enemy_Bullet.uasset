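; Base enemy projectile for the 2D platforming kit that damages the player on contact.
; A sphere overlap with Player_Character calls its Damage function with current HP minus the bullet's damage plus the damage value for text, then destroys the bullet.
; Overlaps with other actors are ignored.
; On BeginPlay it stores the ProjectileMovement velocity as DefaultVelocity, which is not used elsewhere in this graph.
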(event OnComponentBeginOverlap(Sphere)
  (params (OverlappedComponent :type Primitive%20Component%20Object%20Reference) (OtherActor :type Actor%20Object%20Reference) (OtherComp :type Primitive%20Component%20Object%20Reference) (OtherBodyIndex :type Integer) (bFromSweep :type Boolean) (SweepResult :type Hit%20Result%20Structure%20%28by%20ref%29))
  (bind _asplayer_character (Utilities|Casting|CastToPlayer_Character OtherActor))
  (Default|Damage _asplayer_character (- (Variables|/Game/2DPlatformingKit/Blueprints/Player/Player_Character.Player_Character_C|GetPlayer%20HP _asplayer_character) (Variables|Default|GetDamage)) (Variables|Default|GetDamage))
  (Actor|DestroyActor))

(event EventBeginPlay
  (Variables|Default|SetDefault%20Velocity (Variables|/Script/Engine.MovementComponent|GetVelocity (Variables|Default|GetProjectileMovement))))

(fn ConstructionScript)