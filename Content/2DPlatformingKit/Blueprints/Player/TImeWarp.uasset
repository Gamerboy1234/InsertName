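; Time warp projectile for a 2D platformer that creates a growing field slowing enemies and bullets.
; A timeline enlarges its sphere trigger, and the actor destroys itself after a delay once growth finishes.
; Overlaps use a cast chain to alter each type's movement, restoring defaults on exit for some types.
; Tick raises damage, after a delay, on the last enemy and player bullet stored while inside.
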(event OnComponentEndOverlap(TimeTrigger)
  (params (OverlappedComponent :type Primitive%20Component%20Object%20Reference) (OtherActor :type Actor%20Object%20Reference) (OtherComp :type Primitive%20Component%20Object%20Reference) (OtherBodyIndex :type Integer))
  ;[1 1 1] Collsion list
  (bind _asmaster_enemy_bp (Utilities|Casting|CastToMaster_Enemy_BP OtherActor)
    (:then
      (Components|Timeline|SetPlayRate (Variables|/Game/2DPlatformingKit/Blueprints/BP_Enemies/TOBEDELETED/Master_Enemy_BP.Master_Enemy_BP_C|GetPaperFlipbook _asmaster_enemy_bp) 1.0)
      (Variables|/Script/Engine.InterpToMovementComponent|SetDuration (Variables|/Game/2DPlatformingKit/Blueprints/BP_Enemies/TOBEDELETED/Master_Enemy_BP.Master_Enemy_BP_C|GetInterpToMovement _asmaster_enemy_bp) (Variables|/Game/2DPlatformingKit/Blueprints/BP_Enemies/TOBEDELETED/Master_Enemy_BP.Master_Enemy_BP_C|GetDefault%20Duration _asmaster_enemy_bp)))
    (:CastFailed
      (bind _asmaster_enemy_bullet (Utilities|Casting|CastToMaster_Enemy_Bullet OtherActor)
        (:then
          (Variables|/Script/Engine.MovementComponent|SetVelocity (Variables|/Game/2DPlatformingKit/Blueprints/Player/Master_Enemy_Bullet.Master_Enemy_Bullet_C|GetProjectileMovement _asmaster_enemy_bullet) (Variables|/Game/2DPlatformingKit/Blueprints/Player/Master_Enemy_Bullet.Master_Enemy_Bullet_C|GetDefault%20Velocity _asmaster_enemy_bullet))
          (Variables|TimeSlow|SetIs%20Master%20Enemy%20Bullet%20in?%20 false))
        (:CastFailed
          (bind _ascorrupted_bp (Utilities|Casting|CastTo OtherActor)
            (:then
              (Variables|/Script/InsertNameV2.TheCorrupted|Setvelocity _ascorrupted_bp (Variables|Default|GetDefault%20Vecity _ascorrupted_bp)))
            (:CastFailed
              (bind _asbullet_master (Utilities|Casting|CastToBullet_Master OtherActor))
              (Variables|/Script/Engine.MovementComponent|SetVelocity (Variables|/Game/2DPlatformingKit/Blueprints/Player/Bullet_Master.Bullet_Master_C|GetProjectileMovement _asbullet_master) (Variables|/Game/2DPlatformingKit/Blueprints/Player/Bullet_Master.Bullet_Master_C|GetDefault%20Velocity _asbullet_master))
              (Variables|TimeSlow|SetIs%20Player%20Bullet%20in? false))))))))

(event OnComponentBeginOverlap(TimeTrigger)
  (params (OverlappedComponent :type Primitive%20Component%20Object%20Reference) (OtherActor :type Actor%20Object%20Reference) (OtherComp :type Primitive%20Component%20Object%20Reference) (OtherBodyIndex :type Integer) (bFromSweep :type Boolean) (SweepResult :type Hit%20Result%20Structure%20%28by%20ref%29))
  ;[1 1 1] Collsion list
  (bind _asmaster_enemy_bp (Utilities|Casting|CastToMaster_Enemy_BP OtherActor)
    (:then
      (Components|Timeline|SetPlayRate (Variables|/Game/2DPlatformingKit/Blueprints/BP_Enemies/TOBEDELETED/Master_Enemy_BP.Master_Enemy_BP_C|GetPaperFlipbook _asmaster_enemy_bp) (Variables|TimeSlow|GetSprite%20Play%20Rate))
      (Variables|/Script/Engine.InterpToMovementComponent|SetDuration (Variables|/Game/2DPlatformingKit/Blueprints/BP_Enemies/TOBEDELETED/Master_Enemy_BP.Master_Enemy_BP_C|GetInterpToMovement _asmaster_enemy_bp) (/ (Variables|/Script/Engine.InterpToMovementComponent|GetDuration (Variables|/Game/2DPlatformingKit/Blueprints/BP_Enemies/TOBEDELETED/Master_Enemy_BP.Master_Enemy_BP_C|GetInterpToMovement _asmaster_enemy_bp)) (Variables|TimeSlow|GetSpeed%20to%20Divde))))
    (:CastFailed
      (bind _asmaster_enemy_bullet (Utilities|Casting|CastToMaster_Enemy_Bullet OtherActor)
        (:then
          (Variables|Refs|SetMaster%20Enemy%20Bullet _asmaster_enemy_bullet)
          (Variables|/Script/Engine.MovementComponent|SetVelocity (Variables|/Game/2DPlatformingKit/Blueprints/Player/Master_Enemy_Bullet.Master_Enemy_Bullet_C|GetProjectileMovement _asmaster_enemy_bullet) (/ (Variables|/Script/Engine.MovementComponent|GetVelocity (Variables|/Game/2DPlatformingKit/Blueprints/Player/Master_Enemy_Bullet.Master_Enemy_Bullet_C|GetProjectileMovement _asmaster_enemy_bullet)) (Variables|TimeSlow|GetHalf%20Bullet%20Velocity)))
          (Variables|TimeSlow|SetIs%20Master%20Enemy%20Bullet%20in?%20 true))
        (:CastFailed
          (bind _asthe_corrupted (Utilities|Casting|CastToTheCorrupted OtherActor)
            (:then
              (Variables|/Script/InsertNameV2.TheCorrupted|Setvelocity _asthe_corrupted (/ (Variables|/Script/InsertNameV2.TheCorrupted|Getvelocity _asthe_corrupted) (Variables|TimeSlow|GetSpeed%20to%20Divde))))
            (:CastFailed
              (bind _asjn_ranged_bp (Utilities|Casting|CastToJN_Ranged_BP OtherActor)
                (:then
                  (Variables|/Script/InsertNameV2.JN_Ranged|Setvelocity1 _asjn_ranged_bp (- (Variables|/Script/InsertNameV2.JN_Ranged|Getvelocity1 _asjn_ranged_bp) (Variables|TimeSlow|GetSpeed%20to%20Divde))))
                (:CastFailed
                  (bind _asbullet_master (Utilities|Casting|CastToBullet_Master OtherActor))
                  (Variables|Refs|SetBullet%20Master _asbullet_master)
                  (Variables|/Script/Engine.MovementComponent|SetVelocity (Variables|/Game/2DPlatformingKit/Blueprints/Player/Bullet_Master.Bullet_Master_C|GetProjectileMovement _asbullet_master) (/ (Variables|/Script/Engine.MovementComponent|GetVelocity (Variables|/Game/2DPlatformingKit/Blueprints/Player/Bullet_Master.Bullet_Master_C|GetProjectileMovement _asbullet_master)) (Variables|TimeSlow|GetHalf%20Bullet%20Velocity)))
                  (Variables|TimeSlow|SetIs%20Player%20Bullet%20in? true))))))))))

(event EventTick
  (params (DeltaSeconds :type Float%20%28single-precision%29))
  (Utilities|FlowControl|Sequence
    (:then_0
      ;[1 1 1] Despawn
      (if (Variables|Misc|GetTime%20Line%20Done?)
        (Utilities|FlowControl|Delay (Variables|Misc|GetDespawn%20Delay))
        (Actor|DestroyActor)))
    (:then_1
      (if (Variables|TimeSlow|GetIs%20Master%20Enemy%20Bullet%20in?%20)
        ;[1 1 1] Increasse Damage of master enemy bullet
        (Utilities|IsValid (Variables|Refs|GetMaster%20Enemy%20Bullet)
          (:Is%20Valid
            (Utilities|FlowControl|Delay (Variables|TimeSlow|GetDamage%20Increase%20Delay))
            (Variables|/Game/2DPlatformingKit/Blueprints/Player/Master_Enemy_Bullet.Master_Enemy_Bullet_C|SetDamage (Variables|Refs|GetMaster%20Enemy%20Bullet) (+ (Variables|/Game/2DPlatformingKit/Blueprints/Player/Master_Enemy_Bullet.Master_Enemy_Bullet_C|GetDamage (Variables|Refs|GetMaster%20Enemy%20Bullet)) (Variables|TimeSlow|GetDamage%20Increase))))
          (:Is%20Not%20Valid
            (Variables|TimeSlow|SetIs%20Master%20Enemy%20Bullet%20in?%20 false)))))
    (:then_2
      (if (Variables|TimeSlow|GetIs%20Player%20Bullet%20in?)
        ;[1 1 1] Increasse Damage of player bullet
        (Utilities|IsValid (Variables|Refs|GetBullet%20Master)
          (:Is%20Valid
            (Utilities|FlowControl|Delay (Variables|TimeSlow|GetDamage%20Increase%20Delay))
            (Variables|/Game/2DPlatformingKit/Blueprints/Player/Bullet_Master.Bullet_Master_C|SetDamge (Variables|Refs|GetBullet%20Master) (+ (Variables|/Game/2DPlatformingKit/Blueprints/Player/Bullet_Master.Bullet_Master_C|GetDamge (Variables|Refs|GetBullet%20Master)) (Variables|TimeSlow|GetDamage%20Increase))))
          (:Is%20Not%20Valid
            (Variables|TimeSlow|SetIs%20Player%20Bullet%20in? false)))))))

(event EventBeginPlay
  (bind _projectilemovement (Variables|Default|GetProjectileMovement))
  ;[1 1 1] Set Timeline vars
  (Components|Timeline|SetTimelineLength (Variables|Default|GetGrow%20TimeLine) (Variables|SphereGrowth|GetGrowth%20Time))
  (Variables|Misc|SetTime%20Line%20Done? false)
  ;[1 1 1] Get Player Ref
  (bind _asplayer_character (Utilities|Casting|CastToPlayer_Character (Game|GetPlayerCharacter 0)))
  (Variables|Misc|SetPlayer%20Ref _asplayer_character)
  ;[1 1 1] Starting Radius
  (Components|Sphere|SetSphereRadius (Variables|Default|GetTimeTrigger) (Variables|SphereGrowth|GetStarting%20Radius) true)
  ;[1 1 1] Setting Speed and gravity
  (Variables|/Script/Engine.ProjectileMovementComponent|SetInitialSpeed _projectilemovement (Variables|Misc|GetStarting%20Speed))
  (Variables|/Script/Engine.ProjectileMovementComponent|SetMaxSpeed _projectilemovement (Variables|Misc|GetMax%20Speed))
  (Variables|/Script/Engine.ProjectileMovementComponent|SetProjectileGravityScale _projectilemovement (Variables|Misc|GetGravity))
  ;[1 1 1] Grow Trigger Over Time
  (bind _float_track (Timeline|Grow%20TimeLine PlayFromStart)
    (:Update
      (Components|Sphere|SetSphereRadius (Variables|Default|GetTimeTrigger) (+ (Variables|/Script/Engine.SphereComponent|GetSphereRadius (Variables|Default|GetTimeTrigger)) _float_track) true))
    (:Finished
      (Variables|Misc|SetTime%20Line%20Done? true))))

(fn ConstructionScript)