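; JetFireBall is a player-related fire projectile from the 2D platforming kit that burns enemies and ignites magnet platforms.
; On spawn it caches the player and sets a despawn lifespan.
; Trigger overlap applies a ticking fire damage debuff to enemies not already burning, or switches a MagnetPlatform to its fire texture and destroys itself.
; A ClearFire function destroys every JetFireBall in the level.
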(event OnComponentBeginOverlap(Trigger)
  (params (OverlappedComponent :type Primitive%20Component%20Object%20Reference) (OtherActor :type Actor%20Object%20Reference) (OtherComp :type Primitive%20Component%20Object%20Reference) (OtherBodyIndex :type Integer) (bFromSweep :type Boolean) (SweepResult :type Hit%20Result%20Structure%20%28by%20ref%29))
  ;[1 1 1] Damage Code
  (bind _asmaster_enemy_ai_bp (Utilities|Casting|CastToMaster_Enemy_AI_BP OtherActor)
    (:then
      (if (not (Default|GetIsonFire? _asmaster_enemy_ai_bp))
        (Variables|Default|SetMaster%20Enemy%20AI _asmaster_enemy_ai_bp)
        (Default|ApplyDebuff (Variables|Default|GetMaster%20Enemy%20AI) (Variables|Default|GetDamage%20Over%20Time) (Variables|Default|GetOccurrences) (Variables|Default|GetDamage%20Ticks%20) "5.000000,5.000000,5.000000" true "/Game/2DPlatformingKit/Blueprints/BP_Enemies/General/Debuffs/Debuffs/Fire_Damage_E.Fire_Damage_E_C" _asmaster_enemy_ai_bp)))
    (:CastFailed
      (bind _asmagnet_platform (Utilities|Casting|CastToMagnetPlatform OtherActor))
      (Default|UpdateTexturetoFire _asmagnet_platform)
      (Actor|DestroyActor))))

(event EventBeginPlay
  ;[1 1 1] Get Player Ref
  (Variables|Default|SetPlayer%20Ref (CallFunction|GetPlayer self))
  ;[1 1 1] Set Life span of fire
  (Actor|SetLifeSpan (Variables|Default|GetDespawn%20Delay)))

(fn ConstructionScript)

(fn ClearFire
  (bind _outactors (Actor|GetAllActorsOfClass "JetFireBall_C"))
  (for _array_element _outactors
    (Actor|DestroyActor _array_element)))