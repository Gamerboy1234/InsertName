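; Camera manager for a 2D platformer that tracks a camera target and the active camera zone.
; Camera triggers pass a name, which is trimmed of its first character and any hyphen suffix, then matched to a zone actor's name.
; On start or zone change, the zone's actor bounds become Min and Max limits in X and Z, keeping the camera's Y.
; Camera movement itself is absent from these graphs.
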(event EventSetCameraTarget
  (params (New%20Target :type Actor%20Object%20Reference))
  (Variables|Actor's|SetCamera%20Target New%20Target))

(event EventOnCameraTrigger
  (params (Name :type String))
  (CallFunction|GetCameraZone Name)
  (if (Variables|Actor's|GetDo%20Update)
    (CallFunction|SetCameraZoneMinandMax (Variables|Actor's|GetCurrent%20Index))))

(event EventBeginPlay
  (Variables|Actor's|SetCurrent%20Index 0)
  (CallFunction|SetCameraZoneMinandMax (Variables|Actor's|GetCurrent%20Index)))

(fn ConstructionScript)

(fn SetCameraZoneMinandMax
  (params (Index :type Integer))
  (bind _camera_zones (Variables|Actor's|GetCamera%20Zones))
  (bind _cameracomponent (Variables|CameraActor|GetCameraComponent))
  (bind _returnvalue (Transformation|GetWorldLocation _cameracomponent))
  (bind _output (Utilities|Array|Get(acopy) _camera_zones Index))
  (bind _y (Math|Vector|BreakVector _returnvalue))
  (bind (_origin _boxextent) (Collision|GetActorBounds _output false))
  ;[1 1 1] Get Bounds: Location (origin) && Half Length (Box Extent)
  (Variables|Default|SetLocation _origin)
  (Variables|Default|SetCoordinates _boxextent)
  ;[1 1 1] Left and Bottom Coordinates
  (Variables|Coordinates|SetMin (Math|Vector|MakeVector (- (.X (Math|Vector|BreakVector (Variables|Default|GetLocation))) (.X (Math|Vector|BreakVector (Variables|Default|GetCoordinates)))) _y (- (.Z (Math|Vector|BreakVector (Variables|Default|GetLocation))) (.Z (Math|Vector|BreakVector (Variables|Default|GetCoordinates))))))
  ;[1 1 1] Right and Top Coordinates
  (Variables|Coordinates|SetMax (Math|Vector|MakeVector (+ (.X (Math|Vector|BreakVector (Variables|Default|GetLocation))) (.X (Math|Vector|BreakVector (Variables|Default|GetCoordinates)))) _y (+ (.Z (Math|Vector|BreakVector (Variables|Default|GetLocation))) (.Z (Math|Vector|BreakVector (Variables|Default|GetCoordinates))))))
  (return))

(fn GetCameraZone
  (params (Name :type String))
  (bind _returnvalue (Utilities|String|Len Name))
  (bind _returnvalue_2 (- _returnvalue 1))
  (bind _returnvalue_3 (Utilities|String|GetSubstring Name 1 _returnvalue_2))
  (bind (_lefts _rights _returnvalue_4) (Utilities|String|Split _returnvalue_3 "-"))
  (if _returnvalue_4
    (Variables|Actor's|SetCamera%20Zone%20Name _lefts)
    (else
      (Variables|Actor's|SetCamera%20Zone%20Name _returnvalue_3)))
  (bind (_array_element _array_index) (Utilities|Array|ForEachLoopwithBreak (Variables|Actor's|GetCamera%20Zones) :!label _label)
    (:LoopBody
      (if (Utilities|Enum|Equal(Enum) (Utilities|String|ToString(Object) _array_element) (Variables|Actor's|GetCamera%20Zone%20Name))
        (if (!= _array_index (Variables|Actor's|GetCurrent%20Index))
          (Variables|Actor's|SetCurrent%20Index _array_index)
          (Variables|Actor's|SetDo%20Update true)
          (goto _label Break)
          (else
            (Variables|Actor's|SetDo%20Update false)
            (goto _label Break)))))))