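; Base player projectile for the 2D platforming kit that damages enemies on overlap and despawns after a set delay.
; The construction script applies exposed speed and gravity values to the projectile movement component.
; A cast chain on trigger overlap damages master-AI enemies unless DamageCheck returns true, damages Beetle Leech enemies, and makes inner eggs spawn enemies.
; Successful hits, tilemaps and static meshes destroy the bullet.
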(event OnComponentBeginOverlap(Trigger)
  (params (OverlappedComponent :type Primitive%20Component%20Object%20Reference) (OtherActor :type Actor%20Object%20Reference) (OtherComp :type Primitive%20Component%20Object%20Reference) (OtherBodyIndex :type Integer) (bFromSweep :type Boolean) (SweepResult :type Hit%20Result%20Structure%20%28by%20ref%29))
  (bind _player_ref (Variables|BaseInfo|GetPlayer%20Ref))
  ;[1 1 1] Damage Code
  (bind _asmaster_enemy_ai (Utilities|Casting|CastToMaster_Enemy_AI OtherActor)
    (:then
      (Utilities|IsValid _asmaster_enemy_ai
        (:Is%20Valid
          (bind _success_ (Default|DamageCheck _asmaster_enemy_ai (Variables|BaseInfo|GetDamage) (Variables|/Game/2DPlatformingKit/Blueprints/Player/Player_Character.Player_Character_C|GetChose%20Heal? _player_ref) (Variables|/Game/2DPlatformingKit/Blueprints/Player/Player_Character.Player_Character_C|GetChose%20Damage? _player_ref) (Variables|/Game/2DPlatformingKit/Blueprints/Player/Player_Character.Player_Character_C|GetFire%20Damage%20Buff%20Amount (Variables|BaseInfo|GetPlayer%20Ref))))
          (if (not _success_)
            (CallFunction|DamageEnemy _asmaster_enemy_ai (Variables|BaseInfo|GetDamage))
            (Actor|DestroyActor)))))
    (:CastFailed
      (bind _asleech_inner_egg_c (Utilities|Casting|CastToLeech_InnerEgg_C OtherActor)
        (:then
          (Default|SpawnEnemy _asleech_inner_egg_c))
        (:CastFailed
          (Utilities|Casting|CastToPaperTileMapActor OtherActor
            (:then
              (Actor|DestroyActor))
            (:CastFailed
              (bind _asbeetle_leech_db_e (Utilities|Casting|CastToBeetle_Leech_DB_E OtherActor)
                (:then
                  (Default|Damage _asbeetle_leech_db_e (- (Variables|/Game/2DPlatformingKit/Blueprints/BP_Enemies/General/Damage_Effects/Beetle_Leech_DB_E.Beetle_Leech_DB_E_C|GetHP _asbeetle_leech_db_e) (Variables|BaseInfo|GetDamage)) (Variables|BaseInfo|GetDamage))
                  (Actor|DestroyActor))
                (:CastFailed
                  (Utilities|Casting|CastToStaticMeshActor OtherActor)
                  (Actor|DestroyActor))))))))))

(event EventBeginPlay
  ;[1 1 1] Set Player Ref
  (bind _asplayer_character (Utilities|Casting|CastToPlayer_Character (Game|GetPlayerCharacter 0)))
  (Variables|BaseInfo|SetPlayer%20Ref _asplayer_character))

(event EventTick
  (params (DeltaSeconds :type Float%20%28single-precision%29))
  ;[1 1 1] Despawn
  (Utilities|FlowControl|Delay (Variables|BaseInfo|GetDespawn%20Delay))
  (Actor|DestroyActor))

(fn ConstructionScript
  (bind _projectilemovement (Variables|Default|GetProjectileMovement))
  ;[1 1 1] Setting main var
  (Variables|/Script/Engine.ProjectileMovementComponent|SetMaxSpeed _projectilemovement (Variables|BaseInfo|GetMax%20Speed))
  (Variables|/Script/Engine.ProjectileMovementComponent|SetInitialSpeed _projectilemovement (Variables|BaseInfo|GetStarting%20Speed))
  (Variables|/Script/Engine.ProjectileMovementComponent|SetProjectileGravityScale _projectilemovement (Variables|BaseInfo|GetGravity))
  (Variables|BaseInfo|SetDefault%20Velocity (Variables|/Script/Engine.MovementComponent|GetVelocity (Variables|Default|GetProjectileMovement))))