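; Player left-side collision helper that detects Leech_E enemies and turns them into an attached leech debuff.
; A fast looping timer, rather than attachment, keeps the actor offset to the player's left.
; When LeftBox overlaps a leech and that side is free, it spawns an Attached_Leech_EFX carrying the leech's HP.
; It then updates the player's leech counts and flag, applies the damage-over-time debuff and destroys the enemy.
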(event OnComponentBeginOverlap(LeftBox)
  (params (OverlappedComponent :type Primitive%20Component%20Object%20Reference) (OtherActor :type Actor%20Object%20Reference) (OtherComp :type Primitive%20Component%20Object%20Reference) (OtherBodyIndex :type Integer) (bFromSweep :type Boolean) (SweepResult :type Hit%20Result%20Structure%20%28by%20ref%29))
  (bind _player_ref (Variables|Default|GetPlayer%20Ref))
  (bind _player_ref_2 (Variables|Default|GetPlayer%20Ref))
  (bind _player_ref_3 (Variables|Default|GetPlayer%20Ref))
  (bind _asleech_e (Utilities|Casting|CastToLeech_E OtherActor))
  (if (not (Variables|/Game/2DPlatformingKit/Blueprints/Player/Player_Character.Player_Character_C|GetLeech%20on%20Left (Variables|Default|GetPlayer%20Ref)))
    (bind _returnvalue (Game|SpawnActorfromClass "/Game/2DPlatformingKit/Blueprints/BP_Combat/Debuffs/Attached_Leech_EFX.Attached_Leech_EFX_C" (Math|Transform|MakeTransform (Transformation|GetActorLocation (Variables|Default|GetPlayer%20Ref)) "0, 0, 0" "0.080000,0.080000,0.080000") "Undefined" 0 false false 0))
    (Default|SetHP _returnvalue (Variables|/Game/2DPlatformingKit/Blueprints/BP_Enemies/General/Master_Enemy_AI.Master_Enemy_AI_C|GetCurrent%20HP _asleech_e) (Variables|/Game/2DPlatformingKit/Blueprints/BP_Enemies/General/Master_Enemy_AI.Master_Enemy_AI_C|GetMax%20HP _asleech_e))
    (Math|Integer|IncrementInt (Variables|/Game/2DPlatformingKit/Blueprints/Player/Player_Character.Player_Character_C|GetAmount%20of%20Left%20Leeches _player_ref)
      (:%20%20
        (Math|Integer|IncrementInt (Variables|/Game/2DPlatformingKit/Blueprints/Player/Player_Character.Player_Character_C|GetTotal%20Amount%20of%20Leeches _player_ref)
          (:%20%20
            (bind _applyed_debuff (Default|ApplyDebuff _player_ref_2 "/Game/2DPlatformingKit/Blueprints/BP_Combat/Debuffs/Leech_DB.Leech_DB_C" (Variables|/Game/2DPlatformingKit/Blueprints/Player/Player_Character.Player_Character_C|GetLeech%20Damage%20Over%20Time _player_ref_2) (Variables|/Game/2DPlatformingKit/Blueprints/Player/Player_Character.Player_Character_C|GetLeech%20Ticks _player_ref_2) (Variables|/Game/2DPlatformingKit/Blueprints/Player/Player_Character.Player_Character_C|GetLeech%20Damage%20Occurrence _player_ref_2) "/Game/2DPlatformingKit/Blueprints/BP_Combat/Debuffs/Attached_Leech_EFX.Attached_Leech_EFX_C" false true 0.0))
            (Variables|/Game/2DPlatformingKit/Blueprints/Player/Player_Character.Player_Character_C|SetLeech%20Debuff _player_ref_3 _applyed_debuff)
            (Variables|/Game/2DPlatformingKit/Blueprints/Player/Player_Character.Player_Character_C|SetLeech%20on%20Left _player_ref_3 true)
            (Actor|DestroyActor _asleech_e)))))))

(event Custom|Set%20Location
  (Transformation|SetActorLocation (+ (Transformation|GetActorLocation (Variables|Default|GetPlayer%20Ref)) "-30.000000, 0, 0") false false))

(event EventBeginPlay
  (bind _asplayer_character (Utilities|Casting|CastToPlayer_Character (Game|GetPlayerCharacter 0)))
  (Variables|Default|SetPlayer%20Ref _asplayer_character)
  (Utilities|Time|SetTimerbyEvent (delegate Custom|Set%20Location) 0.001 true))

(fn ConstructionScript)