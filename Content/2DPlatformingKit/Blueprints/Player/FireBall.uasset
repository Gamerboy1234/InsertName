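; Fireball projectile for the 2D platforming kit that burns enemies on contact, with speed and gravity set in the construction script.
; Left or right timelines adjust its X velocity by SlowDown after spawn.
; Trigger overlap walks a cast chain of enemy and boss classes, applying damage (except Master_Enemy_AI), attaching Fire_BP and starting damage over time.
; It destroys itself on such hits or after a Tick-driven despawn delay.
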(event OnComponentBeginOverlap(Trigger)
  (params (OverlappedComponent :type Primitive%20Component%20Object%20Reference) (OtherActor :type Actor%20Object%20Reference) (OtherComp :type Primitive%20Component%20Object%20Reference) (OtherBodyIndex :type Integer) (bFromSweep :type Boolean) (SweepResult :type Hit%20Result%20Structure%20%28by%20ref%29))
  ;[1 1 1] Damage Code
  (bind _asmaster_enemy_bp (Utilities|Casting|CastToMaster_Enemy_BP OtherActor)
    (:then
      (Variables|Default|SetMaster%20Enemy _asmaster_enemy_bp)
      (Default|Damge _asmaster_enemy_bp (- (Variables|/Game/2DPlatformingKit/Blueprints/Enemy/NonBTAI/Master_Enemy_BP.Master_Enemy_BP_C|GetCurrent%20HP _asmaster_enemy_bp) (Variables|Default|GetDamge)) (Variables|Default|GetDamge))
      (Components|Movement|StopMovementImmediately (Variables|Default|GetProjectileMovement))
      (CallFunction|StopSlowDown)
      (bind _returnvalue (Game|SpawnActorfromClass "/Game/2DPlatformingKit/Blueprints/Inventory/Blueprints/ItemClasses/Spells/SpellEffects/Fire_BP.Fire_BP_C" (Transformation|GetActorTransform _asmaster_enemy_bp) "Undefined" 0 0))
      (bind _output_get (Variables|Default|SetFire _returnvalue))
      (Transformation|AttachActorToActor _output_get (Variables|Default|GetMaster%20Enemy) "Gun" "KeepRelative" "KeepRelative" "KeepRelative" false)
      (Transformation|SetActorTransform (Variables|Default|GetFire) (Transformation|GetActorTransform (Variables|Default|GetMaster%20Enemy)) false true)
      (Default|StartDamageOverTimeSlot1 (Variables|Default|GetMaster%20Enemy) (Variables|Default|GetDamage%20Over%20Time) (Variables|Default|GetFire) (Variables|Default|GetOccurrences) (Variables|Default|GetDamage%20Ticks%20))
      (Actor|DestroyActor))
    (:CastFailed
      (bind _aspriest (Utilities|Casting|CastToPriest OtherActor)
        (:then
          (Variables|Default|SetPriest%20Boss _aspriest)
          (Default|Damge _aspriest (- (Variables|/Game/2DPlatformingKit/Levels/BossBlueprints/Priest.Priest_C|GetCurrent%20HP _aspriest) (Variables|Default|GetDamge)) (Variables|Default|GetDamge))
          (Components|Movement|StopMovementImmediately (Variables|Default|GetProjectileMovement))
          (CallFunction|StopSlowDown)
          (bind _returnvalue_2 (Game|SpawnActorfromClass "/Game/2DPlatformingKit/Blueprints/Inventory/Blueprints/ItemClasses/Spells/SpellEffects/Fire_BP.Fire_BP_C" (Transformation|GetActorTransform (Variables|Default|GetPriest%20Boss)) "Undefined" 0 0))
          (bind _output_get_2 (Variables|Default|SetFire _returnvalue_2))
          (Transformation|AttachActorToActor _output_get_2 (Variables|Default|GetPriest%20Boss) "Gun" "KeepRelative" "KeepRelative" "KeepRelative" false)
          (Transformation|SetActorTransform (Variables|Default|GetFire) (Transformation|GetActorTransform (Variables|Default|GetPriest%20Boss)) false true)
          (Default|StartDamageOverTime (Variables|Default|GetPriest%20Boss) (Variables|Default|GetDamage%20Over%20Time) (Variables|Default|GetFire) (Variables|Default|GetOccurrences) (Variables|Default|GetDamage%20Ticks%20))
          (Actor|DestroyActor))
        (:CastFailed
          (bind _asjn_ranged_bp (Utilities|Casting|CastToJN_Ranged_BP OtherActor)
            (:then
              (bind _output_get_3 (Variables|Default|SetJN%20Ranged _asjn_ranged_bp))
              (Default|Damage _output_get_3 (Variables|Default|GetDamge))
              (Components|Movement|StopMovementImmediately (Variables|Default|GetProjectileMovement))
              (CallFunction|StopSlowDown)
              (bind _returnvalue_3 (Game|SpawnActorfromClass "/Game/2DPlatformingKit/Blueprints/Inventory/Blueprints/ItemClasses/Spells/SpellEffects/Fire_BP.Fire_BP_C" (Transformation|GetActorTransform (Variables|Default|GetJN%20Ranged)) "Undefined" 0 0))
              (bind _output_get_4 (Variables|Default|SetFire _returnvalue_3))
              (Transformation|AttachActorToActor _output_get_4 (Variables|Default|GetJN%20Ranged) "Gun" "KeepRelative" "KeepRelative" "KeepRelative" false)
              (Transformation|SetActorTransform (Variables|Default|GetFire) (Transformation|GetActorTransform (Variables|Default|GetJN%20Ranged)) false true)
              (Default|StartDamageOverTime (Variables|Default|GetJN%20Ranged) (Variables|Default|GetDamage%20Ticks%20) (Variables|Default|GetDamage%20Over%20Time) (Variables|Default|GetFire) (Variables|Default|GetOccurrences))
              (Actor|DestroyActor))
            (:CastFailed
              (bind _ascorrupted_bp (Utilities|Casting|CastToCorrupted_BP OtherActor)
                (:then
                  (bind _output_get_5 (Variables|Default|SetThe%20Corrupted _ascorrupted_bp))
                  (Default|Damge _output_get_5 (- (Variables|/Game/2DPlatformingKit/Blueprints/Enemy/NonBTAI/Corrupted_BP.Corrupted_BP_C|GetCurrent%20HP _ascorrupted_bp) (Variables|Default|GetDamge)) (Variables|Default|GetDamge))
                  (Components|Movement|StopMovementImmediately (Variables|Default|GetProjectileMovement))
                  (CallFunction|StopSlowDown)
                  (bind _returnvalue_4 (Game|SpawnActorfromClass "/Game/2DPlatformingKit/Blueprints/Inventory/Blueprints/ItemClasses/Spells/SpellEffects/Fire_BP.Fire_BP_C" (Transformation|GetActorTransform (Variables|Default|GetThe%20Corrupted)) "Undefined" 0 0))
                  (bind _output_get_6 (Variables|Default|SetFire _returnvalue_4))
                  (Transformation|AttachActorToActor _output_get_6 (Variables|Default|GetThe%20Corrupted) "Gun" "KeepRelative" "KeepRelative" "KeepRelative" false)
                  (Transformation|SetActorTransform (Variables|Default|GetFire) (Transformation|GetActorTransform (Variables|Default|GetThe%20Corrupted)) false true)
                  (Default|StartDamageOverTime (Variables|Default|GetThe%20Corrupted) (Variables|Default|GetDamage%20Ticks%20) (Variables|Default|GetDamage%20Over%20Time) (Variables|Default|GetFire) (Variables|Default|GetOccurrences))
                  (Actor|DestroyActor))
                (:CastFailed
                  (bind _asmaster_enemy_ai (Utilities|Casting|CastToMaster_Enemy_AI OtherActor))
                  (Variables|Default|SetMaster%20Enemy%20AI _asmaster_enemy_ai)
                  (Components|Movement|StopMovementImmediately (Variables|Default|GetProjectileMovement))
                  (CallFunction|StopSlowDown)
                  (bind _returnvalue_5 (Game|SpawnActorfromClass "/Game/2DPlatformingKit/Blueprints/Inventory/Blueprints/ItemClasses/Spells/SpellEffects/Fire_BP.Fire_BP_C" (Transformation|GetActorTransform (Variables|Default|GetMaster%20Enemy%20AI)) "Undefined" 0 0))
                  (bind _output_get_7 (Variables|Default|SetFire _returnvalue_5))
                  (Transformation|AttachActorToActor _output_get_7 (Variables|Default|GetMaster%20Enemy%20AI) "Gun" "KeepRelative" "KeepRelative" "KeepRelative" false)
                  (Transformation|SetActorTransform (Variables|Default|GetFire) (Transformation|GetActorTransform (Variables|Default|GetMaster%20Enemy%20AI)) false true)
                  (Default|StartDamageOverTimeSlot1 (Variables|Default|GetMaster%20Enemy%20AI) (Variables|Default|GetDamage%20Over%20Time) (Variables|Default|GetFire) (Variables|Default|GetOccurrences) (Variables|Default|GetDamage%20Ticks%20))
                  (Actor|DestroyActor))))))))))

(event Custom|Stop%20Slow%20Down
  (bind _left_slowdown (Variables|Default|GetLeft%20SlowDown))
  (bind _right_slow_down (Variables|Default|GetRight%20Slow%20Down))
  ;[1 1 1] Slow Down Code
  (Utilities|IsValid _left_slowdown
    (:Is%20Valid
      (Audio|Components|Audio|Stop _left_slowdown))
    (:Is%20Not%20Valid
      (Utilities|IsValid _right_slow_down
        (:Is%20Valid
          (Audio|Components|Audio|Stop _right_slow_down))))))

(event EventTick
  (params (DeltaSeconds :type Float%20%28single-precision%29))
  ;[1 1 1] Despawn
  (Utilities|FlowControl|Delay (Variables|Default|GetDespawn%20Delay))
  (Actor|DestroyActor))

(event EventBeginPlay
  ;[1 1 1] Get Player Ref
  (bind _asplayer_character (Utilities|Casting|CastToPlayer_Character (Game|GetPlayerCharacter 0)))
  (Variables|Default|SetPlayer%20Ref _asplayer_character)
  ;[1 1 1] Slow Down Code
  (if (> (.x (Variables|/Script/Engine.MovementComponent|GetVelocity (Variables|Default|GetProjectileMovement))) -1.0)
    (Timeline|Right%20Slow%20Down PlayFromStart
      (:Update
        (if (> (.x (Variables|/Script/Engine.MovementComponent|GetVelocity (Variables|Default|GetProjectileMovement))) -1.0)
          (Game|Components|ProjectileMovement|SetVelocityinLocalSpace (Variables|Default|GetProjectileMovement) (Math|Vector|MakeVector (- (.x (Variables|/Script/Engine.MovementComponent|GetVelocity (Variables|Default|GetProjectileMovement))) (Variables|Default|GetSlow%20Down%20)) 0.0 0.0))
          (else
            (Audio|Components|Audio|Stop (Variables|Default|GetRight%20Slow%20Down))))))
    (else
      (Timeline|Left%20SlowDown PlayFromStart
        (:Update
          (if (< (.x (Variables|/Script/Engine.MovementComponent|GetVelocity (Variables|Default|GetProjectileMovement))) 1.0)
            (Game|Components|ProjectileMovement|SetVelocityinLocalSpace (Variables|Default|GetProjectileMovement) (Math|Vector|MakeVector (* (+ (.x (Variables|/Script/Engine.MovementComponent|GetVelocity (Variables|Default|GetProjectileMovement))) (Variables|Default|GetSlow%20Down%20)) -1.0) 0.0 0.0))
            (else
              (Audio|Components|Audio|Stop (Variables|Default|GetLeft%20SlowDown)))))))))

(fn ConstructionScript
  (bind _projectilemovement (Variables|Default|GetProjectileMovement))
  ;[1 1 1] Setting Speed and gravity
  (Variables|/Script/Engine.ProjectileMovementComponent|SetInitialSpeed _projectilemovement (Variables|Default|GetStarting%20Speed))
  (Variables|/Script/Engine.ProjectileMovementComponent|SetMaxSpeed _projectilemovement (Variables|Default|GetMax%20Speed))
  (Variables|/Script/Engine.ProjectileMovementComponent|SetProjectileGravityScale _projectilemovement (Variables|Default|GetGravity)))