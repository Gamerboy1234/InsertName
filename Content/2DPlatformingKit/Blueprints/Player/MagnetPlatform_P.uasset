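; Magnet platform projectile for a 2D platformer that flies out, stops in place and destroys itself after a set lifespan.
; Construction applies speed and gravity to its ProjectileMovement; BeginPlay locks it to Y=0.
; Movement stops when its trigger overlaps anything but the gun, or when Tick finds its X at or below EndPoint.X.
; On spawn it counts instances of its class and destroys those indexed beyond MaxPlatforms.
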(event OnComponentBeginOverlap(Trigger)
  (params (OverlappedComponent :type Primitive%20Component%20Object%20Reference) (OtherActor :type Actor%20Object%20Reference) (OtherComp :type Primitive%20Component%20Object%20Reference) (OtherBodyIndex :type Integer) (bFromSweep :type Boolean) (SweepResult :type Hit%20Result%20Structure%20%28by%20ref%29))
  ;[1 1 1] Stop when it walls
  (Utilities|Casting|CastToMaster_GunBP OtherActor
    (:CastFailed
      (Components|Movement|StopMovementImmediately (Variables|Default|GetProjectileMovement)))))

(event EventBeginPlay
  (bind _returnvalue (Transformation|GetActorLocation))
  ;[1 1 1] Check to see if platform count is above max platforms
  (CallFunction|CountPlatforms)
  (bind _asplayer_character (Utilities|Casting|CastToPlayer_Character (Game|GetPlayerCharacter 0)))
  (Variables|Default|SetPlayer%20ref _asplayer_character)
  ;[1 1 1] Set Y level to 0
  (Transformation|SetActorLocation (Math|Vector|MakeVector (.x _returnvalue) 0.0 (.z _returnvalue)) false true))

(event EventTick
  (params (DeltaSeconds :type Float%20%28single-precision%29))
  (Utilities|FlowControl|Sequence
    (:then_0
      ;[1 1 1] Life Span
      (Utilities|FlowControl|Delay (Variables|Default|GetPlatform%20Life%20Span))
      (Actor|DestroyActor))
    (:then_1
      (if (>= (.x (Variables|Default|GetEnd%20Point)) (.x (Transformation|GetActorLocation)))
        (Components|Movement|StopMovementImmediately (Variables|Default|GetProjectileMovement))))))

(fn ConstructionScript
  (bind _projectilemovement (Variables|Default|GetProjectileMovement))
  (Variables|/Script/Engine.ProjectileMovementComponent|SetInitialSpeed _projectilemovement (Variables|Default|GetStarting%20Speed))
  (Variables|/Script/Engine.ProjectileMovementComponent|SetMaxSpeed _projectilemovement (Variables|Default|GetMax%20Speed))
  (Variables|/Script/Engine.ProjectileMovementComponent|SetProjectileGravityScale (Variables|Default|GetProjectileMovement) (Variables|Default|GetGravity))
  (Variables|Default|SetEnd%20Point "0, 0, 0"))

(fn CountPlatforms
  ;[1 1 1] Count Platforms
  (bind _outactors (Actor|GetAllActorsOfClass (Utilities|GetClass self)))
  (Variables|Default|SetPlatforms _outactors)
  (if (> (Utilities|Array|Length _outactors) (Variables|Default|GetMax%20Platforms))
    ;[1 1 1] Remove last placed platform
    (for (_array_element _array_index) (Variables|Default|GetPlatforms)
      (if (> _array_index (Variables|Default|GetMax%20Platforms))
        (Math|Integer|DecrementInt _array_index
          (:%20%20
            (Actor|DestroyActor _array_element)))))))