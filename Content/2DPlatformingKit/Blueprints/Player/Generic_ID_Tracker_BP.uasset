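; Generic ID tracker Blueprint in the 2D platforming kit that hands out random integer IDs and records each one in an array.
; GenID draws a random number, checks it against the stored IDs with a linear search, and adds it through AddToID before returning it.
; A collision gets a single retry, after which it stores and returns zero, so uniqueness is not guaranteed.
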(fn ConstructionScript)

(fn AddtoID
  (params (ID :type Integer))
  (Utilities|Array|Add (Variables|Default|GetID) ID))

(fn GenID
  (bind _output_get (LocalVariables|Setlocal%20ID (Class|RandomNumberNoRepeat|RandomNumber 0 1000000)))
  (if (not (CallFunction|NumberAlreadyExist? _output_get))
    (CallFunction|AddtoID (LocalVariables|Getlocal%20ID))
    (return (LocalVariables|Getlocal%20ID))
    (else
      (LocalVariables|Setlocal%20ID (Class|RandomNumberNoRepeat|RandomNumber 0 1000000))
      (if (not (CallFunction|NumberAlreadyExist? (LocalVariables|Getlocal%20ID)))
        (CallFunction|AddtoID (LocalVariables|Getlocal%20ID))
        (return (LocalVariables|Getlocal%20ID))
        (else
          (CallFunction|AddtoID)
          (return 0))))))

(fn NumberAlreadyExist?
  (params (ID :type Integer))
  (LocalVariables|SetLocal%20ID ID)
  (bind _array_element (Utilities|Array|ForEachLoopwithBreak (Variables|Default|GetID) :!label _label)
    (:LoopBody
      (if (== (LocalVariables|GetLocal%20ID) _array_element)
        (LocalVariables|SetLocal%20Bool true)
        (goto _label Break)
        (else
          (LocalVariables|SetLocal%20Bool false))))
    (:Completed
      (return (LocalVariables|GetLocal%20Bool)))))