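; Temporary magnet platform for the 2D platformer player that can be set ablaze by the jet to burn enemies.
; On BeginPlay it scans actors of its own class, destroying those indexed above MaxPlatforms; a Delay on Tick handles its lifespan.
; UpdateTexturetoFire tints the sprite and burns the last overlapping enemy.
; While lit, new overlaps apply a fire debuff to Master_Enemy_AI not already burning.
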(event OnComponentEndOverlap(FireCoillision)
  (params (OverlappedComponent :type Primitive%20Component%20Object%20Reference) (OtherActor :type Actor%20Object%20Reference) (OtherComp :type Primitive%20Component%20Object%20Reference) (OtherBodyIndex :type Integer))
  ;[1 1 1] If jet has been used on magnet and a enemy hit the platform set it on fire
  (Utilities|Casting|CastToMaster_Enemy_AI OtherActor)
  (Variables|FireDamage|SetDid%20enemy%20touch%20platform? false))

(event OnComponentBeginOverlap(FireCoillision)
  (params (OverlappedComponent :type Primitive%20Component%20Object%20Reference) (OtherActor :type Actor%20Object%20Reference) (OtherComp :type Primitive%20Component%20Object%20Reference) (OtherBodyIndex :type Integer) (bFromSweep :type Boolean) (SweepResult :type Hit%20Result%20Structure%20%28by%20ref%29))
  ;[1 1 1] If jet has been used on magnet and a enemy hit the platform set it on fire
  (bind _asmaster_enemy_ai (Utilities|Casting|CastToMaster_Enemy_AI OtherActor))
  (Variables|FireDamage|SetDid%20enemy%20touch%20platform? true)
  (Variables|Default|SetTouched%20Enemy _asmaster_enemy_ai)
  (if (Variables|FireDamage|GetOn%20Fire?)
    (if (not (Variables|/Game/2DPlatformingKit/Blueprints/BP_Enemies/General/Master_Enemy_AI.Master_Enemy_AI_C|GetCurrently%20on%20Fire? _asmaster_enemy_ai))
      (CallFunction|ApplyFireDamage _asmaster_enemy_ai))))

(event Custom|Update%20Texture%20to%20Fire
  ;[1 1 1] When hit by SP Jet this updates the texture and set's enemies on fire
  (Sprite|SetSpriteColor (Variables|Default|GetPlatform%20Sprite) "(R=1.000000,G=0.154240,B=0.000000,A=1.000000)")
  (Variables|FireDamage|SetOn%20Fire? true)
  (if (Variables|FireDamage|GetDid%20enemy%20touch%20platform?)
    (CallFunction|ApplyFireDamage (Variables|Default|GetTouched%20Enemy))))

(event EventBeginPlay
  ;[1 1 1] Check to see if platform count is above max platforms
  (CallFunction|CountPlatforms)
  (bind _asplayer_character (Utilities|Casting|CastToPlayer_Character (Game|GetPlayerCharacter 0)))
  (Variables|PlatformInfo|SetPlayer%20ref _asplayer_character))

(event EventTick
  (params (DeltaSeconds :type Float%20%28single-precision%29))
  ;[1 1 1] Life Span
  (Utilities|FlowControl|Delay (Variables|PlatformInfo|GetPlatform%20Life%20Span))
  (Actor|DestroyActor))

(fn ConstructionScript)

(fn CountPlatforms
  ;[1 1 1] Count Platforms
  (bind _outactors (Actor|GetAllActorsOfClass (Utilities|GetClass self)))
  (Variables|PlatformInfo|SetPlatforms _outactors)
  (if (> (Utilities|Array|Length _outactors) (Variables|PlatformInfo|GetMax%20Platforms))
    ;[1 1 1] Remove last placed platform
    (for (_array_element _array_index) (Variables|PlatformInfo|GetPlatforms)
      (if (> _array_index (Variables|PlatformInfo|GetMax%20Platforms))
        (Math|Integer|DecrementInt _array_index
          (:%20%20
            (Actor|DestroyActor _array_element)))))))

(fn ApplyFireDamage
  (params (Enemy :type Master%20Enemy%20AI%20Object%20Reference))
  (bind _output_get (LocalVariables|SetLocal%20E Enemy))
  (Default|ApplyDebuff _output_get (Variables|FireDamage|GetAmount%20of%20Fire%20Damage) "/Game/2DPlatformingKit/Blueprints/BP_Combat/Spells/SpellEffects/Fire_BP_EFX.Fire_BP_EFX_C" (Variables|FireDamage|GetFire%20Damage%20Occurrence) (Variables|FireDamage|GetFire%20Ticks) "5.000000,5.000000,5.000000")
  (Variables|/Game/2DPlatformingKit/Blueprints/BP_Enemies/General/Master_Enemy_AI.Master_Enemy_AI_C|SetCurrently%20on%20Fire? (LocalVariables|GetLocal%20E) true))