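; Tracker Blueprint that shows floating combat text for damage at a target actor's on-screen position.
; AddtoCombatText stores the actor and, only if no valid widget exists, creates a Floating_Combat_Text widget with the damage and a reference to itself.
; Tick projects the actor's location to screen space each frame and moves the widget there.
; Later calls while the widget is valid retarget it without updating the damage.
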(event Custom|Add%20to%20Combat%20Text
  (params (Actor%20to%20Add :type Actor%20Object%20Reference) (Damage :type Float%20%28single-precision%29))
  ;[1 1 1] Setup Actor array and create floating combat text
  (Variables|Default|SetActor Actor%20to%20Add)
  (Utilities|IsValid (Variables|Default|GetWidget%20Ref)
    (:Is%20Not%20Valid
      (bind _returnvalue (UserInterface|CreateWidget "/Game/2DPlatformingKit/Widgets/Player_Widgets/Floating_Combat_Text.Floating_Combat_Text_C" 0 Damage self))
      (bind _output_get (Variables|Default|SetWidget%20Ref _returnvalue))
      (UserInterface|Viewport|AddtoViewport _output_get 0))))

(event EventTick
  (params (DeltaSeconds :type Float%20%28single-precision%29))
  ;[1 1 1] Update Widget location
  (Utilities|IsValid (Variables|Default|GetWidget%20Ref)
    (:Is%20Valid
      (Utilities|IsValid (Variables|Default|GetActor)
        (:Is%20Valid
          (Class|UserWidget|SetPositioninViewport (Variables|Default|GetWidget%20Ref) (.ScreenLocation (Class|PlayerController|ProjectWorldLocationtoScreen (Game|GetPlayerController 0) (Transformation|GetActorLocation (Variables|Default|GetActor)) true)) false))))))

(fn ConstructionScript)