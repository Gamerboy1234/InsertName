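; Camera zone actor for a 2D platformer that becomes the player's view target, with a configurable blend, when the Player_Character overlaps its collision box.
; Each tick its camera eases toward the player's X and Z, clamped within a bounds box, while keeping its own Y.
; The construction script applies exposed transforms, extents and FOV to the camera and both boxes.
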(event OnComponentBeginOverlap(ActorCollsion)
  (params (OverlappedComponent :type Primitive%20Component%20Object%20Reference) (OtherActor :type Actor%20Object%20Reference) (OtherComp :type Primitive%20Component%20Object%20Reference) (OtherBodyIndex :type Integer) (bFromSweep :type Boolean) (SweepResult :type Hit%20Result%20Structure%20%28by%20ref%29))
  (bind _asplayer_character (Utilities|Casting|CastToPlayer_Character OtherActor))
  (Variables|Default|SetPlayer%20Ref _asplayer_character)
  ;[1 1 1] Changing Camera
  (Game|Player|SetViewTargetwithBlend (Game|GetPlayerController 0) self (Variables|CameraSettings|GetBlend%20Time) (Variables|CameraSettings|GetBlend%20Func) (Variables|CameraSettings|GetBlend%20Exp) false))

(event EventTick
  (params (DeltaSeconds :type Float%20%28single-precision%29))
  (bind _returnvalue (Game|GetPlayerCharacter 0))
  (bind _camera_bound_box (Variables|Default|GetCamera%20Bound%20Box))
  (bind _camera (Variables|Default|GetCamera))
  (bind _returnvalue_2 (Transformation|GetActorLocation _returnvalue))
  (bind (_origin _boxextent) (Collision|GetComponentBounds _camera_bound_box))
  (bind _returnvalue_3 (- _origin _boxextent))
  (bind _returnvalue_4 (+ _origin _boxextent))
  ;[1 1 1] Move Camera With Player
  (Transformation|SetWorldLocation (Variables|Default|GetCamera) (Math|Interpolation|VInterpTo (Transformation|GetWorldLocation _camera) (Math|Vector|MakeVector (Math|Float|Clamp(Float) (.x _returnvalue_2) (.x _returnvalue_3) (.x _returnvalue_4)) (.y (Transformation|GetWorldLocation _camera)) (Math|Float|Clamp(Float) (.z _returnvalue_2) (.z _returnvalue_3) (.z _returnvalue_4))) DeltaSeconds (Variables|CameraSettings|GetCamera%20Lag)) false false))

(fn ConstructionScript
  (bind _actor_collsion (Variables|Default|GetActor%20Collsion))
  (bind _camera_bound_box (Variables|Default|GetCamera%20Bound%20Box))
  (bind _camera (Variables|Default|GetCamera))
  (Utilities|FlowControl|Sequence
    (:then_0
      (Transformation|SetRelativeTransform _camera (Variables|CameraSettings|GetCamera%20Tarnsform) false false)
      (Variables|/Script/Engine.CameraComponent|SetFieldOfView _camera (Variables|CameraSettings|GetFOV)))
    (:then_1
      (Transformation|SetRelativeTransform _actor_collsion (Variables|CameraSettings|GetActor%20Collsion%20Transform) false false)
      (Components|Box|SetBoxExtent _actor_collsion (Variables|CameraSettings|GetActor%20Collsion%20Extent) true))
    (:then_2
      (Transformation|SetRelativeTransform _camera_bound_box (Variables|CameraSettings|GetCamera%20Bounds%20Transform) false false)
      (Components|Box|SetBoxExtent _camera_bound_box (Variables|CameraSettings|GetCamera%20Bounds%20Box%20Extent) true))))