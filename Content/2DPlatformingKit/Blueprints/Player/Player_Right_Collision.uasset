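; Player_Right_Collision is a hitbox that trails the player's right side to catch incoming leeches.
; On BeginPlay it caches the Player_Character and starts a fast looping timer that moves it to a fixed world X offset from the player.
; Each RightBox overlap runs the player's flame magnet damage check.
; If the actor is a Leech_E that can attach, it spawns a right-side attached leech on the player.
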(event OnComponentBeginOverlap(RightBox)
  (params (OverlappedComponent :type Primitive%20Component%20Object%20Reference) (OtherActor :type Actor%20Object%20Reference) (OtherComp :type Primitive%20Component%20Object%20Reference) (OtherBodyIndex :type Integer) (bFromSweep :type Boolean) (SweepResult :type Hit%20Result%20Structure%20%28by%20ref%29))
  (bind _player_ref (Variables|Default|GetPlayer%20Ref))
  ;[1 1 1] If leech hits this box then attach it to the player
  (Default|FlameMagnetDamageCheck (Variables|Default|GetPlayer%20Ref) OtherActor)
  (bind _asleech_e (Utilities|Casting|CastToLeech_E OtherActor))
  (Variables|Default|SetIncoming%20Leech _asleech_e)
  (if (CallFunction|CanIncomingLeechAttach? (Variables|Default|GetIncoming%20Leech) (Variables|Default|GetPlayer%20Ref) false true)
    (Utilities|SpawnAttachedLeech true false (Math|Transform|MakeTransform (Transformation|GetActorLocation _player_ref) "0, 0, 0" "0.150000,0.150000,0.150000") (Variables|Default|GetIncoming%20Leech) _player_ref)))

(event Custom|Set%20Location
  ;[1 1 1] Keep Hitbox on player's right side
  (Transformation|SetActorLocation (+ (Transformation|GetActorLocation (Variables|Default|GetPlayer%20Ref)) "30.000000, 0, 0") false false))

(event EventBeginPlay
  ;[1 1 1] Keep Hitbox on player's right side
  (bind _asplayer_character (Utilities|Casting|CastToPlayer_Character (Game|GetPlayerCharacter 0)))
  (Variables|Default|SetPlayer%20Ref _asplayer_character)
  (Utilities|Time|SetTimerbyEvent (delegate Custom|Set%20Location) 0.001 true))

(fn ConstructionScript)