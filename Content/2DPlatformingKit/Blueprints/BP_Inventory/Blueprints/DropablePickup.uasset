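; Dropped-item pickup that flies out on projectile movement, then stops with zero gravity after a short delay and expires ten seconds later.
; Player overlap on the trigger calls PickupItem after a brief delay when pickup is allowed, then clears CanPickUp.
; An overlap while pickup is blocked only starts a timed re-enable of CanPickUp, without collecting the item.
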(event OnComponentBeginOverlap(Trigger)
  (params (OverlappedComponent :type Primitive%20Component%20Object%20Reference) (OtherActor :type Actor%20Object%20Reference) (OtherComp :type Primitive%20Component%20Object%20Reference) (OtherBodyIndex :type Integer) (bFromSweep :type Boolean) (SweepResult :type Hit%20Result%20Structure%20%28by%20ref%29))
  ;[1 1 1] On overlay start pickup event
  (Utilities|Casting|CastToPlayer_Character OtherActor)
  (if (Variables|Default|GetCan%20Pick%20up?)
    (CallFunction|PickupEvent)
    (else
      (CallFunction|PickupDelay))))

(event Custom|Pickup%20Delay
  ;[1 1 1] Start Pickup Delay
  (Utilities|FlowControl|Delay 2.0)
  (Variables|Default|SetCan%20Pick%20up? true))

(event EventBeginPlay
  (bind _projectilemovement (Variables|Default|GetProjectileMovement))
  ;[1 1 1] Get Player ref and stop movement
  (bind _asplayer_character (Utilities|Casting|CastToPlayer_Character (Game|GetPlayerCharacter 0)))
  (Variables|Default|SetPlayer%20Ref _asplayer_character)
  (Utilities|FlowControl|Delay 0.3)
  (Components|Movement|StopMovementImmediately _projectilemovement)
  (Variables|/Script/Engine.ProjectileMovementComponent|SetProjectileGravityScale _projectilemovement 0.0)
  (Variables|Default|SetIs%20Done%20Moving? true)
  (Actor|SetLifeSpan 1e+01))

(event EventPickupEvent
  ;[1 1 1] Start Item Pickup
  (Utilities|FlowControl|Delay 0.3)
  (if (Variables|Default|GetCan%20Pick%20up?)
    (CallFunction|PickupItem)
    (Variables|Default|SetCan%20Pick%20up? false)))

(fn ConstructionScript
  (|CallParentFunction))