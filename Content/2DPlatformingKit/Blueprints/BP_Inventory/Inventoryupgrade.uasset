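; Inventory upgrade item for the 2D platforming kit that expands the player's inventory slot count when used.
; On use, it checks the player character's inventory and shows an on-screen message if that inventory already has 100 or more slots.
; Otherwise it adds a configurable number of slots, removes one of itself from its inventory index without spawning a dropped actor, and destroys itself if the removal succeeds.
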(event EventItemUsed
  (bind _asplayer_character (Utilities|Casting|CastToPlayer_Character (Game|GetPlayerCharacter 0)))
  (Variables|Default|SetPlayer%20Ref _asplayer_character)
  (if (>= (Variables|/Game/2DPlatformingKit/Blueprints/BP_Inventory/Blueprints/Inventory_Master.Inventory_Master_C|GetAmountofSlots (Variables|/Game/2DPlatformingKit/Blueprints/Player/Player_Character.Player_Character_C|GetInventory%20Ref (Variables|Default|GetPlayer%20Ref))) 100)
    (Utilities|UIScreenText "Inventory fully upgraded")
    (else
      (Default|AddInventorySlots (Variables|Default|GetInventory) (Variables|Default|GetAmount%20of%20Slots%20to%20add))
      (bind _success (Default|RemoveItematIndex (Variables|Default|GetInventory) (Variables|Default|GetIndex) 1 false))
      (if _success
        (Actor|DestroyActor)))))

(fn ConstructionScript
  (|CallParentFunction))