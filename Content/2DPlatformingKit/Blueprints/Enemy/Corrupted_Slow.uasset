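; Corrupted_Slow is an enemy Blueprint in the 2D platforming kit that detects the player nearby along the X axis.
; Each Tick it fires two short Visibility line traces from its location, one toward each side.
; If either trace hits the player character, it sets the Ag flag, which this file never clears or acts on.
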(event EventTick
  (params (DeltaSeconds :type Float%20%28single-precision%29))
  (bind _returnvalue (Transformation|GetActorLocation))
  (bind _returnvalue_2 (Transformation|GetActorLocation))
  (Utilities|FlowControl|Sequence
    (:then_0
      (bind _outhit (Collision|LineTraceByChannel _returnvalue_2 (+ _returnvalue_2 "-100.000000, 0, 0") "TraceTypeQuery1" false 0 "None"))
      (if (== (.HitActor (Collision|BreakHitResult _outhit)) (Game|GetPlayerCharacter 0))
        (Variables|Default|Setag true)))
    (:then_1
      (bind _outhit_2 (Collision|LineTraceByChannel _returnvalue (+ _returnvalue "100.000000, 0, 0") "TraceTypeQuery1" false 0 "None"))
      (if (== (.HitActor (Collision|BreakHitResult _outhit_2)) (Game|GetPlayerCharacter 0))
        (Variables|Default|Setag true)))))

(fn ConstructionScript)