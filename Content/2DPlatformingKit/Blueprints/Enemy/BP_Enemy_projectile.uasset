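; Enemy projectile for the 2D platforming kit that resolves its impact when its collision component hits something, then destroys itself.
; Hit components tagged as destroyable send their actor a damage interface message with the hit normal for knockback.
; Block-tagged components count as shield blocks and take no damage; anything else counts as a generic collision.
; Each outcome spawns its own particle effect and half-scale hit sprite actor at the impact location.
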(event OnComponentHit(Collision)
  (params (HitComponent :type Primitive%20Component%20Object%20Reference) (OtherActor :type Actor%20Object%20Reference) (OtherComp :type Primitive%20Component%20Object%20Reference) (NormalImpulse :type Vector :default "0, 0, 0") (Hit :type Hit%20Result%20Structure%20%28by%20ref%29))
  (bind _collision (Variables|Default|GetCollision))
  (bind _returnvalue (Transformation|GetWorldLocation _collision))
  ;[1 1 1] Enemy Projectile
  ;;[0.1595 0.2271 1] Check to see if it hits an object with the destroyable tag
  (if (Components|ComponentHasTag OtherComp (Variables|Default|GetDestroyableTag))
    ;;[0.1595 0.2271 1] Blueprint Interface Damage function
    (Class|InteractionHandler|ActorDamagedbyObject(Message) OtherActor (Variables|Default|GetDamage) (.Normal (Collision|BreakHitResult Hit)))
    ;;[0.1595 0.2271 1] If hit actor then spawn blood FX at the location
    (Effects|SpawnEmitteratLocation (Variables|Default|GetbloodHitFX) _returnvalue)
    (Game|SpawnActorfromClass (Variables|Default|GetactorHitSprite) (Math|Transform|MakeTransform _returnvalue "0, 0, 0" "0.500000,0.500000,0.500000") "AdjustIfPossibleButDontSpawnIfColliding" 0 0)
    (Actor|DestroyActor)
    (else
      ;;[0.1595 0.2271 1] Check to see if we hit the player Shield
      (if (Components|ComponentHasTag OtherComp (Variables|Default|GetBlockTag))
        (Development|PrintString "Damage Blocked by Shield")
        ;;[0.1595 0.2271 1] If we hit the player shield then spawn block FX
        (Effects|SpawnEmitteratLocation (Variables|Default|GetshieldBlockFX) _returnvalue)
        (Game|SpawnActorfromClass (Variables|Default|GetshieldHitSprite) (Math|Transform|MakeTransform _returnvalue "0, 0, 0" "0.500000,0.500000,0.500000") "AdjustIfPossibleButDontSpawnIfColliding" 0 0)
        (Actor|DestroyActor)
        (else
          ;;[0.1595 0.2271 1] IF we hit a collider then spawn generic collide FX
          (Effects|SpawnEmitteratLocation (Variables|Default|GetgroundHitFX) _returnvalue)
          (Game|SpawnActorfromClass (Variables|Default|GetgroundHitSprite) (Math|Transform|MakeTransform _returnvalue "0, 0, 0" "0.500000,0.500000,0.500000") "AdjustIfPossibleButDontSpawnIfColliding" 0 0)
          (Actor|DestroyActor))))))

(fn ConstructionScript)