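; The Corrupted is a 2D platformer enemy that detects the player at close range.
; It caches the player character on BeginPlay.
; Each Tick it fires two short Visibility line traces along world X, one in each direction, ignoring itself.
; A hit on the player sets the Ag flag, which this graph never clears or acts on.
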(event EventTick
  (params (DeltaSeconds :type Float%20%28single-precision%29))
  (bind _returnvalue (Transformation|GetActorLocation))
  (bind _returnvalue_2 (Transformation|GetActorLocation))
  (Utilities|FlowControl|Sequence
    (:then_0
      (bind _outhit (Collision|LineTraceByChannel _returnvalue_2 (+ _returnvalue_2 "50.000000, 0, 0") "TraceTypeQuery1" false (Utilities|Array|MakeArray self) "None"))
      (if (== (.HitActor (Collision|BreakHitResult _outhit)) (Variables|Default|GetPlayer%20Ref))
        (Variables|Default|Setag true)))
    (:then_1
      (bind _outhit_2 (Collision|LineTraceByChannel _returnvalue (+ _returnvalue "-50.000000, 0, 0") "TraceTypeQuery1" false (Utilities|Array|MakeArray self) "None"))
      (if (== (.HitActor (Collision|BreakHitResult _outhit_2)) (Variables|Default|GetPlayer%20Ref))
        (Variables|Default|Setag true)))))

(event EventBeginPlay
  (bind _asplayer_character (Utilities|Casting|CastToPlayer_Character (Game|GetPlayerCharacter 0)))
  (Variables|Default|SetPlayer%20Ref _asplayer_character))

(fn ConstructionScript)