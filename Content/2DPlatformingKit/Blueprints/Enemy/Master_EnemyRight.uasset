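; Master_EnemyRight is a 2D platformer enemy that patrols between PointA and PointB using InterpToMovement, built in the construction script.
; Each reversal alternates the flipbook's rotation to flip the sprite.
; Trigger overlap damages Player_Character and launches it along the sweep normal's X for knockback.
; Its damage event overwrites HP and destroys it below zero, while Tick updates a widget HP bar that appears after the first hit.
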(event OnComponentBeginOverlap(Trigger)
  (params (OverlappedComponent :type Primitive%20Component%20Object%20Reference) (OtherActor :type Actor%20Object%20Reference) (OtherComp :type Primitive%20Component%20Object%20Reference) (OtherBodyIndex :type Integer) (bFromSweep :type Boolean) (SweepResult :type Hit%20Result%20Structure%20%28by%20ref%29))
  ;[1 1 1] Damage the playing on overlap and Knock Back
  (Utilities|FlowControl|Sequence
    (:then_0
      (bind _asplayer_character (Utilities|Casting|CastToPlayer_Character OtherActor))
      (Default|Damge _asplayer_character (- (Variables|/Game/2DPlatformingKit/Blueprints/Player/Player_Character.Player_Character_C|GetPlayer%20HP _asplayer_character) (Variables|Default|GetDamage))))
    (:then_1
      (Character|LaunchCharacter _asplayer_character (Math|Vector|MakeVector (* (.x (.Normal (Collision|BreakHitResult SweepResult))) (Variables|Default|GetKnockBack%20-X)) 0.0 0.0) false false))))

(event OnInterptoReverse(InterpToMovement)
  (params (ImpactResult :type Hit%20Result%20Structure%20%28by%20ref%29) (Time :type Float%20%28single-precision%29))
  (bind _paperflipbook (Variables|Default|GetPaperFlipbook))
  ;[1 1 1] Flip's Sprite based on direction
  (Utilities|FlowControl|FlipFlop
    (:A
      (Transformation|SetWorldRotation _paperflipbook "0,0.000000, 0" false false))
    (:B
      (Transformation|SetWorldRotation _paperflipbook "0,180.000000, 0" false false))))

(event Custom|Damge
  (params (HP :type Float%20%28single-precision%29))
  ;[1 1 1] Damage Enemy
  (bind _output_get (Variables|Default|SetHP HP))
  (Variables|Default|SetTaken%20Damage true)
  (if (< _output_get 0.0)
    (Actor|DestroyActor)))

(event EventTick
  (params (DeltaSeconds :type Float%20%28single-precision%29))
  (bind _hp_bar (Variables|Default|GetHP%20Bar))
  ;[1 1 1] HP bar Code
  (Utilities|FlowControl|Sequence
    (:then_0
      (|HPBarCode))
    (:then_1
      (if (Variables|Default|GetTaken%20Damage)
        (Rendering|SetVisibility _hp_bar true false)
        (else
          (Rendering|SetVisibility _hp_bar false false))))))

(fn ConstructionScript
  (Variables|/Script/Engine.InterpToMovementComponent|SetControlPoints (Variables|Default|GetInterpToMovement) (Utilities|Array|MakeArray (Utilities|Struct|MakeInterpControlPoint (Variables|Default|GetPoint%20A%20) true) (Utilities|Struct|MakeInterpControlPoint (Variables|Default|GetPoint%20B) true))))