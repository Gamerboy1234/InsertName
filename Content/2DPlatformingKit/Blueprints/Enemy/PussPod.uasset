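; PussPod is a 2D platformer enemy that lies idle until the player enters its aggro zone, then turns into a damaging hazard.
; A one-time delayed sequence plays an eye animation, swaps to a moving flipbook, then shows the final sprite and enables the damage zone's collision.
; Hits on that zone damage the player and launch them horizontally along the hit normal.
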(event OnComponentBeginOverlap(AgroZone)
  (params (OverlappedComponent :type Primitive%20Component%20Object%20Reference) (OtherActor :type Actor%20Object%20Reference) (OtherComp :type Primitive%20Component%20Object%20Reference) (OtherBodyIndex :type Integer) (bFromSweep :type Boolean) (SweepResult :type Hit%20Result%20Structure%20%28by%20ref%29))
  (bind _asplayer_character (Utilities|Casting|CastToPlayer_Character OtherActor))
  (Variables|Default|SetPlayer%20Ref _asplayer_character)
  (if (not (Variables|Default|GetAggro?))
    (Sprite|SetFlipbook (Variables|Default|GetIdle%20FlipBook) (Variables|Default|GetEye%20Animation))
    (Variables|Default|SetAggro? true)
    (Utilities|FlowControl|Delay (Variables|Default|GetBlink%20Delay))
    (Utilities|FlowControl|Delay (Variables|Default|GetMovment%20Delay))
    (Rendering|SetVisibility (Variables|Default|GetIdle%20FlipBook) false false)
    (Rendering|SetVisibility (Variables|Default|GetMovement%20FlipBook) true false)
    (Sprite|SetFlipbook (Variables|Default|GetMovement%20FlipBook) (Variables|Default|GetMoving%20Animation))
    (Utilities|FlowControl|Delay (Variables|Default|GetAttack%20Delay))
    (Rendering|SetVisibility (Variables|Default|GetMovement%20FlipBook) false false)
    (Rendering|SetVisibility (Variables|Default|GetSprite) true false)
    (Collision|SetCollisionEnabled (Variables|Default|GetDamage%20Zone) "QueryAndPhysics")))

(event OnComponentHit(DamageZone)
  (params (HitComponent :type Primitive%20Component%20Object%20Reference) (OtherActor :type Actor%20Object%20Reference) (OtherComp :type Primitive%20Component%20Object%20Reference) (NormalImpulse :type Vector :default "0, 0, 0") (Hit :type Hit%20Result%20Structure%20%28by%20ref%29))
  (bind _asplayer_character (Utilities|Casting|CastToPlayer_Character OtherActor))
  (bind _output_get (Variables|Default|SetPlayer%20Ref _asplayer_character))
  (Default|Damage _output_get (- (Variables|/Game/2DPlatformingKit/Blueprints/Player/Player_Character.Player_Character_C|GetPlayer%20HP (Variables|Default|GetPlayer%20Ref)) (Variables|Damage|GetDamage%20Amount)) (Variables|Damage|GetDamage%20Amount))
  (Character|LaunchCharacter (Variables|Default|GetPlayer%20Ref) (Math|Vector|MakeVector (* (.x (.Normal (Collision|BreakHitResult Hit))) (Variables|Damage|GetKnockback%20X)) 0.0 0.0) false false))

(event EventBeginPlay
  (Rendering|SetVisibility (Variables|Default|GetSprite) false false)
  (Rendering|SetVisibility (Variables|Default|GetMovement%20FlipBook) false false)
  (Collision|SetCollisionEnabled (Variables|Default|GetDamage%20Zone) "NoCollision"))

(fn ConstructionScript)