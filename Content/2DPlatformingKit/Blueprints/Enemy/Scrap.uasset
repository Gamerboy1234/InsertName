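; Scrap pickup in the 2D platforming kit that adds scrap to the player character on overlap, then destroys itself.
; BeginPlay sets its lifespan and rolls a random amount, though the pickup grants ScrapToAdd rather than that roll.
; Tick applies a blinking sprite material when the configured lifespan variable is under two seconds, without counting down the remaining time.
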(event OnComponentBeginOverlap(Trigger)
  (params (OverlappedComponent :type Primitive%20Component%20Object%20Reference) (OtherActor :type Actor%20Object%20Reference) (OtherComp :type Primitive%20Component%20Object%20Reference) (OtherBodyIndex :type Integer) (bFromSweep :type Boolean) (SweepResult :type Hit%20Result%20Structure%20%28by%20ref%29))
  (bind _asplayer_character (Utilities|Casting|CastToPlayer_Character OtherActor))
  (bind _output_get (Variables|Default|SetPlayer%20Ref _asplayer_character))
  (Default|AddScrap _output_get (Variables|Default|GetScrap%20to%20add))
  (Actor|DestroyActor))

(event EventTick
  (params (DeltaSeconds :type Float%20%28single-precision%29))
  (if (< (Variables|Default|GetObject%20Live%20Span) 2.0)
    (Rendering|Material|SetMaterial (Variables|Default|GetPaperSprite) 0 "/Game/2DPlatformingKit/Blueprints/Inventory/Blueprints/ItemClasses/Spells/Tecromancer/Mats/BlinkingScrap.BlinkingScrap")))

(event EventBeginPlay
  (Variables|Default|SetRan%20Amount (Math|Random|RandomIntegerinRange (Variables|Default|GetMin%20Amount) (Variables|Default|GetMax%20Amount)))
  (Actor|SetLifeSpan (Variables|Default|GetObject%20Live%20Span)))

(fn ConstructionScript)