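; Corrupted enemy for the 2D platforming kit that turns aggressive when short line traces to either side hit the player.
; Damage updates HP, spawns floating text and briefly shows an HP bar; death disables collision and despawns after a delay.
; A looping timer applies damage over time with an attached effect actor.
; DamageCheck lets a Warden player end that effect early, turning remaining ticks into boosted damage.
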(event Custom|Damage%20Over%20Time
  (bind _damage_amount (Variables|Default|GetDamage%20Amount))
  ;[1 1 1] Damage Over time
  (if (not (Variables|Default|GetIs%20Dead?))
    (CallFunction|Damge (- (Variables|Default|GetCurrent%20HP) _damage_amount) _damage_amount)
    (bind _result (Math|Float|DecrementFloat (Variables|Default|GetTick's%20Left))
      (:%20%20
        (if (<= _result 0.0)
          (Utilities|Time|ClearandInvalidateTimerbyHandle (Variables|Default|GetEvent%20Timer))
          (Variables|Default|SetTaken%20Damage%20over%20Time? false)
          (Utilities|IsValid (Variables|Default|GetDamage%20Over%20Time%20Actor)
            (:Is%20Valid
              (Actor|DestroyActor (Variables|Default|GetDamage%20Over%20Time%20Actor)))))))
    (else
      (Utilities|Time|ClearandInvalidateTimerbyHandle (Variables|Default|GetEvent%20Timer))
      (Variables|Default|SetTaken%20Damage%20over%20Time? false)
      (Utilities|IsValid (Variables|Default|GetDamage%20Over%20Time%20Actor)
        (:Is%20Valid
          (Actor|DestroyActor (Variables|Default|GetDamage%20Over%20Time%20Actor)))))))

(event Custom|Damge
  (params (HP%20to%20Subtract :type Float%20%28single-precision%29) (Damage%20Amount :type Float%20%28single-precision%29))
  ;[1 1 1] Damage Enemy
  (Variables|Default|SetCurrent%20HP HP%20to%20Subtract)
  (bind _returnvalue (UserInterface|CreateWidget "/Game/2DPlatformingKit/Widgets/Player_Widgets/Floating_Text.Floating_Text_C" 0 Damage%20Amount self))
  (UserInterface|Viewport|AddtoViewport _returnvalue 0)
  (Variables|Default|SetTaken%20Damage true)
  (if (< (Variables|Default|GetCurrent%20HP) 1.0)
    (Variables|Default|SetIs%20Dead? true)
    (Variables|Default|SetTaken%20Damage false)
    (Variables|/Game/2DPlatformingKit/Blueprints/Player/Player_Character.Player_Character_C|SetIs%20in%20Combat? (Variables|Default|GetPlayer%20Ref) false)
    (Variables|Default|Setag false)
    (Collision|SetActorEnableCollision false)
    (Utilities|FlowControl|Delay (Variables|Default|GetDespawn%20Delay))
    (Actor|DestroyActor)))

(event Custom|Start%20Damage%20Over%20Time
  (params (Length :type Float%20%28single-precision%29) (Damage :type Float%20%28single-precision%29) (Attached%20Fire :type Actor%20Object%20Reference) (Occurrences :type Float%20%28single-precision%29))
  ;[1 1 1] Damage Over time
  (Variables|Default|SetDamage%20Amount Damage)
  (Variables|Default|SetTick's%20Left Length)
  (Variables|Default|SetTaken%20Damage%20over%20Time? true)
  (Variables|Default|SetDamage%20Over%20Time%20Actor Attached%20Fire)
  (bind _returnvalue (Utilities|Time|SetTimerbyEvent (delegate Custom|Damage%20Over%20Time) Occurrences true))
  (Variables|Default|SetEvent%20Timer _returnvalue))

(event Custom|Dead
  ;[1 1 1] Damage Enemy
  (Variables|Default|SetIs%20Dead? true)
  (Variables|Default|SetTaken%20Damage false)
  (Variables|/Game/2DPlatformingKit/Blueprints/Player/Player_Character.Player_Character_C|SetIs%20in%20Combat? (Variables|Default|GetPlayer%20Ref) false)
  (Variables|Default|Setag false)
  (Collision|SetActorEnableCollision false)
  (Utilities|FlowControl|Delay (Variables|Default|GetDespawn%20Delay))
  (Actor|DestroyActor))

(event EventBeginPlay
  ;[1 1 1] Get Player Character
  (bind _asplayer_character (Utilities|Casting|CastToPlayer_Character (Game|GetPlayerCharacter 0)))
  (Variables|Default|SetPlayer%20Ref _asplayer_character)
  (Variables|Default|SetDefault%20Vecity (Variables|Default|Getvelocity)))

(event EventTick
  (params (DeltaSeconds :type Float%20%28single-precision%29))
  (bind _returnvalue (Transformation|GetActorLocation))
  (bind _returnvalue_2 (Transformation|GetActorLocation))
  (bind _hp_bar (Variables|Default|GetHP%20Bar))
  ;[1 1 1] Look for player
  (Utilities|FlowControl|Sequence
    (:then_0
      (bind _outhit (Collision|LineTraceByChannel _returnvalue_2 (+ _returnvalue_2 "-100.000000, 0, 0") "TraceTypeQuery1" false 0 "None"))
      (if (== (.HitActor (Collision|BreakHitResult _outhit)) (Game|GetPlayerCharacter 0))
        (Variables|Default|Setag true)))
    (:then_1
      (bind _outhit_2 (Collision|LineTraceByChannel _returnvalue (+ _returnvalue "100.000000, 0, 0") "TraceTypeQuery1" false 0 "None"))
      (if (== (.HitActor (Collision|BreakHitResult _outhit_2)) (Game|GetPlayerCharacter 0))
        (Variables|Default|Setag true)))
    (:then_2
      ;[1 1 1] HP Bar Code
      (if (Variables|Default|GetTaken%20Damage)
        (Rendering|SetVisibility _hp_bar true false)
        (Utilities|FlowControl|Delay 3.0)
        (Rendering|SetVisibility (Variables|Default|GetHP%20Bar) false false)
        (Variables|Default|SetTaken%20Damage false)
        (else
          (Rendering|SetVisibility _hp_bar false false)))
      (bind _asenemy_hpbar (Utilities|Casting|CastToEnemy_HPBar (UserInterface|GetUserWidgetObject (Variables|Default|GetHP%20Bar))))
      (Progress|SetPercent (Variables|/Game/2DPlatformingKit/Widgets/Enemy_Widgets/Enemy_HPBar.Enemy_HPBar_C|GetHPBar _asenemy_hpbar) (/ (Variables|Default|GetCurrent%20HP) (Variables|Default|GetMax%20HP))))))

(fn ConstructionScript)

(fn DamageCheck
  (params (Damage :type Float%20%28single-precision%29))
  (bind _tick_s_left (Variables|Default|GetTick's%20Left))
  (LocalVariables|SetLocal%20Damage Damage)
  (if (and (Variables|Default|GetTaken%20Damage%20over%20Time?) (Variables|/Game/2DPlatformingKit/Blueprints/Player/Player_Character.Player_Character_C|GetIs%20Warden? (Variables|Default|GetPlayer%20Ref)))
    (Utilities|Time|ClearandInvalidateTimerbyHandle (Variables|Default|GetEvent%20Timer))
    (Variables|Default|SetTaken%20Damage%20over%20Time? false)
    (Utilities|IsValid (Variables|Default|GetDamage%20Over%20Time%20Actor)
      (:Is%20Valid
        (Actor|DestroyActor (Variables|Default|GetDamage%20Over%20Time%20Actor)))
      (:Is%20Not%20Valid
        _))
    (Development|PrintString (Utilities|String|ToString(Text) (Utilities|Text|FormatText "Ticks Left: {ticks}" _tick_s_left)))
    (Development|PrintString (Utilities|String|ToString(Text) (Utilities|Text|FormatText "Damage: {ticks}" (Class|DamageIncreass|IncreaseDamage _tick_s_left (LocalVariables|GetLocal%20Damage)))))
    (CallFunction|Damge (- (Variables|Default|GetCurrent%20HP) (Class|DamageIncreass|IncreaseDamage _tick_s_left (LocalVariables|GetLocal%20Damage))) (Class|DamageIncreass|IncreaseDamage _tick_s_left (LocalVariables|GetLocal%20Damage)))
    (else
      (return false))))