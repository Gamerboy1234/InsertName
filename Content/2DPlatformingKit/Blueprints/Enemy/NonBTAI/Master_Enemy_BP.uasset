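; Base 2D enemy without a behavior tree that patrols, shoots the player and respawns after death.
; InterpToMovement runs the two-point patrol with random pauses; the attack routine uses range and line-trace checks to halt it and fire bullets.
; It handles contact knockback, stun and damage over time, which Warden players consume for damage or healing.
; Death drops scrap for Engineers, then hides the enemy far below until respawn instead of destroying it.
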(event OnComponentHit(Trigger)
  (params (HitComponent :type Primitive%20Component%20Object%20Reference) (OtherActor :type Actor%20Object%20Reference) (OtherComp :type Primitive%20Component%20Object%20Reference) (NormalImpulse :type Vector :default "0, 0, 0") (Hit :type Hit%20Result%20Structure%20%28by%20ref%29))
  ;[1 1 1] Knockback on overlap
  (if (Variables|Movement|GetCan%20KnockBack?)
    (bind _asplayer_character (Utilities|Casting|CastToPlayer_Character OtherActor))
    (if (not (Variables|Default|GetIs%20Dead?))
      (Character|LaunchCharacter _asplayer_character (Math|Vector|MakeVector (* (.x (.Normal (Collision|BreakHitResult Hit))) (Variables|Movement|GetKnockBack%20-X)) 0.0 0.0) false false)
      (Utilities|DamagePlayer))))

(event OnInterptoReverse(InterpToMovement)
  (params (ImpactResult :type Hit%20Result%20Structure%20%28by%20ref%29) (Time :type Float%20%28single-precision%29))
  (bind _gun_front (Variables|Default|GetGun%20Front))
  (bind _paperflipbook (Variables|Default|GetPaperFlipbook))
  ;[1 1 1] Flip's Sprite based on direction
  (if (not (Variables|Default|GetPlayer%20In%20Agrro%20Zone))
    (Utilities|FlowControl|FlipFlop
      (:A
        (Utilities|GunVisablityFront)
        (Transformation|SetWorldRotation _paperflipbook (Variables|Movement|GetRotator%201) false false)
        (Transformation|SetWorldRotation _gun_front (Variables|Movement|GetGun%20Rot%202) false false)
        (if (Variables|Movement|GetWant%20to%20Pause%20Movement?)
          (Utilities|RandomInt)
          (Utilities|PauseMovement)))
      (:B
        (Utilities|GunVisablityBack)
        (Transformation|SetWorldRotation _paperflipbook (Variables|Movement|GetRotator%202) false false)
        (Transformation|SetWorldRotation _gun_front (Variables|Movement|GetGun%20Rot%201) false false)
        (if (Variables|Movement|GetWant%20to%20Pause%20Movement?)
          (Utilities|RandomInt)
          (Utilities|PauseMovement))))))

(event Custom|BasIc%20Attack
  ;[1 1 1] HP bar Code/Attack Code
  (|AttackCodeBasic))

(event Custom|Damage%20Over%20Time
  (bind _damage_amount (Variables|Default|GetDamage%20Amount))
  ;[1 1 1] Damage over time
  (if (not (Variables|Default|GetIs%20Dead?))
    (CallFunction|Damge (- (Variables|HPValues|GetCurrent%20HP) _damage_amount) _damage_amount)
    (Math|Float|DecrementFloat (Variables|Default|GetTick's%20Left)
      (:%20%20
        (if (<= (Variables|Default|GetTick's%20Left) 0.0)
          (Utilities|Time|ClearandInvalidateTimerbyHandle (Variables|Default|GetEvent%20Timer))
          (Variables|Default|SetTaken%20Damage%20over%20Time? false)
          (Utilities|IsValid (Variables|Default|GetDamage%20Over%20Time%20Actor)
            (:Is%20Valid
              (Actor|DestroyActor (Variables|Default|GetDamage%20Over%20Time%20Actor)))))))
    (else
      (Utilities|Time|ClearandInvalidateTimerbyHandle (Variables|Default|GetEvent%20Timer))
      (Variables|Default|SetTaken%20Damage%20over%20Time? false)
      (Utilities|IsValid (Variables|Default|GetDamage%20Over%20Time%20Actor)
        (:Is%20Valid
          (Actor|DestroyActor (Variables|Default|GetDamage%20Over%20Time%20Actor)))))))

(event Custom|Damge
  (params (HP%20to%20Subtract :type Float%20%28single-precision%29) (Damage%20Amount :type Float%20%28single-precision%29))
  (bind _returnvalue (Transformation|GetActorLocation))
  (bind _returnvalue_2 (Transformation|GetActorLocation))
  ;[1 1 1] Damage Enemy
  (Variables|HPValues|SetCurrent%20HP HP%20to%20Subtract)
  (bind _returnvalue_3 (UserInterface|CreateWidget "/Game/2DPlatformingKit/Widgets/Player_Widgets/Floating_Text.Floating_Text_C" 0 Damage%20Amount self))
  (UserInterface|Viewport|AddtoViewport _returnvalue_3 0)
  (Variables|Default|SetTaken%20Damage true)
  (if (< (Variables|HPValues|GetCurrent%20HP) 1.0)
    (Variables|Default|SetIs%20Dead? true)
    (Development|SetHiddeninGame (Variables|Default|GetTarget%20Marker%20Sprite) true false)
    (Sprite|SetFlipbook (Variables|Default|GetPaperFlipbook) (Variables|Animation|GetFlipbook%20Death))
    (Variables|Default|SetTaken%20Damage false)
    (Variables|/Game/2DPlatformingKit/Blueprints/Player/Player_Character.Player_Character_C|SetIs%20in%20Combat? (Variables|Default|GetPlayer%20Ref) false)
    (Components|Movement|StopMovementImmediately (Variables|Default|GetInterpToMovement))
    (Collision|SetActorEnableCollision false)
    (Utilities|SpawnDrops)
    (Utilities|FlowControl|Delay (Variables|Spawning|GetDespawn%20Delay))
    (Transformation|SetWorldLocation (Variables|Default|GetScene) (Math|Vector|MakeVector (.x _returnvalue_2) (.y _returnvalue_2) -3e+04) false true)
    ;[1 1 1] Respawn
    (Utilities|FlowControl|Delay (Variables|Spawning|GetRespawn%20Time))
    (Transformation|SetWorldLocation (Variables|Default|GetScene) (Math|Vector|MakeVector (.x _returnvalue) (.y _returnvalue) (.z (Variables|Spawning|GetRespawn%20Point))) false true)
    (Sprite|SetFlipbook (Variables|Default|GetPaperFlipbook) (Variables|Animation|GetFlipBook%20Walking))
    (Class|InterptoMovementComponent|RestartMovement (Variables|Default|GetInterpToMovement) 1.0)
    (Variables|HPValues|SetCurrent%20HP (Variables|HPValues|GetMaxHP))
    (Variables|Default|SetIs%20Dead? false)
    (Collision|SetActorEnableCollision true)
    (Rendering|SetVisibility (Variables|Default|GetGun%20Front) true false)))

(event Custom|Start%20Damage%20Over%20Time%20Slot%201
  (params (Damage :type Float%20%28single-precision%29) (Attached%20Actor :type Actor%20Object%20Reference) (Occurrences :type Float%20%28single-precision%29) (Tick :type Float%20%28single-precision%29))
  ;[1 1 1] Damage over time
  (Variables|Default|SetTaken%20Damage%20over%20Time? true)
  (Variables|Default|SetDamage%20Amount Damage)
  (bind _output_get (Variables|Default|SetTick's%20Left Tick))
  (Variables|Default|SetMax%20Damage%20Tick _output_get)
  (Variables|Default|SetDamage%20Over%20Time%20Actor Attached%20Actor)
  (bind _returnvalue (Utilities|Time|SetTimerbyEvent (delegate Custom|Damage%20Over%20Time) Occurrences true))
  (Variables|Default|SetEvent%20Timer _returnvalue))

(event Custom|Stun
  (params (Stun%20Duration :type Float%20%28single-precision%29))
  ;[1 1 1] Stun Debuff
  (Variables|Default|SetStun%20Duration Stun%20Duration)
  (Variables|Default|SetIs%20Stunned? true)
  (Components|Tick|SetComponentTickEnabled (Variables|Default|GetInterpToMovement) false)
  (Utilities|FlowControl|Delay (Variables|Default|GetStun%20Duration))
  (Components|Tick|SetComponentTickEnabled (Variables|Default|GetInterpToMovement) true)
  (Variables|Default|SetIs%20Stunned? false))

(event Custom|HPBar%20Code
  ;[1 1 1] HP bar Code/Attack Code
  (Utilities|FlowControl|Sequence
    (:then_0
      (|HPBarCode))
    (:then_1
      (|HPBarVisablity))))

(event Custom|Dead
  (bind _returnvalue (Transformation|GetActorLocation))
  (bind _returnvalue_2 (Transformation|GetActorLocation))
  ;[1 1 1] Damage Enemy
  (Variables|Default|SetIs%20Dead? true)
  (Development|SetHiddeninGame (Variables|Default|GetTarget%20Marker%20Sprite) true false)
  (Sprite|SetFlipbook (Variables|Default|GetPaperFlipbook) (Variables|Animation|GetFlipbook%20Death))
  (Variables|Default|SetTaken%20Damage false)
  (Variables|/Game/2DPlatformingKit/Blueprints/Player/Player_Character.Player_Character_C|SetIs%20in%20Combat? (Variables|Default|GetPlayer%20Ref) false)
  (Components|Movement|StopMovementImmediately (Variables|Default|GetInterpToMovement))
  (Collision|SetActorEnableCollision false)
  (Utilities|SpawnDrops)
  (Utilities|FlowControl|Delay (Variables|Spawning|GetDespawn%20Delay))
  (Transformation|SetWorldLocation (Variables|Default|GetScene) (Math|Vector|MakeVector (.x _returnvalue_2) (.y _returnvalue_2) -3e+04) false true)
  ;[1 1 1] Respawn
  (Utilities|FlowControl|Delay (Variables|Spawning|GetRespawn%20Time))
  (Transformation|SetWorldLocation (Variables|Default|GetScene) (Math|Vector|MakeVector (.x _returnvalue) (.y _returnvalue) (.z (Variables|Spawning|GetRespawn%20Point))) false true)
  (Sprite|SetFlipbook (Variables|Default|GetPaperFlipbook) (Variables|Animation|GetFlipBook%20Walking))
  (Class|InterptoMovementComponent|RestartMovement (Variables|Default|GetInterpToMovement) 1.0)
  (Variables|HPValues|SetCurrent%20HP (Variables|HPValues|GetMaxHP))
  (Variables|Default|SetIs%20Dead? false)
  (Collision|SetActorEnableCollision true)
  (Rendering|SetVisibility (Variables|Default|GetGun%20Front) true false))

(event EventBeginPlay
  (bind _asplayer_character (Utilities|Casting|CastToPlayer_Character (Game|GetPlayerCharacter 0)))
  (Variables|Default|SetPlayer%20Ref _asplayer_character)
  (Variables|/Script/Engine.InterpToMovementComponent|SetDuration (Variables|Default|GetInterpToMovement) (Variables|Movement|GetDefault%20Duration))
  ;[1 1 1] Event BeginPlay set walking flipbook
  (CallFunction|CanWalk (Variables|Movement|GetCan%20Walk?))
  (if (Math|Rotator|Equal(Rotator) (Transformation|GetActorRotation (Variables|Default|GetPlayer%20Ref)) "0,180.000000, 0" 0.0001)
    (Utilities|GunVisablityBack)
    (else
      (Utilities|GunVisablityFront))))

(fn ConstructionScript
  (Variables|/Script/Engine.InterpToMovementComponent|SetControlPoints (Variables|Default|GetInterpToMovement) (Utilities|Array|MakeArray (Utilities|Struct|MakeInterpControlPoint (Variables|Movement|GetPoint%20A%20) true) (Utilities|Struct|MakeInterpControlPoint (Variables|Movement|GetPoint%20B) true)))
  (Variables|/Script/Engine.InterpToMovementComponent|SetDuration (Variables|Default|GetInterpToMovement) (Variables|Movement|GetAnimation%20Speed)))

(fn CanWalk
  (params (Can%20Walk? :type Boolean))
  (if Can%20Walk?
    ;[1 1 1] Is Walking
    (Sprite|SetFlipbook (Variables|Default|GetPaperFlipbook) (Variables|Animation|GetFlipBook%20Walking))
    (Rendering|Components|Sprite|SetSprite (Variables|Default|GetGun%20Front) (Variables|Animation|GetGun%20Sprite))
    (Rendering|Components|Sprite|SetSprite (Variables|Default|GetGun%20Back) (Variables|Animation|GetGun%20Sprite))
    (bind _asplayer_character (Utilities|Casting|CastToPlayer_Character (Game|GetPlayerCharacter 0)))
    (Variables|Default|SetPlayer%20Ref _asplayer_character)
    (Components|Tick|SetComponentTickEnabled (Variables|Default|GetInterpToMovement) true)
    (else
      ;[1 1 1] Can't Walk
      (Sprite|SetFlipbook (Variables|Default|GetPaperFlipbook) (Variables|Animation|GetFlipBook%20Idle))
      (Rendering|Components|Sprite|SetSprite (Variables|Default|GetGun%20Front) (Variables|Animation|GetGun%20Sprite))
      (Rendering|Components|Sprite|SetSprite (Variables|Default|GetGun%20Back) (Variables|Animation|GetGun%20Sprite))
      (bind _asplayer_character_2 (Utilities|Casting|CastToPlayer_Character (Game|GetPlayerCharacter 0)))
      (Variables|Default|SetPlayer%20Ref _asplayer_character_2)
      (Components|Tick|SetComponentTickEnabled (Variables|Default|GetInterpToMovement) false))))

(fn DamageCheck
  (params (Gun%20Damage :type Float%20%28single-precision%29) (Heal? :type Boolean) (Damage? :type Boolean))
  (LocalVariables|SetLocal%20Heal%20 Heal?)
  (LocalVariables|SetLocal%20Damage Damage?)
  (LocalVariables|SetLocal%20Gun%20Damage Gun%20Damage)
  (if (and (Variables|Default|GetTaken%20Damage%20over%20Time?) (Variables|/Game/2DPlatformingKit/Blueprints/Player/Player_Character.Player_Character_C|GetIs%20Warden? (Variables|Default|GetPlayer%20Ref)))
    (if (LocalVariables|GetLocal%20Damage)
      (Utilities|Time|ClearandInvalidateTimerbyHandle (Variables|Default|GetEvent%20Timer))
      (Variables|Default|SetTaken%20Damage%20over%20Time? false)
      (Utilities|IsValid (Variables|Default|GetDamage%20Over%20Time%20Actor)
        (:Is%20Valid
          (Actor|DestroyActor (Variables|Default|GetDamage%20Over%20Time%20Actor)))
        (:Is%20Not%20Valid
          _))
      (CallFunction|Damge (- (Variables|HPValues|GetCurrent%20HP) (Class|DamageIncreass|IncreaseDamage (Variables|Default|GetTick's%20Left) (LocalVariables|GetLocal%20Gun%20Damage))) (Class|DamageIncreass|IncreaseDamage (Variables|Default|GetTick's%20Left) (LocalVariables|GetLocal%20Gun%20Damage)))
      (return true)
      (elif (LocalVariables|GetLocal%20Heal%20)
        (Utilities|Time|ClearandInvalidateTimerbyHandle (Variables|Default|GetEvent%20Timer))
        (Variables|Default|SetTaken%20Damage%20over%20Time? false)
        (Utilities|IsValid (Variables|Default|GetDamage%20Over%20Time%20Actor)
          (:Is%20Valid
            (Actor|DestroyActor (Variables|Default|GetDamage%20Over%20Time%20Actor)))
          (:Is%20Not%20Valid
            _))
        (Default|Heal (Variables|Default|GetPlayer%20Ref) (Variables|Default|GetTick's%20Left))
        (return true)
        (else
          (return false))))
    (else
      (return false))))