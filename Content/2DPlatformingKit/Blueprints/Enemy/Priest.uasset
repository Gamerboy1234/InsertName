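; Priest enemy for the 2D platforming kit that repeatedly throws rocks.
; BeginPlay fires the first throw after a short delay, spawning a Master_Enemy_Bullet at the Direction component's transform.
; That throw sets HasShotOnce, which lets Tick repeat throws through a Delay that paces the fire rate.
; DropBoulder runs once after the first throw and is a stub that only prints a debug string.
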(event Custom|Rock%20Throw
  (Game|SpawnActorfromClass "/Game/2DPlatformingKit/Blueprints/Player/Master_Enemy_Bullet.Master_Enemy_Bullet_C" (Transformation|GetWorldTransform (Variables|Default|GetDirection)) "Undefined" 0 1.0 0)
  (Variables|Default|SetHas%20Shot%20once? true))

(event Custom|Drop%20Boulder
  (Development|PrintString "ATtack"))

(event EventBeginPlay
  (Utilities|FlowControl|Delay 2.0)
  (CallFunction|RockThrow)
  (Utilities|FlowControl|Delay 3.0)
  (CallFunction|DropBoulder))

(event EventTick
  (params (DeltaSeconds :type Float%20%28single-precision%29))
  (if (Variables|Default|GetHas%20Shot%20once?)
    (Utilities|FlowControl|Delay 2.0)
    (CallFunction|RockThrow)))

(fn ConstructionScript)