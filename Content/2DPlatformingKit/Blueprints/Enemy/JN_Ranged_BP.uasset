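; Ranged 2D platformer enemy that throws spears from its arrow component and is destroyed when its HP drops below one.
; Tick throws a spear after a delay at full ammo, also refreshing the briefly shown HP bar on that branch.
; Below full ammo, line traces along positive and negative X look for dropped spears, recording location and turning the enemy.
; Damage stores the passed-in HP and shows floating damage text.
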(event Custom|Damage
  (params (HP%20To%20Subtract :type Float%20%28single-precision%29) (Incoming%20Damage :type Float%20%28single-precision%29))
  (Variables|Default|SetIncoming%20Damage Incoming%20Damage)
  (Variables|Default|SetCurrent%20HP HP%20To%20Subtract)
  (bind _returnvalue (UserInterface|CreateWidget "/Game/2DPlatformingKit/Widgets/Floating_Text.Floating_Text_C" 0 Incoming%20Damage self))
  (UserInterface|Viewport|AddtoViewport _returnvalue 0)
  (Variables|Default|SetTaken%20Damge true)
  (if (< (Variables|Default|GetCurrent%20HP) 1.0)
    (Variables|Default|Setdead true)
    (Variables|Default|SetTaken%20Damge false)
    (Actor|DestroyActor)))

(event EventTick
  (params (DeltaSeconds :type Float%20%28single-precision%29))
  (bind _hpbar (Variables|Default|GetHPBar))
  (if (< (Variables|Default|GetSpearAmmount) (Variables|Default|GetmaxSpearAmount))
    (CallFunction|FindDroppedSpear)
    (else
      (Utilities|FlowControl|Delay 3.0)
      (Math|Integer|DecrementInt (Variables|Default|GetSpearAmmount)
        (:%20%20
          (Game|SpawnActorfromClass "/Game/2DPlatformingKit/Blueprints/Player/E_Spear.E_Spear_C" (Transformation|GetWorldTransform (Variables|Default|GetArrow)) "Undefined" 0 0.5 3e+02 3e+02 5.0 1.0 0)
          (if (Variables|Default|GetTaken%20Damge)
            (Rendering|SetVisibility _hpbar true false)
            (Utilities|FlowControl|Delay 3.0)
            (Rendering|SetVisibility (Variables|Default|GetHPBar) false false)
            (Variables|Default|SetTaken%20Damge false)
            (else
              (Rendering|SetVisibility _hpbar false false)))
          (bind _asenemy_hpbar (Utilities|Casting|CastToEnemy_HPBar (UserInterface|GetUserWidgetObject (Variables|Default|GetHPBar))))
          (Progress|SetPercent (Variables|/Game/2DPlatformingKit/Widgets/Enemy_HPBar.Enemy_HPBar_C|GetHPBar _asenemy_hpbar) (/ (Variables|Default|GetCurrent%20HP) (Variables|Default|GetMax%20HP))))))))

(fn ConstructionScript)

(fn FindDroppedSpear
  (bind _line_1 (Variables|Default|GetLine%201))
  (bind _line_2 (Variables|Default|GetLine%202))
  (bind _returnvalue (Transformation|GetWorldLocation _line_1))
  (bind _returnvalue_2 (Transformation|GetWorldLocation _line_2))
  (Utilities|FlowControl|Sequence
    (:then_0
      (bind _outhit (Collision|LineTraceForObjects _returnvalue (+ _returnvalue "1000.000000,0.000000,0.000000") (Utilities|Array|MakeArray "ObjectTypeQuery9") false 0 "None"))
      (bind _outactors (Actor|GetAllActorsOfClass "/Game/2DPlatformingKit/Blueprints/Player/DroppedSpear_BP.DroppedSpear_BP_C"))
      (bind _array_element (Utilities|Array|ForEachLoopwithBreak _outactors :!label _label)
        (:LoopBody
          (if (== (.HitActor (Collision|BreakHitResult _outhit)) _array_element)
            (goto _label Break)))
        (:Completed
          (bind _output_get (LocalVariables|SetDropped%20Spear (.HitActor (Collision|BreakHitResult _outhit))))
          (Utilities|IsValid _output_get
            (:Is%20Valid
              (Variables|Default|SetSpearLocation (Transformation|GetActorLocation _output_get))
              (Variables|Default|SetSpearFound true)
              (Variables|Default|SetisRight true)
              (Variables|Default|SetisLeft false)
              (Transformation|SetActorRotation "0,180.000000, 0"))))))
    (:then_1
      (bind _outhit_2 (Collision|LineTraceForObjects _returnvalue_2 (+ _returnvalue_2 "-1000.000000,0.000000,0.000000") (Utilities|Array|MakeArray "ObjectTypeQuery9") false 0 "None"))
      (bind _outactors_2 (Actor|GetAllActorsOfClass "/Game/2DPlatformingKit/Blueprints/Player/DroppedSpear_BP.DroppedSpear_BP_C"))
      (bind _array_element_2 (Utilities|Array|ForEachLoopwithBreak _outactors_2 :!label _label_2)
        (:LoopBody
          (if (== (.HitActor (Collision|BreakHitResult _outhit_2)) _array_element_2)
            (goto _label_2 Break)))
        (:Completed
          (bind _output_get_2 (LocalVariables|SetDropped%20Spear (.HitActor (Collision|BreakHitResult _outhit_2))))
          (Utilities|IsValid _output_get_2
            (:Is%20Valid
              (Variables|Default|SetSpearLocation (Transformation|GetActorLocation _output_get_2))
              (Variables|Default|SetSpearFound true)
              (Variables|Default|SetisRight false)
              (Variables|Default|SetisLeft true)
              (Transformation|SetActorRotation "0, 0, 0"))))))))