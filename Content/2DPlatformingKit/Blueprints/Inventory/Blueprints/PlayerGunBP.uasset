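; PlayerGunBP is the player's gun in the 2D platforming kit's inventory, adding cooldown timing and cooldown bar updates after firing.
; When firing ends with the gun on cooldown, it stretches the GunCD timeline to the GunCoolDown duration and restarts it.
; Each timeline update passes playback position and length to UpdateCDBar, and completion calls ResetGunCooldown.
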(event EventOnFireEnd
  (bind _guncd (Variables|Default|GetGunCD))
  ;[1 1 1] Update Gun Cooldown bar
  (if (Class|MasterGun|GetGunonCooldown)
    (Components|Timeline|SetTimelineLength (Variables|Default|GetGunCD) (Variables|Default|GetGunCoolDown))
    (Timeline|GunCD PlayFromStart
      (:Update
        (Class|MasterGun|UpdateCDBar (Components|Timeline|GetPlaybackPosition _guncd) (Components|Timeline|GetTimelineLength _guncd) (Variables|Default|GetGunCoolDown)))
      (:Finished
        (Class|MasterGun|ResetGunCooldown)))))

(fn ConstructionScript)