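; Machine gun item Blueprint for the 2D platforming kit that fires automatically while the Attack input is held.
; Pressing Attack, if the player is not dead, opens a gate that spawns a Bullet_Master at the Arrow transform with damage from the item info.
; A short Delay re-enters the gate to loop the fire until releasing Attack closes it.
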(event Input|ActionEvents|InputActionAttack
  (params (Key :type Key%20Structure))
  (:Pressed
    (if (not (Variables|/Game/2DPlatformingKit/Blueprints/Player/Player_Character.Player_Character_C|GetIs%20Dead (Variables|Default|GetPlayer%20Ref)))
      (Utilities|FlowControl|Sequence
        (:then_0
          (goto _label Open))
        (:then_1
          (Utilities|FlowControl|Gate true :!label _label
            (:Exit
              (Utilities|FlowControl|Sequence
                (:then_0
                  (Game|SpawnActorfromClass "/Game/2DPlatformingKit/Blueprints/Player/Bullet_Master.Bullet_Master_C" (Transformation|GetWorldTransform (Variables|Default|GetArrow)) "Undefined" 0 (.Damage (Utilities|Struct|BreakS_ItemInfo (Variables|Default|GetItem%20Info))) 2.0 0))
                (:then_1
                  (Utilities|FlowControl|Delay 0.2)
                  (goto _label)))))))))
  (:Released
    (goto _label Close)))

(fn ConstructionScript
  (|CallParentFunction))