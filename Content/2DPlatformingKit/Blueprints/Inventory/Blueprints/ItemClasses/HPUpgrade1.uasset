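; HPUpgrade1 is an inventory item in the 2D platforming kit that upgrades the player's health when used.
; On BeginPlay it caches the player character reference.
; When used, it switches the inventory's HP bar from tier 1 to 2 and calls the player's HP upgrade with current HP plus HPToAdd.
; It then removes one from its inventory slot and destroys itself if that succeeds.
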(event EventBeginPlay
  (bind _asplayer_character (Utilities|Casting|CastToPlayer_Character (Game|GetPlayerCharacter 0)))
  (Variables|Default|SetPlayer%20Ref _asplayer_character))

(event EventEventItemUsed
  (bind _player_ref (Variables|Default|GetPlayer%20Ref))
  (Default|HPBar1to2 (Variables|/Game/2DPlatformingKit/Blueprints/Player/Player_Character.Player_Character_C|GetInventory%20Ref (Variables|Default|GetPlayer%20Ref)))
  (Default|HPUpgrade _player_ref (+ (Variables|/Game/2DPlatformingKit/Blueprints/Player/Player_Character.Player_Character_C|GetPlayer%20HP _player_ref) (Variables|Default|GetHP%20To%20Add)))
  (bind _success (Default|RemoveItematIndex (Variables|Default|GetInventory) (Variables|Default|GetIndex) 1))
  (if _success
    (Actor|DestroyActor)))

(fn ConstructionScript
  (|CallParentFunction))