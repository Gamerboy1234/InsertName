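; Player gun item in the inventory system that fires trace-based light attacks and a charged heavy knockback attack.
; The Attack input fires directly, while releasing Weapon Charge picks heavy or light depending on whether the charge delay completed.
; Light fire loops multi-target traces on a fire-rate delay while attack is held, driving a cooldown bar; a single-target variant is also defined.
; Spell mod equip events are empty stubs.
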(event EventBeginPlay
  ;[1 1 1] Setting Default Values
  (|CallParentFunction))

(event EventUnequippedSpellMod
  ;[1 1 1] Spell Mod Effects
)

(event EventFireGun
  ;[1 1 1] Fire gun and setup delay
  (if (Variables|WeaponCharge|GetCan%20Shoot)
    (Utilities|GoThroughMultipleEnimes)))

(event EventEquippedSpellMod
  ;[1 1 1] Spell Mod Effects
)

(event Input|ActionEvents|InputActionAttack
  (params (Key :type Key%20Structure :default "None"))
  ;[1 1 1] Charge weapon to do hevey attack or just do light attack
  (:Pressed
    (Utilities|LightAttack :!label _label))
  (:Released
    (goto _label Released)))

(event Input|ActionEvents|InputActionWeaponCharge
  (params (Key :type Key%20Structure :default "None"))
  ;[1 1 1] Charge weapon to do hevey attack or just do light attack
  (:Pressed
    (Utilities|HeveyorLightAttack :!label _label
      (:Hevey%20Attack%20
        (Utilities|HeveyAttack :!label _label_2))
      (:%20Light%20Attack
        (Utilities|LightAttack :!label _label_3))))
  (:Released
    (Utilities|FlowControl|Sequence
      (:then_0
        (goto _label Released%20))
      (:then_1
        (goto _label_3 Released))
      (:then_2
        (goto _label_2 Released)))))

(fn ConstructionScript
  (|CallParentFunction))