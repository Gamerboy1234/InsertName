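; Base chest armor item class for the 2D platforming kit's inventory.
; When the item is used, it passes itself to EquipChest on the player referenced by its Inventory.
; A successful equip enables input on the item for player controller 0, while a failed one destroys the actor.
; BeginPlay and construction only call the parent class.
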(event EventBeginPlay
  (|CallParentFunction))

(event EventEventItemUsed
  (bind _success_ (Default|EquipChest (Variables|/Game/2DPlatformingKit/Blueprints/Inventory/Blueprints/Inventory_Master.Inventory_Master_C|GetPlayerRef (Variables|Default|GetInventory)) self))
  (if _success_
    (Input|EnableInput (Game|GetPlayerController 0))
    (else
      (Actor|DestroyActor))))

(fn ConstructionScript
  (|CallParentFunction))