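; Inventory item that acts as a med pack crafting recipe, teaching the player to craft it when used.
; On use it adds its RecipeToAdd class to the player inventory's unlocked craftables and refreshes the crafting menu.
; It then removes one of itself from the inventory, shows a learned-recipe screen message, and destroys the actor if removal succeeded.
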(event EventBeginPlay
  (bind _asplayer_character (Utilities|Casting|CastToPlayer_Character (Game|GetPlayerCharacter 0)))
  (Variables|Default|SetPlayer%20Ref _asplayer_character))

(event EventItemUsed
  (bind _player_ref (Variables|Default|GetPlayer%20Ref))
  (bind _inventory_ref (Variables|/Game/2DPlatformingKit/Blueprints/Player/Player_Character.Player_Character_C|GetInventory%20Ref _player_ref))
  (Utilities|Array|Add (Variables|/Game/2DPlatformingKit/Blueprints/Inventory/Blueprints/Inventory_Master.Inventory_Master_C|GetUnlockedCraftableItems (Variables|/Game/2DPlatformingKit/Blueprints/Player/Player_Character.Player_Character_C|GetInventory%20Ref (Variables|Default|GetPlayer%20Ref))) (Variables|Default|GetRecipe%20to%20Add))
  (Default|InitCraftMenu (Variables|/Game/2DPlatformingKit/Widgets/HUD.HUD_C|GetCraftingMenu (Variables|/Game/2DPlatformingKit/Blueprints/Inventory/Blueprints/Inventory_Master.Inventory_Master_C|GetHUD (Variables|/Game/2DPlatformingKit/Blueprints/Player/Player_Character.Player_Character_C|GetInventory%20Ref (Variables|Default|GetPlayer%20Ref)))) _inventory_ref)
  (Default|UpdateCraftMenu _inventory_ref)
  (bind _success (Default|RemoveItematIndex (Variables|/Game/2DPlatformingKit/Blueprints/Player/Player_Character.Player_Character_C|GetInventory%20Ref (Variables|Default|GetPlayer%20Ref)) (Variables|Default|GetIndex) 1 false))
  (Utilities|UIScreenText (Utilities|Text|FormatText "You learned how to craft a {Recipe}" (Utilities|Struct|BreakS_ItemInfo (Utilities|GetClassDefaults (Variables|Default|GetRecipe%20to%20Add)))))
  (if _success
    (Actor|DestroyActor)))

(fn ConstructionScript
  (|CallParentFunction))