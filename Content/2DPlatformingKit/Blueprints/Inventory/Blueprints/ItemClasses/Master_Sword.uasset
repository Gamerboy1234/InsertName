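; Master sword item class for the 2D platforming kit inventory, which equips itself on the player when used.
; On use it calls the player's EquipSword with itself.
; A successful equip enables input on the sword from the first player controller, while a failed one destroys the actor.
; BeginPlay and construction only call their parent logic.
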(event EventBeginPlay
  (|CallParentFunction))

(event EventEventItemUsed
  (bind _success_ (Default|EquipSword (Variables|Default|GetPlayer%20Ref) self))
  (if _success_
    (Input|EnableInput (Game|GetPlayerController 0))
    (else
      (Actor|DestroyActor))))

(fn ConstructionScript
  (|CallParentFunction))