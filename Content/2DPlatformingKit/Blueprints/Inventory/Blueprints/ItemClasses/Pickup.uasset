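; Pickup actor that adds an item to the player's inventory when the player overlaps its trigger.
; On overlap it casts to Player_Character and calls AddItem on its InventoryRef with the configured item class and amount.
; After a successful add, a Rest below zero becomes the new Amount; any other Rest, including a positive leftover, destroys the pickup.
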(event OnComponentBeginOverlap(Trigger)
  (params (OverlappedComponent :type Primitive%20Component%20Object%20Reference) (OtherActor :type Actor%20Object%20Reference) (OtherComp :type Primitive%20Component%20Object%20Reference) (OtherBodyIndex :type Integer) (bFromSweep :type Boolean) (SweepResult :type Hit%20Result%20Structure%20%28by%20ref%29))
  (bind _asplayer_character (Utilities|Casting|CastToPlayer_Character OtherActor))
  (Utilities|IsValid (Variables|/Game/2DPlatformingKit/Blueprints/Player/Player_Character.Player_Character_C|GetInventory%20Ref _asplayer_character)
    (:Is%20Valid
      (bind (_success_ _rest) (Default|AddItem (Variables|/Game/2DPlatformingKit/Blueprints/Player/Player_Character.Player_Character_C|GetInventory%20Ref _asplayer_character) (Variables|Default|GetItem%20to%20Add) (Variables|Default|GetAmount)))
      (if _success_
        (if (< _rest 0)
          (Variables|Default|SetAmount _rest)
          (else
            (Actor|DestroyActor)))))))

(fn ConstructionScript)