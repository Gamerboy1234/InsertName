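; Shotgun weapon item for the 2D platforming kit's inventory, firing a three-pellet spread.
; On the Attack input, while the player is not dead, it spawns three Bullet_Master actors at the transforms of three Arrow components.
; Each bullet takes its damage from the item's info and carries a short despawn delay, limiting the shot's lifetime.
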(event Input|ActionEvents|InputActionAttack
  (params (Key :type Key%20Structure))
  (bind _item_info (Variables|Default|GetItem%20Info))
  (bind _damage (Utilities|Struct|BreakS_ItemInfo _item_info))
  (:Pressed
    (if (not (Variables|/Game/2DPlatformingKit/Blueprints/Player/Player_Character.Player_Character_C|GetIs%20Dead (Variables|Default|GetPlayer%20Ref)))
      (Game|SpawnActorfromClass "/Game/2DPlatformingKit/Blueprints/Player/Bullet_Master.Bullet_Master_C" (Transformation|GetWorldTransform (Variables|Default|GetArrow)) "Undefined" 0 _damage 0.5 0)
      (Game|SpawnActorfromClass "/Game/2DPlatformingKit/Blueprints/Player/Bullet_Master.Bullet_Master_C" (Transformation|GetWorldTransform (Variables|Default|GetArrow1)) "Undefined" 0 _damage 0.5 0)
      (Game|SpawnActorfromClass "/Game/2DPlatformingKit/Blueprints/Player/Bullet_Master.Bullet_Master_C" (Transformation|GetWorldTransform (Variables|Default|GetArrow2)) "Undefined" 0 _damage 0.5 0))))

(fn ConstructionScript
  (|CallParentFunction))