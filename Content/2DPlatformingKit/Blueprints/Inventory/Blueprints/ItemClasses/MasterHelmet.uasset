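; MasterHelmet is the helmet item class for the 2D platforming kit's inventory, handling what happens when a helmet item is used.
; On BeginPlay it caches a reference to the player character.
; The ItemUsed event passes the helmet to EquipHelmet through the inventory's player reference, enabling input on a true result and destroying the actor on a false one.
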(event EventEventItemUsed
  (bind _success_ (Default|EquipHelmet (Variables|/Game/2DPlatformingKit/Blueprints/Inventory/Blueprints/Inventory_Master.Inventory_Master_C|GetPlayerRef (Variables|Default|GetInventory)) self))
  (if _success_
    (Input|EnableInput (Game|GetPlayerController 0))
    (else
      (Actor|DestroyActor))))

(event EventBeginPlay
  (bind _asplayer_character (Utilities|Casting|CastToPlayer_Character (Game|GetPlayerCharacter 0)))
  (Variables|Default|SetPlayer%20Ref _asplayer_character))

(fn ConstructionScript
  (|CallParentFunction))