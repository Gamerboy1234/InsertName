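; Random pickup for the 2D platforming kit's inventory that chooses which item it grants when play begins.
; A random roll sets ItemToAdd to a health upgrade, Dirt, Drone, Terriable_Gun or Data_Crystal, or to None on the remaining outcome.
; A second random Select on return is redundant, as all its wired options read ItemToAdd.
; Construction defers to the parent class.
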(event EventBeginPlay
  (CallFunction|RamdomPickup))

(fn ConstructionScript
  (|CallParentFunction))

(fn RamdomPickup
  (switch int (Math|Random|RandomIntegerinRange 0 5)
    (:Default
      (Variables|Default|SetItem%20to%20Add 0))
    (:0
      (bind _output_get (Variables|Default|SetItem%20to%20Add "/Game/2DPlatformingKit/Blueprints/Inventory/Blueprints/ItemClasses/HPUpgrade1.HPUpgrade1_C"))
      (return (Utilities|Select :Index (Math|Random|RandomIntegerinRange 0 5) :Option%200 _output_get :Option%201 (stale _output_get_2) :Option%202 (stale _output_get_3) :Option%203 (stale _output_get_4) :Option%204 (stale _output_get_5))))
    (:1
      (bind _output_get_2 (Variables|Default|SetItem%20to%20Add "/Game/2DPlatformingKit/Blueprints/Inventory/Blueprints/ItemClasses/Dirt.Dirt_C"))
      (return (Utilities|Select :Index (Math|Random|RandomIntegerinRange 0 5) :Option%200 _output_get :Option%201 _output_get_2 :Option%202 (stale _output_get_3) :Option%203 (stale _output_get_4) :Option%204 (stale _output_get_5))))
    (:2
      (bind _output_get_3 (Variables|Default|SetItem%20to%20Add "/Game/2DPlatformingKit/Blueprints/Inventory/Blueprints/ItemClasses/Drone.Drone_C"))
      (return (Utilities|Select :Index (Math|Random|RandomIntegerinRange 0 5) :Option%200 _output_get :Option%201 _output_get_2 :Option%202 _output_get_3 :Option%203 (stale _output_get_4) :Option%204 (stale _output_get_5))))
    (:3
      (bind _output_get_4 (Variables|Default|SetItem%20to%20Add "/Game/2DPlatformingKit/Blueprints/Inventory/Blueprints/ItemClasses/Terriable_Gun.Terriable_Gun_C"))
      (return (Utilities|Select :Index (Math|Random|RandomIntegerinRange 0 5) :Option%200 _output_get :Option%201 _output_get_2 :Option%202 _output_get_3 :Option%203 _output_get_4 :Option%204 (stale _output_get_5))))
    (:4
      (bind _output_get_5 (Variables|Default|SetItem%20to%20Add "/Game/2DPlatformingKit/Blueprints/Inventory/Blueprints/ItemClasses/Data_Crystal.Data_Crystal_C"))
      (return (Utilities|Select :Index (Math|Random|RandomIntegerinRange 0 5) :Option%200 _output_get :Option%201 _output_get_2 :Option%202 _output_get_3 :Option%203 _output_get_4 :Option%204 _output_get_5)))))