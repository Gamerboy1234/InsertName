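; Slot-based inventory that stores item classes with amounts in an array sized to AmountofSlots on BeginPlay.
; Query functions read item info from class defaults and find empty slots or non-full stacks.
; AddItem tops up stackable items to MaxStackSize before using empty slots, and places non-stackable items one per slot.
; It recurses on any overflow and returns success plus the amount that did not fit.
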(event EventBeginPlay
  (Utilities|Array|Resize (Variables|Default|GetSlots) (Variables|Default|GetAmountofSlots)))

(fn ConstructionScript)

(fn IsSlotEmpty?
  (params (Index :type Integer))
  (return (not (Utilities|IsValidClass (.ItemClass (Utilities|Struct|BreakS_InventorySlots (Utilities|Array|Get(acopy) (Variables|Default|GetSlots) Index)))))))

(fn GetItemInfoatIndex
  (params (Index :type Integer))
  (bind _slots (Variables|Default|GetSlots))
  (bind _output (Utilities|Array|Get(acopy) _slots Index))
  (bind (_itemclass _amount) (Utilities|Struct|BreakS_InventorySlots _output))
  (if (Utilities|IsValidClass _itemclass)
    (return false (Utilities|GetClassDefaults _itemclass) _amount)
    (else
      (return true "" 0))))

(fn SearchEmptySlot
  (bind (_array_element _array_index) (Utilities|Array|ForEachLoopwithBreak (Variables|Default|GetSlots) :!label _label)
    (:LoopBody
      (if (not (Utilities|IsValidClass (.ItemClass (Utilities|Struct|BreakS_InventorySlots _array_element))))
        (LocalVariables|SetLocal%20Bool true)
        (LocalVariables|SetLocal%20Index _array_index)
        (goto _label Break)))
    (:Completed
      (return (LocalVariables|GetLocal%20Bool) (LocalVariables|GetLocal%20Index)))))

(fn SearchFreeStack
  (params (Item%20Class :type Master%20Item%20Class%20Reference))
  (bind (_array_element _array_index) (Utilities|Array|ForEachLoopwithBreak (Variables|Default|GetSlots))
    (:LoopBody
      (if (Utilities|IsValidClass (.ItemClass (Utilities|Struct|BreakS_InventorySlots _array_element)))
        (if (and (== (.ItemClass (Utilities|Struct|BreakS_InventorySlots _array_element)) Item%20Class) (< (.Amount (Utilities|Struct|BreakS_InventorySlots _array_element)) (Variables|Default|GetMaxStackSize)))
          (LocalVariables|SetLocal%20Bool true)
          (LocalVariables|SetLocal%20Index _array_index))))
    (:Completed
      (return (LocalVariables|GetLocal%20Bool) (LocalVariables|GetLocal%20Index)))))

(fn AddItem
  (params (Item%20Class :type Master%20Item%20Class%20Reference) (Amount :type Integer))
  (LocalVariables|SetLocal%20Class Item%20Class)
  (LocalVariables|SetLocal%20Amount Amount)
  (if (.CanBeStacked? (Utilities|Struct|BreakS_ItemInfo (Utilities|GetClassDefaults Item%20Class)))
    (bind (_success_ _index) (CallFunction|SearchFreeStack (LocalVariables|GetLocal%20Class)))
    ;[1 1 1] Stack Items
    (if _success_
      (LocalVariables|SetFound%20Index _index)
      (if (> (+ (.Amount (Utilities|Struct|BreakS_InventorySlots (Utilities|Array|Get(acopy) (Variables|Default|GetSlots) (LocalVariables|GetFound%20Index)))) (LocalVariables|GetLocal%20Amount)) (Variables|Default|GetMaxStackSize))
        (LocalVariables|SetLocal%20Amount (- (+ (.Amount (Utilities|Struct|BreakS_InventorySlots (Utilities|Array|Get(acopy) (Variables|Default|GetSlots) (LocalVariables|GetFound%20Index)))) (LocalVariables|GetLocal%20Amount)) (Variables|Default|GetMaxStackSize)))
        (Utilities|Array|SetArrayElem (Variables|Default|GetSlots) (LocalVariables|GetFound%20Index) (Utilities|Struct|MakeS_InventorySlots (LocalVariables|GetLocal%20Class) (Variables|Default|GetMaxStackSize)))
        (bind _rest (CallFunction|AddItem (LocalVariables|GetLocal%20Class) (LocalVariables|GetLocal%20Amount)))
        (return true _rest)
        (else
          (Utilities|Array|SetArrayElem (Variables|Default|GetSlots) (LocalVariables|GetFound%20Index) (Utilities|Struct|MakeS_InventorySlots (LocalVariables|GetLocal%20Class) (+ (.Amount (Utilities|Struct|BreakS_InventorySlots (Utilities|Array|Get(acopy) (Variables|Default|GetSlots) (LocalVariables|GetFound%20Index)))) (LocalVariables|GetLocal%20Amount))))
          (return true 0)))
      (else
        ;[1 1 1] Current Stack is Full
        (bind (_success__2 _index_2) (CallFunction|SearchEmptySlot))
        (if _success__2
          (bind _output_get (LocalVariables|SetFound%20Index _index_2))
          (if (> (LocalVariables|GetLocal%20Amount) (Variables|Default|GetMaxStackSize))
            (Utilities|Array|SetArrayElem (Variables|Default|GetSlots) _output_get (Utilities|Struct|MakeS_InventorySlots (LocalVariables|GetLocal%20Class) (Variables|Default|GetMaxStackSize)))
            (bind _rest_2 (CallFunction|AddItem (LocalVariables|GetLocal%20Class) (- (LocalVariables|GetLocal%20Amount) (Variables|Default|GetMaxStackSize))))
            (return true _rest_2)
            (else
              (Utilities|Array|SetArrayElem (Variables|Default|GetSlots) (LocalVariables|GetFound%20Index) (Utilities|Struct|MakeS_InventorySlots (LocalVariables|GetLocal%20Class) (LocalVariables|GetLocal%20Amount)))
              (return true 0)))
          (else
            (return false (LocalVariables|GetLocal%20Amount))))))
    (else
      ;[1 1 1] Can't Be Stacked
      (bind (_success__3 _index_3) (CallFunction|SearchEmptySlot))
      (if _success__3
        (bind _output_get_2 (LocalVariables|SetFound%20Index _index_3))
        (Utilities|Array|SetArrayElem (Variables|Default|GetSlots) _output_get_2 (Utilities|Struct|MakeS_InventorySlots (LocalVariables|GetLocal%20Class) 1))
        (if (> (LocalVariables|GetLocal%20Amount) 1)
          (bind _rest_3 (CallFunction|AddItem (LocalVariables|GetLocal%20Class) (- (LocalVariables|GetLocal%20Amount) 1)))
          (return true _rest_3)
          (else
            (return true 0)))
        (else
          (return false (LocalVariables|GetLocal%20Amount)))))))

(fn GetAmountatIndex
  (params (Index :type Integer))
  (return (.Amount (Utilities|Struct|BreakS_InventorySlots (Utilities|Array|Get(acopy) (Variables|Default|GetSlots) Index)))))