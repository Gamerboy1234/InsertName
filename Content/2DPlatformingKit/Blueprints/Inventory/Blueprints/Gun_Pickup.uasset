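; Gun pickup for the 2D platforming kit that gives the player an item on overlap, with a configurable sprite and trigger scale.
; A one-time overlap runs the pickup, which stops with a message if the inventory is full.
; Weapons spawn and are used immediately when no gun or sword is equipped.
; Otherwise items enter the inventory, recording remaining amounts under an ID generated by a spawned tracker at BeginPlay.
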(event OnComponentBeginOverlap(Trigger)
  (params (OverlappedComponent :type Primitive%20Component%20Object%20Reference) (OtherActor :type Actor%20Object%20Reference) (OtherComp :type Primitive%20Component%20Object%20Reference) (OtherBodyIndex :type Integer) (bFromSweep :type Boolean) (SweepResult :type Hit%20Result%20Structure%20%28by%20ref%29))
  ;[1 1 1] on overlap start pickup event
  (Utilities|Casting|CastToPlayer_Character OtherActor)
  (Utilities|FlowControl|DoOnce false
    (:Completed
      (CallFunction|PickupEvent))))

(event Custom|Pickup%20Event
  ;[1 1 1] start item pickup
  (bind _asplayer_character (Utilities|Casting|CastToPlayer_Character (Game|GetPlayerCharacter 0)))
  (Variables|Default|SetPlayer%20Ref _asplayer_character)
  (CallFunction|PickupItem))

(event Custom|Pickup%20Item
  ;[1 1 1] pickup item
  (Utilities|PickUpItem (Variables|Default|GetPlayer%20Ref)))

(event EventBeginPlay
  ;[1 1 1] Set Pickup ID
  (bind _returnvalue (Game|SpawnActorfromClass "/Game/2DPlatformingKit/Blueprints/Player/Generic_ID_Tracker_BP.Generic_ID_Tracker_BP_C" (Math|Transform|MakeTransform "0, 0, 0" "0, 0, 0" "1,1,1") "Undefined" 0 0))
  (bind _output_get (Variables|Default|SetGeneric%20ID%20Tracker _returnvalue))
  (bind _id (Default|GenID _output_get))
  (Variables|Default|SetID _id))

(fn ConstructionScript
  (bind _papersprite (Variables|Default|GetPaperSprite))
  (bind _returnvalue (Transformation|GetWorldTransform _papersprite))
  (Rendering|Components|Sprite|SetSprite _papersprite (Variables|Default|GetSprite))
  (Transformation|SetWorldTransform (Variables|Default|GetTrigger) (Math|Transform|MakeTransform (.location _returnvalue) (.rotation _returnvalue) (Variables|Default|GetCollision%20Scale)) false false))