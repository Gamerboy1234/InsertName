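; SpellPickup is a world pickup in the 2D platforming kit that teaches the player a configured spell on overlap.
; When a Player_Character enters the trigger, it spawns a temporary SpellAdder with the spell class and its default ItemInfo, then calls ItemUsed.
; On success it shows a learned-spell message and destroys itself; the SpellAdder is destroyed either way.
; The construction script applies the configured sprite.
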(event OnComponentBeginOverlap(Trigger)
  (params (OverlappedComponent :type Primitive%20Component%20Object%20Reference) (OtherActor :type Actor%20Object%20Reference) (OtherComp :type Primitive%20Component%20Object%20Reference) (OtherBodyIndex :type Integer) (bFromSweep :type Boolean) (SweepResult :type Hit%20Result%20Structure%20%28by%20ref%29))
  (bind _spell_to_add_ (Variables|Default|GetSpell%20to%20Add%20))
  (bind _item_info (Utilities|GetClassDefaults _spell_to_add_))
  (bind _asplayer_character (Utilities|Casting|CastToPlayer_Character OtherActor))
  (Variables|Default|SetPlayer%20Ref _asplayer_character)
  (bind _returnvalue (Game|SpawnActorfromClass "/Game/2DPlatformingKit/Blueprints/Inventory/Blueprints/ItemClasses/Other/SpellAdder.SpellAdder_C" (Math|Transform|MakeTransform "0, 0, 0" "0, 0, 0" "1,1,1") "Undefined" 0 _spell_to_add_ _item_info 0 0 0))
  (bind _output_get (Variables|Default|SetSpell%20Adder _returnvalue))
  (Default|ItemUsed _output_get)
  (if (Variables|/Game/2DPlatformingKit/Blueprints/Inventory/Blueprints/ItemClasses/Other/SpellAdder.SpellAdder_C|GetSuccess? (Variables|Default|GetSpell%20Adder))
    (Utilities|UIScreenText (Utilities|Text|FormatText "You Learned The {SpellName} Spell" (.Name (Utilities|Struct|BreakS_ItemInfo _item_info))))
    (Actor|DestroyActor)
    (Actor|DestroyActor (Variables|Default|GetSpell%20Adder))
    (else
      (Actor|DestroyActor (Variables|Default|GetSpell%20Adder)))))

(fn ConstructionScript
  (Rendering|Components|Sprite|SetSprite (Variables|Default|GetPaperSprite) (Variables|Default|GetSprite)))