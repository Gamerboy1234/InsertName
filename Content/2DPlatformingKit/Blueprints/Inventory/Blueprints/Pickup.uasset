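; Pickup is a 2D sprite item that adds a configurable item and amount to the player's inventory when the player character overlaps its trigger.
; On pickup, the sprite eases toward the player, shrinks and hides.
; A successful add records the pickup's ID and leftover amount in the inventory's LootedPickups, then either updates Amount or destroys the actor, based on the returned remainder.
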(event OnComponentBeginOverlap(Trigger)
  (params (OverlappedComponent :type Primitive%20Component%20Object%20Reference) (OtherActor :type Actor%20Object%20Reference) (OtherComp :type Primitive%20Component%20Object%20Reference) (OtherBodyIndex :type Integer) (bFromSweep :type Boolean) (SweepResult :type Hit%20Result%20Structure%20%28by%20ref%29))
  ;[1 1 1] on overlap start pickup event
  (Utilities|Casting|CastToPlayer_Character OtherActor)
  (CallFunction|PickupEvent))

(event Custom|Pickup%20Event
  ;[1 1 1] start item pickup
  (bind _asplayer_character (Utilities|Casting|CastToPlayer_Character (Game|GetPlayerCharacter 0)))
  (Variables|Default|SetPlayer%20Ref _asplayer_character)
  (CallFunction|PickupItem))

(event Custom|Pickup%20Item
  (bind _player_ref (Variables|Default|GetPlayer%20Ref))
  ;[1 1 1] pickup item
  (Utilities|PickUpItem _player_ref _player_ref))

(fn ConstructionScript
  (Rendering|Components|Sprite|SetSprite (Variables|Default|GetPaperSprite) (Variables|Default|GetSprite)))