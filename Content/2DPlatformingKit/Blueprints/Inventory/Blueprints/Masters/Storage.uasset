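; Master storage Blueprint for chest-style containers in the 2D platforming kit, holding a fixed-size slot array seeded from start items.
; Slot functions add, remove, swap and merge items, with AddItem recursing to spread stackable or single items across slots.
; Most edits refresh the matching slot in the HUD Chest widget, which it shows or hides.
; Transfer functions accept items from the player inventory, while Take All input empties storage into it.
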(event Custom|Update%20Slot%20At%20Index
  (params (Index :type Integer))
  (Default|UpdateSlot (Utilities|Array|Get(acopy) (Variables|/Game/2DPlatformingKit/Widgets/Inventory_Widgets/ChestWidget.ChestWidget_C|GetSlots%20Widgets (Variables|Default|GetChest%20%20Widget)) Index)))

(event EventBeginPlay
  (Variables|Default|SetSlots (Variables|Default|GetStart%20Items))
  (Variables|Default|SetChest%20%20Widget (Variables|/Game/2DPlatformingKit/Widgets/Player_Widgets/HUD.HUD_C|GetChest (Variables|/Game/2DPlatformingKit/Blueprints/Inventory/Blueprints/Masters/Inventory_Master.Inventory_Master_C|GetHUD (Variables|/Game/2DPlatformingKit/Blueprints/Player/Player_Character.Player_Character_C|GetInventory%20Ref (Variables|Default|GetPlayerRef)))))
  (Utilities|Array|Resize (Variables|Default|GetSlots) (Variables|Default|GetAmountofSlots))
  (Input|EnableInput (Game|GetPlayerController 0)))

(event Input|ActionEvents|InputActionTakeAll
  (params (Key :type Key%20Structure))
  ;[1 1 1] Take all items in storage and move to inventory
  (:Pressed
    (if (not (Default|InventoryFull? (Variables|/Game/2DPlatformingKit/Blueprints/Player/Player_Character.Player_Character_C|GetInventory%20Ref (Variables|Default|GetPlayerRef))))
      (if (Variables|/Game/2DPlatformingKit/Blueprints/Inventory/Blueprints/Chest.Chest_C|GetIs%20Storage%20Open? (Variables|Default|GetChest))
        (Utilities|FlowControl|DoOnce false :!label _label
          (:Completed
            (CallFunction|MoveAlltoInventory (Variables|/Game/2DPlatformingKit/Blueprints/Player/Player_Character.Player_Character_C|GetInventory%20Ref (Variables|Default|GetPlayerRef)))
            (goto _label Reset))))
      (else
        (Utilities|UIScreenText "Inventory Full")))))

(fn ConstructionScript)

(fn IsSlotEmpty?
  (params (Index :type Integer))
  (return (not (Utilities|IsValidClass (.ItemClass (Utilities|Struct|BreakS_InventorySlots (Utilities|Array|Get(acopy) (Variables|Default|GetSlots) Index)))))))

(fn GetItemInfoatIndex
  (params (Index :type Integer))
  (bind _slots (Variables|Default|GetSlots))
  (bind _output (Utilities|Array|Get(acopy) _slots Index))
  (bind (_itemclass _amount) (Utilities|Struct|BreakS_InventorySlots _output))
  (if (Utilities|IsValidClass _itemclass)
    (return false (.Item%20Info (Utilities|GetClassDefaults _itemclass)) _amount)
    (else
      (return true "" 0))))

(fn SearchEmptySlot
  (bind (_array_element _array_index) (Utilities|Array|ForEachLoopwithBreak (Variables|Default|GetSlots) :!label _label)
    (:LoopBody
      (if (not (Utilities|IsValidClass (.ItemClass (Utilities|Struct|BreakS_InventorySlots _array_element))))
        (LocalVariables|SetLocal%20Bool true)
        (LocalVariables|SetLocal%20Index _array_index)
        (goto _label Break)))
    (:Completed
      (return (LocalVariables|GetLocal%20Bool) (LocalVariables|GetLocal%20Index)))))

(fn SearchFreeStack
  (params (Item%20Class :type Master%20Item%20Class%20Reference))
  (bind (_array_element _array_index) (Utilities|Array|ForEachLoopwithBreak (Variables|Default|GetSlots))
    (:LoopBody
      (if (Utilities|IsValidClass (.ItemClass (Utilities|Struct|BreakS_InventorySlots _array_element)))
        (if (and (== (.ItemClass (Utilities|Struct|BreakS_InventorySlots _array_element)) Item%20Class) (< (.Amount (Utilities|Struct|BreakS_InventorySlots _array_element)) (Variables|Default|GetMaxStackSize)))
          (LocalVariables|SetLocal%20Bool true)
          (LocalVariables|SetLocal%20Index _array_index))))
    (:Completed
      (return (LocalVariables|GetLocal%20Bool) (LocalVariables|GetLocal%20Index)))))

(fn GetAmountatIndex
  (params (Index :type Integer))
  (return (.Amount (Utilities|Struct|BreakS_InventorySlots (Utilities|Array|Get(acopy) (Variables|Default|GetSlots) Index)))))

(fn RemoveItematIndex
  (params (Index :type Integer) (Amount :type Integer))
  (bind _slots (Variables|Default|GetSlots))
  (LocalVariables|SetLocal%20Index Index)
  (LocalVariables|SetLocal%20Amount Amount)
  (if (and (not (CallFunction|IsSlotEmpty? (LocalVariables|GetLocal%20Index))) (> (LocalVariables|GetLocal%20Amount) 0))
    (if (>= (LocalVariables|GetLocal%20Amount) (CallFunction|GetAmountatIndex (LocalVariables|GetLocal%20Index)))
      (Utilities|Array|SetArrayElem (Variables|Default|GetSlots) (LocalVariables|GetLocal%20Index) (Utilities|Struct|MakeS_InventorySlots 0 0) true)
      (CallFunction|UpdateSlotatIndex (LocalVariables|GetLocal%20Index))
      (return true)
      (else
        (Utilities|Array|SetArrayElem _slots (LocalVariables|GetLocal%20Index) (Utilities|Struct|MakeS_InventorySlots (.ItemClass (Utilities|Struct|BreakS_InventorySlots (Utilities|Array|Get(acopy) _slots (LocalVariables|GetLocal%20Index)))) (- (.Amount (Utilities|Struct|BreakS_InventorySlots (Utilities|Array|Get(acopy) _slots (LocalVariables|GetLocal%20Index)))) (LocalVariables|GetLocal%20Amount))) true)
        (CallFunction|UpdateSlotatIndex (LocalVariables|GetLocal%20Index))
        (return true)))
    (else
      (return false))))

(fn SwapSlots
  (params (Index%201 :type Integer) (Index%202 :type Integer))
  (bind _slots (Variables|Default|GetSlots))
  (bind _returnvalue (Utilities|Array|LastIndex _slots))
  (LocalVariables|SetLocal%20Index%201 Index%201)
  (LocalVariables|SetLocal%20Index%202 Index%202)
  (if (or (> (LocalVariables|GetLocal%20Index%201) _returnvalue) (> (LocalVariables|GetLocal%20Index%202) _returnvalue))
    (return false)
    (else
      (LocalVariables|SetLocal%20Slot%202 (Utilities|Array|Get(acopy) (Variables|Default|GetSlots) (LocalVariables|GetLocal%20Index%202)))
      (Utilities|Array|SetArrayElem (Variables|Default|GetSlots) (LocalVariables|GetLocal%20Index%202) (Utilities|Array|Get(acopy) (Variables|Default|GetSlots) (LocalVariables|GetLocal%20Index%201)))
      (Utilities|Array|SetArrayElem (Variables|Default|GetSlots) (LocalVariables|GetLocal%20Index%201) (LocalVariables|GetLocal%20Slot%202))
      (CallFunction|UpdateSlotatIndex (LocalVariables|GetLocal%20Index%201))
      (CallFunction|UpdateSlotatIndex (LocalVariables|GetLocal%20Index%202))
      (return true))))

(fn AddtoIndex
  (params (From%20Index :type Integer) (To%20Index :type Integer))
  (LocalVariables|SetLocal%20From From%20Index)
  (LocalVariables|SetLocal%20To To%20Index)
  (if (Math|Boolean|ANDBoolean (== (.ItemClass (Utilities|Struct|BreakS_InventorySlots (Utilities|Array|Get(acopy) (Variables|Default|GetSlots) (LocalVariables|GetLocal%20From)))) (.ItemClass (Utilities|Struct|BreakS_InventorySlots (Utilities|Array|Get(acopy) (Variables|Default|GetSlots) (LocalVariables|GetLocal%20To))))) (< (.Amount (Utilities|Struct|BreakS_InventorySlots (Utilities|Array|Get(acopy) (Variables|Default|GetSlots) (LocalVariables|GetLocal%20To)))) (Variables|Default|GetMaxStackSize)) (.CanBeStacked? (Utilities|Struct|BreakS_ItemInfo (.Item%20Info (CallFunction|GetItemInfoatIndex (LocalVariables|GetLocal%20From))))))
    (LocalVariables|SetLocal%20Class (.ItemClass (Utilities|Struct|BreakS_InventorySlots (Utilities|Array|Get(acopy) (Variables|Default|GetSlots) (LocalVariables|GetLocal%20From)))))
    (if (>= (- (Variables|Default|GetMaxStackSize) (CallFunction|GetAmountatIndex (LocalVariables|GetLocal%20To))) (CallFunction|GetAmountatIndex (LocalVariables|GetLocal%20From)))
      (Utilities|Array|SetArrayElem (Variables|Default|GetSlots) (LocalVariables|GetLocal%20To) (Utilities|Struct|MakeS_InventorySlots (LocalVariables|GetLocal%20Class) (+ (CallFunction|GetAmountatIndex (LocalVariables|GetLocal%20To)) (CallFunction|GetAmountatIndex (LocalVariables|GetLocal%20From)))))
      (Utilities|Array|SetArrayElem (Variables|Default|GetSlots) 0 (Utilities|Struct|MakeS_InventorySlots 0 0))
      (CallFunction|UpdateSlotatIndex (LocalVariables|GetLocal%20From))
      (CallFunction|UpdateSlotatIndex (LocalVariables|GetLocal%20To))
      (else
        (Utilities|Array|SetArrayElem (Variables|Default|GetSlots) (LocalVariables|GetLocal%20From) (Utilities|Struct|MakeS_InventorySlots (LocalVariables|GetLocal%20Class) (- (CallFunction|GetAmountatIndex (LocalVariables|GetLocal%20From)) (- (Variables|Default|GetMaxStackSize) (CallFunction|GetAmountatIndex (LocalVariables|GetLocal%20To))))))
        (Utilities|Array|SetArrayElem (Variables|Default|GetSlots) (LocalVariables|GetLocal%20To) (Utilities|Struct|MakeS_InventorySlots (LocalVariables|GetLocal%20Class) (Variables|Default|GetMaxStackSize)))))
    (return true)
    (else
      (return false))))

(fn AddItem
  (params (Item%20Class :type Master%20Item%20Class%20Reference) (Amount :type Integer))
  (LocalVariables|SetLocal%20Class Item%20Class)
  (LocalVariables|SetLocal%20Amount Amount)
  (if (.CanBeStacked? (Utilities|Struct|BreakS_ItemInfo (.Item%20Info (Utilities|GetClassDefaults Item%20Class))))
    (bind (_success_ _index) (CallFunction|SearchFreeStack (LocalVariables|GetLocal%20Class)))
    ;[1 1 1] Stack Items
    (if _success_
      (LocalVariables|SetFound%20Index _index)
      (if (> (+ (.Amount (Utilities|Struct|BreakS_InventorySlots (Utilities|Array|Get(acopy) (Variables|Default|GetSlots) (LocalVariables|GetFound%20Index)))) (LocalVariables|GetLocal%20Amount)) (Variables|Default|GetMaxStackSize))
        (LocalVariables|SetLocal%20Amount (- (+ (.Amount (Utilities|Struct|BreakS_InventorySlots (Utilities|Array|Get(acopy) (Variables|Default|GetSlots) (LocalVariables|GetFound%20Index)))) (LocalVariables|GetLocal%20Amount)) (Variables|Default|GetMaxStackSize)))
        (Utilities|Array|SetArrayElem (Variables|Default|GetSlots) (LocalVariables|GetFound%20Index) (Utilities|Struct|MakeS_InventorySlots (LocalVariables|GetLocal%20Class) (Variables|Default|GetMaxStackSize)))
        (CallFunction|UpdateSlotatIndex (LocalVariables|GetFound%20Index))
        (bind _rest (CallFunction|AddItem (LocalVariables|GetLocal%20Class)))
        (return true _rest)
        (else
          (Utilities|Array|SetArrayElem (Variables|Default|GetSlots) (LocalVariables|GetFound%20Index) (Utilities|Struct|MakeS_InventorySlots (LocalVariables|GetLocal%20Class) (+ (.Amount (Utilities|Struct|BreakS_InventorySlots (Utilities|Array|Get(acopy) (Variables|Default|GetSlots) (LocalVariables|GetFound%20Index)))) (LocalVariables|GetLocal%20Amount))))
          (CallFunction|UpdateSlotatIndex (LocalVariables|GetFound%20Index))
          (return true 0)))
      (else
        ;[1 1 1] Current Stack is Full
        (bind (_success__2 _index_2) (CallFunction|SearchEmptySlot))
        (if _success__2
          (bind _output_get (LocalVariables|SetFound%20Index _index_2))
          (if (> (LocalVariables|GetLocal%20Amount) (Variables|Default|GetMaxStackSize))
            (Utilities|Array|SetArrayElem (Variables|Default|GetSlots) _output_get (Utilities|Struct|MakeS_InventorySlots (LocalVariables|GetLocal%20Class) (Variables|Default|GetMaxStackSize)))
            (CallFunction|UpdateSlotatIndex (LocalVariables|GetFound%20Index))
            (bind _rest_2 (CallFunction|AddItem (LocalVariables|GetLocal%20Class) (- (LocalVariables|GetLocal%20Amount) (Variables|Default|GetMaxStackSize))))
            (return true _rest_2)
            (else
              (Utilities|Array|SetArrayElem (Variables|Default|GetSlots) (LocalVariables|GetFound%20Index) (Utilities|Struct|MakeS_InventorySlots (LocalVariables|GetLocal%20Class) (LocalVariables|GetLocal%20Amount)))
              (CallFunction|UpdateSlotatIndex (LocalVariables|GetFound%20Index))
              (return true 0)))
          (else
            (return false (LocalVariables|GetLocal%20Amount))))))
    (else
      ;[1 1 1] Can't Be Stacked
      (bind (_success__3 _index_3) (CallFunction|SearchEmptySlot))
      (if _success__3
        (bind _output_get_2 (LocalVariables|SetFound%20Index _index_3))
        (Utilities|Array|SetArrayElem (Variables|Default|GetSlots) _output_get_2 (Utilities|Struct|MakeS_InventorySlots (LocalVariables|GetLocal%20Class) 1))
        (CallFunction|UpdateSlotatIndex (LocalVariables|GetFound%20Index))
        (if (> (LocalVariables|GetLocal%20Amount) 1)
          (bind _rest_3 (CallFunction|AddItem (LocalVariables|GetLocal%20Class) (- (LocalVariables|GetLocal%20Amount) 1)))
          (return true _rest_3)
          (else
            (return true 0)))
        (else
          (return false (LocalVariables|GetLocal%20Amount)))))))

(fn AddItemtoIndex
  (params (Index :type Integer) (Item%20Class :type Master%20Item%20Class%20Reference) (Amount :type Integer))
  (if (and (CallFunction|IsSlotEmpty? Index) (<= Amount (Variables|Default|GetMaxStackSize)))
    (Utilities|Array|SetArrayElem (Variables|Default|GetSlots) Index (Utilities|Struct|MakeS_InventorySlots Item%20Class Amount))
    (CallFunction|UpdateSlotatIndex Index)
    (return true)
    (else
      (return false))))

(fn IncreasseAmountatIndex
  (params (Inedex :type Integer) (Amount :type Integer))
  (bind _slots (Variables|Default|GetSlots))
  (bind _output (Utilities|Array|Get(acopy) _slots Inedex))
  (if (and (not (CallFunction|IsSlotEmpty? Inedex)) (<= (+ (CallFunction|GetAmountatIndex Inedex) Amount) (Variables|Default|GetMaxStackSize)))
    (Utilities|Array|SetArrayElem _slots Inedex (Utilities|Struct|MakeS_InventorySlots (.itemclass _output) (+ (.amount _output) Amount)))
    (CallFunction|UpdateSlotatIndex Inedex)
    (return true)
    (else
      (return false))))

(fn ShowChest
  (Widget|SetVisibility (Variables|Default|GetChest%20%20Widget) "Visible")
  (Variables|/Game/2DPlatformingKit/Blueprints/Inventory/Blueprints/Masters/Inventory_Master.Inventory_Master_C|SetIs%20Storage%20Open? (Variables|/Game/2DPlatformingKit/Blueprints/Player/Player_Character.Player_Character_C|GetInventory%20Ref (Variables|Default|GetPlayerRef)) true)
  (return))

(fn HideChest
  (Widget|SetVisibility (Variables|Default|GetChest%20%20Widget) "Hidden")
  (Variables|/Game/2DPlatformingKit/Blueprints/Inventory/Blueprints/Masters/Inventory_Master.Inventory_Master_C|SetIs%20Storage%20Open? (Variables|/Game/2DPlatformingKit/Blueprints/Player/Player_Character.Player_Character_C|GetInventory%20Ref (Variables|Default|GetPlayerRef)) false)
  (return))

(fn MovefromInvtoStorage
  (params (Inventory :type Inventory%20Master%20Object%20Reference) (Inventory%20Index :type Integer) (Storage%20Index :type Integer))
  (LocalVariables|SetLocal%20Inventory Inventory)
  (LocalVariables|SetLocal%20Inv%20Index Inventory%20Index)
  (LocalVariables|SetLocal%20Storage%20Index Storage%20Index)
  (if (CallFunction|IsSlotEmpty? (LocalVariables|GetLocal%20Storage%20Index))
    (LocalVariables|SetAmount%20To%20Add (Default|GetAmountatIndex (LocalVariables|GetLocal%20Inventory) (LocalVariables|GetLocal%20Inv%20Index)))
    (bind _success (CallFunction|AddItemtoIndex (LocalVariables|GetLocal%20Storage%20Index) (Utilities|Struct|BreakS_InventorySlots (Utilities|Array|Get(acopy) (Variables|/Game/2DPlatformingKit/Blueprints/Inventory/Blueprints/Masters/Inventory_Master.Inventory_Master_C|GetSlots (LocalVariables|GetLocal%20Inventory)) (LocalVariables|GetLocal%20Inv%20Index))) (LocalVariables|GetAmount%20To%20Add)))
    (if _success
      (Default|RemoveItematIndex (LocalVariables|GetLocal%20Inventory) (LocalVariables|GetLocal%20Inv%20Index) (LocalVariables|GetAmount%20To%20Add) false)
      (return true)
      (else
        (return false)))
    (elif (Math|Boolean|ANDBoolean (== (Utilities|Struct|BreakS_InventorySlots (Utilities|Array|Get(acopy) (Variables|Default|GetSlots) (LocalVariables|GetLocal%20Storage%20Index))) (Utilities|Struct|BreakS_InventorySlots (Utilities|Array|Get(acopy) (Variables|/Game/2DPlatformingKit/Blueprints/Inventory/Blueprints/Masters/Inventory_Master.Inventory_Master_C|GetSlots (LocalVariables|GetLocal%20Inventory)) (LocalVariables|GetLocal%20Inv%20Index)))) (.CanBeStacked? (Utilities|Struct|BreakS_ItemInfo (.Item%20Info (CallFunction|GetItemInfoatIndex (LocalVariables|GetLocal%20Storage%20Index))))) (< (CallFunction|GetAmountatIndex (LocalVariables|GetLocal%20Storage%20Index)) (Variables|Default|GetMaxStackSize)))
      (LocalVariables|SetAmount%20To%20Add (Math|Integer|SelectInt (- (Variables|Default|GetMaxStackSize) (CallFunction|GetAmountatIndex (LocalVariables|GetLocal%20Storage%20Index))) (Default|GetAmountatIndex (LocalVariables|GetLocal%20Inventory) (LocalVariables|GetLocal%20Inv%20Index)) (> (Default|GetAmountatIndex (LocalVariables|GetLocal%20Inventory) (LocalVariables|GetLocal%20Inv%20Index)) (- (Variables|Default|GetMaxStackSize) (CallFunction|GetAmountatIndex (LocalVariables|GetLocal%20Storage%20Index))))))
      (bind _success_ (CallFunction|IncreasseAmountatIndex (LocalVariables|GetLocal%20Storage%20Index) (LocalVariables|GetAmount%20To%20Add)))
      (if _success_
        (Default|RemoveItematIndex (LocalVariables|GetLocal%20Inventory) (LocalVariables|GetLocal%20Inv%20Index) (LocalVariables|GetAmount%20To%20Add) false)
        (return true)
        (else
          (return false)))
      (else
        (return false)))))

(fn MoveAlltoInventory
  (params (Inventory :type Inventory%20Master%20Object%20Reference))
  (bind _output_get (LocalVariables|SetLocal%20Inv Inventory))
  (Utilities|IsValid _output_get
    (:Is%20Valid
      (for (_array_element _array_index) (Variables|Default|GetSlots)
        (if (Utilities|IsValidClass (.ItemClass (Utilities|Struct|BreakS_InventorySlots _array_element)))
          (bind (_success _rest_) (Default|AddItem (LocalVariables|GetLocal%20Inv) (.ItemClass (Utilities|Struct|BreakS_InventorySlots _array_element)) (.Amount (Utilities|Struct|BreakS_InventorySlots _array_element)) true))
          (if _success
            (CallFunction|RemoveItematIndex _array_index (- (.Amount (Utilities|Struct|BreakS_InventorySlots _array_element)) _rest_)))))
      (return))
    (:Is%20Not%20Valid
      (return))))