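; Inventory master Blueprint from a 2D platforming kit, holding macros that spawn world pickups when items are dropped from inventory slots.
; When Drop is true, each macro spawns a DropablePickup at the player's DropItem transform, passing the slot's item class and its drop sprite from class defaults.
; One macro drops a single item and the other a given amount; a false Drop exits through Else.
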(fn ConstructionScript)