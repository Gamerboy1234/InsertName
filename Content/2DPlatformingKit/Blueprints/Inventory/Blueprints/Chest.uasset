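; Interactable 2D chest that lets the player open an item storage while inside its trigger.
; Overlap toggles input; Interact spawns a Storage actor on first use, then shows its chest widget and refreshes the player's inventory.
; Leaving the trigger closes open storage; closing re-arms the DoOnce.
; Optional BeginPlay generation rolls DataTable chances for starting items, with random amounts gated by the stackable default of the player's MasterItemRef class.
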(event OnComponentBeginOverlap(Trigger)
  (params (OverlappedComponent :type Primitive%20Component%20Object%20Reference) (OtherActor :type Actor%20Object%20Reference) (OtherComp :type Primitive%20Component%20Object%20Reference) (OtherBodyIndex :type Integer) (bFromSweep :type Boolean) (SweepResult :type Hit%20Result%20Structure%20%28by%20ref%29))
  ;[1 1 1] Enable input on collison and diaable input when player leaves
  (bind _asplayer_character (Utilities|Casting|CastToPlayer_Character OtherActor))
  (Variables|Default|SetPlayer%20Ref _asplayer_character)
  (Input|EnableInput (Game|GetPlayerController 0)))

(event OnComponentEndOverlap(Trigger)
  (params (OverlappedComponent :type Primitive%20Component%20Object%20Reference) (OtherActor :type Actor%20Object%20Reference) (OtherComp :type Primitive%20Component%20Object%20Reference) (OtherBodyIndex :type Integer))
  ;[1 1 1] Enable input on collison and diaable input when player leaves
  (bind _asplayer_character (Utilities|Casting|CastToPlayer_Character OtherActor))
  (Variables|Default|SetPlayer%20Ref _asplayer_character)
  (Input|DisableInput (Game|GetPlayerController 0))
  (if (Variables|Default|GetIs%20Storage%20Open?)
    (CallFunction|OnStorageClosed)))

(event Custom|On%20Storage%20Closed
  (bind _player_ref (Variables|Default|GetPlayer%20Ref))
  (bind _player_ref_2 (Variables|Default|GetPlayer%20Ref))
  (bind _inventory_ref (Variables|/Game/2DPlatformingKit/Blueprints/Player/Player_Character.Player_Character_C|GetInventory%20Ref _player_ref))
  (bind _inventory_ref_2 (Variables|/Game/2DPlatformingKit/Blueprints/Player/Player_Character.Player_Character_C|GetInventory%20Ref _player_ref_2))
  ;[1 1 1] Spawn Storage actor and interact and update widgets
  (Variables|Default|SetIs%20Storage%20Open? false)
  (Default|HideChest (Variables|Default|GetStorage))
  (if (Variables|/Game/2DPlatformingKit/Blueprints/Inventory/Blueprints/Inventory_Master.Inventory_Master_C|GetIs%20Visable? _inventory_ref)
    (Default|HideInventory _inventory_ref)
    (Default|ShowInventory _inventory_ref)
    (Utilities|FlowControl|DoOnce false) ; enters at Reset
    (else
      (Utilities|FlowControl|DoOnce false) ; enters at Reset
    )))

(event EventBeginPlay
  ;[1 1 1] Get player ref and randomly gen Items starting items
  (bind _asplayer_character (Utilities|Casting|CastToPlayer_Character (Game|GetPlayerCharacter 0)))
  (Variables|Default|SetPlayer%20Ref _asplayer_character)
  (Variables|Default|SetIs%20Storage%20Open? false)
  (if (Variables|Default|GetRandom%20Gen?)
    (CallFunction|GenerateStartingItems)))

(event Input|ActionEvents|InputActionInteract
  (params (Key :type Key%20Structure))
  (bind _player_ref (Variables|Default|GetPlayer%20Ref))
  (bind _inventory_ref (Variables|/Game/2DPlatformingKit/Blueprints/Player/Player_Character.Player_Character_C|GetInventory%20Ref _player_ref))
  ;[1 1 1] Spawn Storage actor and interact and update widgets
  (:Pressed
    (Utilities|FlowControl|DoOnce false
      (:Completed
        (Utilities|IsValid (Variables|Default|GetStorage)
          (:Is%20Valid
            _)
          (:Is%20Not%20Valid
            (bind _returnvalue (Game|SpawnActorfromClass "/Game/2DPlatformingKit/Blueprints/Inventory/Blueprints/Storage.Storage_C" (Math|Transform|MakeTransform "0, 0, 0" "0, 0, 0" "1,1,1") "Undefined" 0 (Variables|Default|GetAmount%20of%20Slots) (Variables|Default|GetPlayer%20Ref) (Variables|Default|GetSlots%20per%20Row) self (Variables|Default|GetObject%20Name) (Variables|Default|GetStarting%20Items) 0))
            (Variables|Default|SetStorage _returnvalue)))
        (Default|GenerateSlots (Variables|/Game/2DPlatformingKit/Blueprints/Inventory/Blueprints/Storage.Storage_C|GetChest%20%20Widget (Variables|Default|GetStorage)) (Variables|Default|GetStorage))
        (Default|ShowChest (Variables|Default|GetStorage))
        (Default|HideInventory _inventory_ref)
        (Default|ShowInventory _inventory_ref)
        (Variables|Default|SetIs%20Storage%20Open? true)))))

(fn ConstructionScript
  (Rendering|Components|Sprite|SetSprite (Variables|Default|GetPaperSprite) (Variables|Default|GetChest%20Sprite)))

(fn GenerateStartingItems
  (bind _outrownames (DataTable|GetDataTableRowNames (Variables|Default|GetData%20Table%20for%20Random%20Gen)))
  (for _array_element _outrownames
    (bind _returnvalue (Utilities|GetDataTableRow (Variables|Default|GetData%20Table%20for%20Random%20Gen) _array_element)
      (:then
        (if (and (Utilities|IsValidClass (.ItemClass (Utilities|Struct|BreakS_ChestContent _returnvalue))) (<= (Math|Random|RandomIntegerinRange 1 100) (.Chance (Utilities|Struct|BreakS_ChestContent _returnvalue))))
          (if (.CanBeStacked? (Utilities|Struct|BreakS_ItemInfo (.Item%20Info (Utilities|GetClassDefaults (Utilities|GetClass (Variables|/Game/2DPlatformingKit/Blueprints/Player/Player_Character.Player_Character_C|GetMaster%20Item%20Ref (Variables|Default|GetPlayer%20Ref)))))))
            (Utilities|Array|Add (Variables|Default|GetStarting%20Items) (Utilities|Struct|MakeS_InventorySlots (.ItemClass (Utilities|Struct|BreakS_ChestContent _returnvalue)) (Math|Random|RandomIntegerinRange (.MinAmount (Utilities|Struct|BreakS_ChestContent _returnvalue)) (.MaxAmount (Utilities|Struct|BreakS_ChestContent _returnvalue)))))
            (else
              (Utilities|Array|Add (Variables|Default|GetStarting%20Items) (Utilities|Struct|MakeS_InventorySlots (.ItemClass (Utilities|Struct|BreakS_ChestContent _returnvalue)) 1))))))
      (:RowNotFound
        (Development|PrintString "Row Not Found")
        (return))))
  (return))