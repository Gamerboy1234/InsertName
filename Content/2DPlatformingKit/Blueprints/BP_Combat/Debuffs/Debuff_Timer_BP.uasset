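; Debuff timer for the 2D platforming kit that applies damage-over-time to the player.
; Setup stores the debuff parameters, copies a spawned effect's flipbook to the player's front and back overlays (except for the attached leech effect) and starts a looping timer.
; Each tick deals damage multiplied by stack count.
; The timer clears when ticks run out, the debuff is invalid or the player dies, resetting stacks and visuals.
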(event Custom|SetUp%20Timer
  (params (Damage :type Float%20%28single-precision%29) (Damage%20Effect :type Master%20Damage%20Effect%20Class%20Reference) (Ticks :type Float%20%28single-precision%29) (Occurrences :type Float%20%28single-precision%29) (Debuff :type Master%20Debuff%20Object%20Reference))
  ;[1 1 1] Damage Timer
  (Variables|Default|SetDamage Damage)
  (Variables|Default|SetEffect Damage%20Effect)
  (Variables|Default|SetTicks Ticks)
  (Variables|Default|SetOccurrences Occurrences)
  (Variables|Default|SetDebuff Debuff)
  (CallFunction|SpawnEffect (Variables|Default|GetEffect))
  (bind _returnvalue (Utilities|Time|SetTimerbyEvent (delegate Custom|Start%20Timer) (Variables|Default|GetOccurrences) true))
  (Variables|Default|SetDebuff%20Timer _returnvalue))

(event Custom|Start%20Timer
  (bind _debuff (Variables|Default|GetDebuff))
  ;[1 1 1] Damage Timer
  (Utilities|IsValid (Variables|Default|GetDebuff)
    (:Is%20Valid
      (Variables|Default|SetDebuff%20Stack (Default|GetStackCount _debuff _debuff))
      (if (not (CallFunction|IsPlayerDead self))
        (CallFunction|DamagePlayer self (CallFunction|DebuffDamageMultiplier (Variables|Default|GetDamage) (Variables|Default|GetDebuff%20Stack)))
        (bind _result (Math|Float|DecrementFloat (Variables|Default|GetTicks))
          (:%20%20
            (if (<= _result 0.0)
              (CallFunction|ClearTimer))))
        (else
          (CallFunction|ClearTimer))))
    (:Is%20Not%20Valid
      (CallFunction|ClearTimer))))

(event EventBeginPlay
  ;[1 1 1] Get Player
  (Variables|Default|SetPlayer%20Ref (CallFunction|GetPlayer self)))

(fn ConstructionScript)

(fn SpawnEffect
  (params (Effect :type Master%20Damage%20Effect%20Class%20Reference))
  (bind _player_ref (Variables|Default|GetPlayer%20Ref))
  (bind _output_get (LocalVariables|SetLocal%20Effect Effect))
  (if (not (== _output_get "/Game/2DPlatformingKit/Blueprints/BP_Combat/Debuffs/Attached_Leech_EFX.Attached_Leech_EFX_C"))
    (bind _returnvalue (Game|SpawnActorfromClass (LocalVariables|GetLocal%20Effect) (Math|Transform|MakeTransform "0,10000.000000, 0" "0, 0, 0" "1,1,1") "Undefined" 0 0))
    (Default|ApplyEffect _returnvalue)
    (Sprite|SetFlipbook (Variables|/Game/2DPlatformingKit/Blueprints/Player/Player_Character.Player_Character_C|GetDamage%20Over%20Time%20Front _player_ref) (Class|PaperFlipbookComponent|GetFlipbook (Variables|/Game/2DPlatformingKit/Blueprints/BP_Combat/Debuffs/Master_Damage_Effect.Master_Damage_Effect_C|GetPaperFlipbook _returnvalue)))
    (Sprite|SetFlipbook (Variables|/Game/2DPlatformingKit/Blueprints/Player/Player_Character.Player_Character_C|GetDamage%20Over%20Time%20Back _player_ref) (Class|PaperFlipbookComponent|GetFlipbook (Variables|/Game/2DPlatformingKit/Blueprints/BP_Combat/Debuffs/Master_Damage_Effect.Master_Damage_Effect_C|GetPaperFlipbook _returnvalue)))))

(fn ClearTimer
  (Utilities|Time|ClearandInvalidateTimerbyHandle (Variables|Default|GetDebuff%20Timer))
  (Default|ResetStack (Variables|/Game/2DPlatformingKit/Blueprints/Player/Player_Character.Player_Character_C|GetDebuff%20Stack%20Counter (Variables|Default|GetPlayer%20Ref)) (Variables|Default|GetDebuff))
  (Default|ResetDamageOverEffect (Variables|Default|GetPlayer%20Ref) (Variables|Default|GetDebuff)))

(fn DebuffDamageMultiplier
  (params (Damage :type Float%20%28single-precision%29) (Stacks :type Integer))
  (return (* Stacks Damage)))