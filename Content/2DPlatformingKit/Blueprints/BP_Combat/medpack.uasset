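; Medpack inventory item for the 2D platforming kit that heals the player when used.
; On BeginPlay it caches a reference to the Player_Character.
; ItemUsed heals by HPToAdd if HP is below maximum, then removes one from the inventory slot without spawning a drop and destroys itself if removal succeeds.
; At full health it shows a screen message instead and the item is kept.
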(event EventBeginPlay
  (bind _asplayer_character (Utilities|Casting|CastToPlayer_Character (Game|GetPlayerCharacter 0)))
  (Variables|Default|SetPlayer%20Ref _asplayer_character))

(event EventItemUsed
  (bind _player_ref (Variables|Default|GetPlayer%20Ref))
  (if (< (Variables|/Game/2DPlatformingKit/Blueprints/Player/Player_Character.Player_Character_C|GetPlayer%20HP _player_ref) (Variables|/Game/2DPlatformingKit/Blueprints/Player/Player_Character.Player_Character_C|GetMaxHP _player_ref))
    (Default|Heal (Variables|Default|GetPlayer%20Ref) (Variables|Default|GetHP%20to%20Add))
    (bind _success (Default|RemoveItematIndex (Variables|Default|GetInventory) (Variables|Default|GetIndex) 1 false))
    (if _success
      (Actor|DestroyActor))
    (else
      (Utilities|UIScreenText "Health is full"))))

(fn ConstructionScript
  (|CallParentFunction))