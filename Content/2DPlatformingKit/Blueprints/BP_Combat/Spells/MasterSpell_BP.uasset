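; Master spell Blueprint for the 2D platforming kit that runs a spell's cooldown and shows it on its UI spell slot.
; OnCoolDown finds the slot through the game mode, disables and dims it, then plays a timeline sized to the cooldown.
; Each update drives the slot material's Percent and countdown text, saving progress so paused cooldowns can resume.
; Completion calls ResetSpell and restores the slot.
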(event Custom|On%20Cool%20Down%20Done
  (Class|MasterSpell|ResetSpell)
  (Utilities|IsValid (Variables|Default|GetSpell%20Slot)
    (:Is%20Valid
      (Widget|SetIsEnabled (Variables|/Game/2DPlatformingKit/Widgets/Inventory_Widgets/ActionSlot.ActionSlot_C|GetItemBTN (Variables|Default|GetSpell%20Slot)) true)
      (Appearance|SetColorandOpacity (Variables|/Game/2DPlatformingKit/Widgets/Inventory_Widgets/ActionSlot.ActionSlot_C|GetItemImage (Variables|Default|GetSpell%20Slot)) "(R=1.000000,G=1.000000,B=1.000000,A=1.000000)" :!class /Script/UMG.Image)
      (Widget|SetVisibility (Variables|/Game/2DPlatformingKit/Widgets/Inventory_Widgets/ActionSlot.ActionSlot_C|GetCoolDownImage (Variables|Default|GetSpell%20Slot)) "Hidden")
      (Variables|/Game/2DPlatformingKit/Widgets/Inventory_Widgets/ActionSlot.ActionSlot_C|SetOnCoolDown? (Variables|Default|GetSpell%20Slot) false))))

(event EventOnCoolDown
  (params (ResumeCooldown :type Boolean) (Time :type Float%20%28single-precision%29))
  (bind _self self)
  (bind _self_2 self)
  (bind _cooldown_time (Variables|Default|GetCoolDown%20Time))
  (bind _sidescrollergamemode (CallFunction|GetSideScrollerGameMode _self))
  (bind _slot (Default|GetSpellSlot _sidescrollergamemode _self_2))
  (if ResumeCooldown
    (Variables|Default|SetSpell%20Slot (Default|GetSpellSlot (CallFunction|GetSideScrollerGameMode self) self))
    (CallFunction|SetupUMG Time)
    (Components|Timeline|SetPlaybackPosition (Variables|Default|GetCoolDown%20Time) (Variables|Default|GetCurrentTimeLinePostion) false true)
    (Timeline|CoolDown%20Time Play
      (:Update
        (CallFunction|UpdateCooldown (Components|Timeline|GetPlaybackPosition _cooldown_time) (Components|Timeline|GetTimelineLength _cooldown_time))
        (if (Variables|Default|GetbCoolDownPaused)
          (Audio|Components|Audio|Stop (Variables|Default|GetCoolDown%20Time))))
      (:Finished
        (if (not (Variables|Default|GetbCoolDownPaused))
          (CallFunction|OnCoolDownDone))))
    (else
      (Utilities|IsValid _slot
        (:Is%20Valid
          (CallFunction|SetupCooldown _slot Time)
          (Timeline|CoolDown%20Time PlayFromStart))
        (:Is%20Not%20Valid
          (Development|PrintString "Was unable to find spell slot" true true "(R=1.000000,G=0.000000,B=0.014467,A=1.000000)" 5.0))))))

(event EventResumeCoolDown
  (bind _cooldowntime (Variables|Default|GetCoolDownTime))
  (Components|Timeline|SetTimelineLength (Variables|Default|GetCoolDown%20Time) _cooldowntime)
  (Variables|Default|SetbCoolDownPaused false)
  (Class|MasterSpell|OnCoolDown true _cooldowntime))

(fn ConstructionScript
  (|CallParentFunction))

(fn SetupScaler
  (Rendering|Material|SetScalarParameterValue (Variables|/Game/2DPlatformingKit/Widgets/Inventory_Widgets/ActionSlot.ActionSlot_C|GetCoolDown%20Mat (Variables|Default|GetSpell%20Slot)) "Percent" 1.0 :!class /Script/Engine.MaterialInstanceDynamic))

(fn UpdateCooldown
  (params (Playback :type Float%20%28single-precision%29) (Length :type Float%20%28single-precision%29))
  (bind _spell_slot (Variables|Default|GetSpell%20Slot))
  (LocalVariables|SetLocal%20Playback Playback)
  (LocalVariables|SetLocal%20Length Length)
  (if (not (Variables|Default|GetbCoolDownPaused))
    (Utilities|IsValid _spell_slot
      (:Is%20Valid
        (Rendering|Material|SetScalarParameterValue (Variables|/Game/2DPlatformingKit/Widgets/Inventory_Widgets/ActionSlot.ActionSlot_C|GetCoolDown%20Mat (Variables|Default|GetSpell%20Slot)) "Percent" (- 1.0 (/ (LocalVariables|GetLocal%20Playback) (LocalVariables|GetLocal%20Length))) :!class /Script/Engine.MaterialInstanceDynamic)
        (Rendering|Components|TextRender|SetText (Variables|/Game/2DPlatformingKit/Widgets/Inventory_Widgets/ActionSlot.ActionSlot_C|GetCoolDownText _spell_slot) (Utilities|Text|ToText(Float) (- (LocalVariables|GetLocal%20Length) (LocalVariables|GetLocal%20Playback)) "HalfToEven" false false 1 324 0 (Math|Integer|SelectInt 1 0 (> (- (LocalVariables|GetLocal%20Length) (LocalVariables|GetLocal%20Playback)) 1.0))))
        (Variables|Default|SetCurrentTimeLinePostion (LocalVariables|GetLocal%20Playback))
        (Variables|Default|SetCurrentScalerValue (- 1.0 (/ (LocalVariables|GetLocal%20Playback) (LocalVariables|GetLocal%20Length))))))))

(fn SetupCooldown
  (params (Spell%20Slot :type Action%20Slot%20Object%20Reference) (Cooldown :type Float%20%28single-precision%29))
  (LocalVariables|SetLocal%20Cooldown Cooldown)
  (Variables|Default|SetSpell%20Slot Spell%20Slot)
  (CallFunction|SetupUMG (LocalVariables|GetLocal%20Cooldown))
  (CallFunction|SetupScaler)
  (Components|Timeline|SetTimelineLength (Variables|Default|GetCoolDown%20Time) (LocalVariables|GetLocal%20Cooldown)))

(fn SetupUMG
  (params (Cooldown :type Float%20%28single-precision%29))
  (bind _spell_slot (Variables|Default|GetSpell%20Slot))
  (LocalVariables|SetLocal%20Cooldown Cooldown)
  (Variables|/Game/2DPlatformingKit/Widgets/Inventory_Widgets/ActionSlot.ActionSlot_C|SetOnCoolDown? _spell_slot true)
  (Widget|SetIsEnabled (Variables|/Game/2DPlatformingKit/Widgets/Inventory_Widgets/ActionSlot.ActionSlot_C|GetItemBTN _spell_slot) false)
  (Appearance|SetColorandOpacity (Variables|/Game/2DPlatformingKit/Widgets/Inventory_Widgets/ActionSlot.ActionSlot_C|GetItemImage (Variables|Default|GetSpell%20Slot)) "(R=0.330000,G=0.330000,B=0.330000,A=1.000000)" :!class /Script/UMG.Image)
  (Rendering|Components|TextRender|SetText (Variables|/Game/2DPlatformingKit/Widgets/Inventory_Widgets/ActionSlot.ActionSlot_C|GetCoolDownText (Variables|Default|GetSpell%20Slot)) (Utilities|Text|ToText(Float) (LocalVariables|GetLocal%20Cooldown) "HalfToEven" false false 1 324 0 0))
  (Widget|SetVisibility (Variables|/Game/2DPlatformingKit/Widgets/Inventory_Widgets/ActionSlot.ActionSlot_C|GetCoolDownImage (Variables|Default|GetSpell%20Slot)) "SelfHitTestInvisible"))