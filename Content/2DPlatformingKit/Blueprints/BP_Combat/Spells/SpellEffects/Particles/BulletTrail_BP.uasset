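; Bullet trail effect that draws a particle beam between a start and end actor, then fades out and removes itself.
; SetTrailLocations feeds the two actors into the beam's source and target parameters.
; After a despawn delay, a timeline drives the dynamic material's "Fade Out" scalar down to zero, then calls RemoveTrail.
; RemoveTrail destroys every trail start and end point actor in the level, not just its own.
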(event Custom|Set%20Trail%20Locations
  (params (Start%20Point :type Bullet%20Trail%20Start%20Point%20Object%20Reference) (End%20Point :type Bullet%20Trail%20End%20Point%20Object%20Reference))
  (bind _particlesystem (Variables|Default|GetParticleSystem))
  ;[1 1 1] Beam Data
  (Effects|Components|ParticleSystem|SetActorParameter _particlesystem "Beam Source" Start%20Point)
  (Effects|Components|ParticleSystem|SetActorParameter _particlesystem "Beam Target" End%20Point))

(event EventBeginPlay
  ;[1 1 1] Fade Out
  (bind _returnvalue (Rendering|Material|CreateDynamicMaterialInstance (Variables|Default|GetParticleSystem) 0 (Rendering|Material|GetMaterial (Variables|Default|GetParticleSystem) 0) "None" :!class /Script/Engine.PrimitiveComponent))
  (Utilities|FlowControl|Delay (Variables|Default|GetDespawn%20Delay))
  (bind _fade_out (Timeline|Fade PlayFromStart)
    (:Update
      (if (> (Math|Float|Lerp 1.0 0.0 _fade_out) 0.0)
        (Rendering|Material|SetScalarParameterValue _returnvalue "Fade Out" (Math|Float|Lerp 1.0 0.0 _fade_out) :!class /Script/Engine.MaterialInstanceDynamic)
        (else
          (Audio|Components|Audio|Stop (Variables|Default|GetFade))
          (CallFunction|RemoveTrail))))))

(fn ConstructionScript)

(fn RemoveTrail
  (bind _outactors (Actor|GetAllActorsOfClass "/Game/2DPlatformingKit/Blueprints/BP_Combat/Spells/SpellEffects/Particles/BulletTrailEndPoint.BulletTrailEndPoint_C"))
  (for _array_element _outactors
    (Actor|DestroyActor _array_element))
  (bind _outactors_2 (Actor|GetAllActorsOfClass "/Game/2DPlatformingKit/Blueprints/BP_Combat/Spells/SpellEffects/Particles/BulletTrailStartPoint.BulletTrailStartPoint_C"))
  (for _array_element_2 _outactors_2
    (Actor|DestroyActor _array_element_2))
  (Actor|DestroyActor))