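; Bullet trail effect actor for the 2D Platforming Kit that draws a particle beam between a bullet and an end point, then fades away.
; SetTrail binds the beam's source and target actors, starts timed removal and creates a dynamic material instance.
; RemoveTrail either destroys immediately or waits, then runs a timeline fading the material's Fade Out parameter.
; Both removal paths also destroy the EndPoint actor if valid.
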(event Custom|Set%20Trail
  (params (Bullet :type Bullet%20Master%20Object%20Reference))
  (bind _trail (Variables|Default|GetTrail))
  (Effects|Components|ParticleSystem|SetActorParameter (Variables|Default|GetTrail) "Beam Source" Bullet)
  (Effects|Components|ParticleSystem|SetActorParameter (Variables|Default|GetTrail) "Beam Target" (Variables|Default|GetEnd%20Point))
  (CallFunction|RemoveTrail false)
  (bind _returnvalue (Rendering|Material|CreateDynamicMaterialInstance _trail 0 (Rendering|Material|GetMaterial _trail 0) "None" :!class /Script/Engine.PrimitiveComponent))
  (Variables|Default|SetMat _returnvalue))

(event Custom|Remove%20Trail
  (params (Instant? :type Boolean))
  (if Instant?
    (Utilities|IsValid (Variables|Default|GetEnd%20Point)
      (:Is%20Valid
        (Actor|DestroyActor (Variables|Default|GetEnd%20Point)))
      (:Is%20Not%20Valid
        _))
    (Actor|DestroyActor)
    (else
      (Utilities|FlowControl|Delay (Variables|Default|GetTrail%20Depawn%20Delay))
      (bind _float_track (Timeline|FadeTime PlayFromStart)
        (:Update
          (Rendering|Material|SetScalarParameterValue (Variables|Default|GetMat) "Fade Out" (Math|Float|Lerp 1.0 0.0 _float_track) :!class /Script/Engine.MaterialInstanceDynamic))
        (:Finished
          (Utilities|IsValid (Variables|Default|GetEnd%20Point)
            (:Is%20Valid
              (Actor|DestroyActor (Variables|Default|GetEnd%20Point))
              (Actor|DestroyActor))
            (:Is%20Not%20Valid
              (Actor|DestroyActor))))))))

(fn ConstructionScript)