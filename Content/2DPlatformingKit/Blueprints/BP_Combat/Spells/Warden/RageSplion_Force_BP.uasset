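; A Warden spell actor that fires a one-shot radial force impulse on spawn, then destroys itself after a despawn delay.
; Its construction script copies radius, force and impulse strength variables onto the RadialForce component.
; At BeginPlay it clears LaunchPlayer if any Master_Enemy_AI is very close to the player.
; That flag adds or removes one object type, apparently the player's, from those the impulse affects.
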(event EventBeginPlay
  (bind _asplayer_character (Utilities|Casting|CastToPlayer_Character (Game|GetPlayerCharacter 0)))
  (Variables|Default|SetPlayer%20Ref _asplayer_character)
  (bind _outactors (Actor|GetAllActorsOfClass "/Game/2DPlatformingKit/Blueprints/BP_Enemies/General/Master_Enemy_AI.Master_Enemy_AI_C"))
  (for _array_element _outactors
    (if (<= (Transformation|GetDistanceTo _array_element (Variables|Default|GetPlayer%20Ref)) 1e+02)
      (Variables|Default|SetLaunch%20Player? false)))
  (if (Variables|Default|GetLaunch%20Player?)
    (Class|RadialForceComponent|AddObjectTypetoAffect (Variables|Default|GetRadialForce) "ObjectTypeQuery14")
    (else
      (Class|RadialForceComponent|RemoveObjectTypetoAffect (Variables|Default|GetRadialForce) "ObjectTypeQuery14")))
  (Class|RadialForceComponent|FireImpulse (Variables|Default|GetRadialForce))
  (Utilities|FlowControl|Delay (Variables|Default|GetDespawn%20Delay))
  (Actor|DestroyActor))

(fn ConstructionScript
  (Variables|/Script/Engine.RadialForceComponent|SetForceStrength (Variables|Default|GetRadialForce) (Variables|Default|GetForce%20Strength))
  (Variables|/Script/Engine.RadialForceComponent|SetRadius (Variables|Default|GetRadialForce) (Variables|Default|GetRadius))
  (Variables|/Script/Engine.RadialForceComponent|SetImpulseStrength (Variables|Default|GetRadialForce) (Variables|Default|GetImpluse%20Strength)))