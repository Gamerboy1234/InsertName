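; Warden spell actor for the 2D Platforming Kit that emits a one-shot radial push when spawned.
; The construction script copies the exposed force strength, radius and impulse strength variables onto its RadialForce component.
; On BeginPlay it fires the impulse, then sets its lifespan so it destroys itself after the despawn delay.
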(event EventBeginPlay
  (Class|RadialForceComponent|FireImpulse (Variables|Default|GetRadialForce))
  (Actor|SetLifeSpan (Variables|Default|GetDespawn%20Delay)))

(fn ConstructionScript
  (Variables|/Script/Engine.RadialForceComponent|SetForceStrength (Variables|Default|GetRadialForce) (Variables|Default|GetForce%20Strength))
  (Variables|/Script/Engine.RadialForceComponent|SetRadius (Variables|Default|GetRadialForce) (Variables|Default|GetRadius))
  (Variables|/Script/Engine.RadialForceComponent|SetImpulseStrength (Variables|Default|GetRadialForce) (Variables|Default|GetImpluse%20Strength)))