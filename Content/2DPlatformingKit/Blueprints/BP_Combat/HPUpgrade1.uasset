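; HPUpgrade1 is an inventory item that raises the player's current and maximum health when used.
; It caches the Player_Character on BeginPlay, then on ItemUsed shows a screen message if max HP has already reached the hardcoded cap.
; Otherwise it adds its configured amounts through HPUpgrade, refreshes the HUD health bar, and destroys itself if removing one from its inventory slot succeeds.
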(event EventBeginPlay
  (bind _asplayer_character (Utilities|Casting|CastToPlayer_Character (Game|GetPlayerCharacter 0)))
  (Variables|Default|SetPlayer%20Ref _asplayer_character))

(event EventItemUsed
  (bind _player_ref (Variables|Default|GetPlayer%20Ref))
  (if (>= (Variables|/Game/2DPlatformingKit/Blueprints/Player/Player_Character.Player_Character_C|GetMaxHP (Variables|Default|GetPlayer%20Ref)) 1e+02)
    (Utilities|UIScreenText "HP already at max")
    (else
      (Default|HPUpgrade _player_ref (+ (Variables|/Game/2DPlatformingKit/Blueprints/Player/Player_Character.Player_Character_C|GetPlayer%20HP _player_ref) (Variables|Default|GetHP%20To%20Add)) (+ (Variables|/Game/2DPlatformingKit/Blueprints/Player/Player_Character.Player_Character_C|GetMaxHP _player_ref) (Variables|Default|GetMaxHP%20To%20Add)))
      (Default|UpdateHealthBar (Variables|/Game/2DPlatformingKit/Blueprints/BP_Inventory/Blueprints/Inventory_Master.Inventory_Master_C|GetHUD (Variables|Default|GetInventory)))
      (bind _success (Default|RemoveItematIndex (Variables|Default|GetInventory) (Variables|Default|GetIndex) 1 false))
      (if _success
        (Actor|DestroyActor)))))

(fn ConstructionScript
  (|CallParentFunction))