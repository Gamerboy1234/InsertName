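; MasterWeapon is a base weapon actor for a 2D platformer that displays a configurable Paper2D sprite and manages energy-gated use.
; It caches the player character on BeginPlay and provides an event that pushes its current and maximum energy to the player.
; A use check compares the player's energy to the item's cost, blocks use while the crafting menu is open, and shows an on-screen warning when energy is short.
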(event Custom|Set%20Weapon%20Energy
  (Default|SetWeaponEngergy (Variables|Default|GetPlayer%20Ref) (Variables|Default|GetCurrent%20Weapon%20Energy) (Variables|Default|GetMax%20Weapon%20Energy)))

(event EventBeginPlay
  (bind _asplayer_character (Utilities|Casting|CastToPlayer_Character (Game|GetPlayerCharacter 0)))
  (Variables|Default|SetPlayer%20Ref _asplayer_character))

(fn ConstructionScript
  (|CallParentFunction)
  (Rendering|Components|Sprite|SetSprite (Variables|Default|GetPaperSprite) (Variables|Default|GetWeapon%20Sprite)))

(fn CanUseWeapon?
  (params (Item%20Info :type S%20Item%20Info%20Structure))
  (if (>= (Variables|/Game/2DPlatformingKit/Blueprints/Player/Player_Character.Player_Character_C|GetCurrent%20Weapon%20Energy (Variables|Default|GetPlayer%20Ref)) (Utilities|Struct|BreakS_ItemInfo Item%20Info))
    (if (not (Variables|/Game/2DPlatformingKit/Widgets/Inventory_Widgets/Inventory.Inventory_C|GetIs%20Crafting%20Menu%20Open? (Variables|/Game/2DPlatformingKit/Widgets/Player_Widgets/HUD.HUD_C|GetInventoryWidget (Variables|/Game/2DPlatformingKit/Blueprints/BP_Inventory/Blueprints/Inventory_Master.Inventory_Master_C|GetHUD (Variables|/Game/2DPlatformingKit/Blueprints/Player/Player_Character.Player_Character_C|GetInventory%20Ref (Variables|Default|GetPlayer%20Ref))))))
      (Variables|Default|SetCan%20Use? true)
      (Variables|Default|SetIn%20Use? true)
      (else
        (Variables|Default|SetCan%20Use? false)
        (Variables|Default|SetIn%20Use? false)))
    (else
      (Variables|Default|SetCan%20Use? false)
      (Variables|Default|SetIn%20Use? false)
      (Utilities|UIScreenText "Not enough energy"))))