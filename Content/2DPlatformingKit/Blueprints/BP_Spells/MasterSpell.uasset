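; MasterSpell is the base spell Blueprint that handles casting and cooldown for the player character in the 2D platforming kit.
; A cast attempt checks cooldown and casting state, notifies the player, then completes instantly or after a timeline-driven HUD cast bar.
; A separate CoolDown event, not called within this graph, runs a timeline that greys out the hotkey slot and drives its material sweep and countdown text until reset.
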(event Custom|On%20Try%20Cast
  ;[1 1 1] Initial Code that sees if you can cast
  (if (and (not (Variables|/Game/2DPlatformingKit/Widgets/Inventory_Widgets/HotKeySlot.HotKeySlot_C|GetDeactivated? (Variables|Misc|GetHotkey%20Slot))) (Variables|SpellBool's|GetOn%20Cooldown?))
    (Utilities|UIScreenText "On Cooldown")
    (elif (and (not (Variables|/Game/2DPlatformingKit/Blueprints/Player/Player_Character.Player_Character_C|GetIs%20Casting? (Variables|Misc|GetPlayer%20Ref))) (not (Variables|SpellBool's|GetCurrently%20Casting)))
      (CallFunction|InInitializeSpellCast))))

(event Custom|InInitialize%20Spell%20Cast
  ;[1 1 1] Starts Casting the Spell
  (Variables|SpellBool's|SetCurrently%20Casting true)
  (Default|BeginCast (Variables|Misc|GetPlayer%20Ref) self)
  (CallFunction|OnSpellCast))

(event Custom|On%20Spell%20Cast
  ;[1 1 1] Spell Effects
  (if (Utilities|Struct|BreakS_ItemInfo (Variables|Default|GetItem%20Info))
    (CallFunction|HasCastBar)
    (else
      (CallFunction|OnCastCompleted))))

(event Custom|On%20CoolDown%20Done
  (bind _hotkey_slot (Variables|Misc|GetHotkey%20Slot))
  ;[1 1 1] Reset Hotkey After Cooldown
  (Variables|SpellBool's|SetOn%20Cooldown? false)
  (Utilities|IsValid _hotkey_slot
    (:Is%20Valid
      (if (Variables|/Game/2DPlatformingKit/Widgets/Inventory_Widgets/HotKeySlot.HotKeySlot_C|GetDeactivated? _hotkey_slot)
        _
        (else
          (Appearance|SetColorandOpacity (Variables|/Game/2DPlatformingKit/Widgets/Inventory_Widgets/HotKeySlot.HotKeySlot_C|GetIcon (Variables|Misc|GetHotkey%20Slot)) "(R=1.000000,G=1.000000,B=1.000000,A=1.000000)" :!class /Script/UMG.Image)
          (Widget|SetIsEnabled (Variables|/Game/2DPlatformingKit/Widgets/Inventory_Widgets/HotKeySlot.HotKeySlot_C|GetItemButton (Variables|Misc|GetHotkey%20Slot)) true)))
      (Widget|SetVisibility (Variables|/Game/2DPlatformingKit/Widgets/Inventory_Widgets/HotKeySlot.HotKeySlot_C|GetCooldownText (Variables|Misc|GetHotkey%20Slot)) "Hidden"))))

(event Custom|CoolDown
  (bind _hotkey_slot (Variables|Misc|GetHotkey%20Slot))
  (bind _item_info (Variables|Default|GetItem%20Info))
  (bind _cooldown_timeline (Variables|Default|GetCoolDown%20Timeline))
  (bind _hotkey_slot_2 (Variables|Misc|GetHotkey%20Slot))
  (bind _cooldown (Utilities|Struct|BreakS_ItemInfo _item_info))
  (bind _returnvalue (Components|Timeline|GetPlaybackPosition _cooldown_timeline))
  (bind _returnvalue_2 (Components|Timeline|GetTimelineLength _cooldown_timeline))
  (bind _returnvalue_3 (- _returnvalue_2 _returnvalue))
  ;[1 1 1] Cool Down code
  (Variables|SpellBool's|SetOn%20Cooldown? true)
  (Utilities|IsValid (Variables|Misc|GetHotkey%20Slot)
    (:Is%20Valid
      (Widget|SetIsEnabled (Variables|/Game/2DPlatformingKit/Widgets/Inventory_Widgets/HotKeySlot.HotKeySlot_C|GetItemButton _hotkey_slot) false)
      (Appearance|SetColorandOpacity (Variables|/Game/2DPlatformingKit/Widgets/Inventory_Widgets/HotKeySlot.HotKeySlot_C|GetIcon _hotkey_slot) "(R=0.330000,G=0.330000,B=0.330000,A=0.800000)" :!class /Script/UMG.Image)
      (Rendering|Material|SetScalarParameterValue (Variables|/Game/2DPlatformingKit/Widgets/Inventory_Widgets/HotKeySlot.HotKeySlot_C|GetCoolDown%20Mat _hotkey_slot) "Percent" 1.0 :!class /Script/Engine.MaterialInstanceDynamic)
      (Rendering|Components|TextRender|SetText (Variables|/Game/2DPlatformingKit/Widgets/Inventory_Widgets/HotKeySlot.HotKeySlot_C|GetCooldownText _hotkey_slot) (Utilities|Text|ToText(Float) _cooldown "HalfToEven" false false 1 324 0 0))
      (Widget|SetVisibility (Variables|/Game/2DPlatformingKit/Widgets/Inventory_Widgets/HotKeySlot.HotKeySlot_C|GetCoolDownImage _hotkey_slot) "SelfHitTestInvisible"))
    (:Is%20Not%20Valid
      _))
  (Components|Timeline|SetTimelineLength (Variables|Default|GetCoolDown%20Timeline) _cooldown)
  (Timeline|CoolDown%20Timeline PlayFromStart
    (:Update
      (Utilities|IsValid _hotkey_slot_2
        (:Is%20Valid
          (Rendering|Material|SetScalarParameterValue (Variables|/Game/2DPlatformingKit/Widgets/Inventory_Widgets/HotKeySlot.HotKeySlot_C|GetCoolDown%20Mat _hotkey_slot_2) "Percent" (- 1.0 (/ _returnvalue _returnvalue_2)) :!class /Script/Engine.MaterialInstanceDynamic)
          (Rendering|Components|TextRender|SetText (Variables|/Game/2DPlatformingKit/Widgets/Inventory_Widgets/HotKeySlot.HotKeySlot_C|GetCooldownText _hotkey_slot_2) (Utilities|Text|ToText(Float) _returnvalue_3 "HalfToEven" false false 1 324 0 (select (> _returnvalue_3 1.0) 0 1))))))
    (:Finished
      (CallFunction|OnCoolDownDone))))

(event Custom|On%20Cast%20Completed
  ;[1 1 1] Ends Cast and what you want the spell do at the end of cast
  (Variables|SpellBool's|SetCurrently%20Casting false)
  (Default|EndCast (Variables|Misc|GetPlayer%20Ref) self))

(event Custom|Has%20Cast%20Bar
  ;[1 1 1] Cast Bar
  (Utilities|FlowControl|DoOnce false :!label _label
    (:Completed
      (Components|Timeline|SetTimelineLength (Variables|Default|GetCast%20Time%20Line) (Utilities|Struct|BreakS_ItemInfo (Variables|Default|GetItem%20Info)))
      (Widget|SetVisibility (Variables|/Game/2DPlatformingKit/Widgets/Player_Widgets/HUD.HUD_C|GetCastBarOverlay (Variables|/Game/2DPlatformingKit/Blueprints/Inventory/Blueprints/Inventory_Master.Inventory_Master_C|GetHUD (Variables|/Game/2DPlatformingKit/Blueprints/Player/Player_Character.Player_Character_C|GetInventory%20Ref (Variables|Misc|GetPlayer%20Ref)))) "HitTestInvisible")
      (Widget|SetVisibility (Variables|/Game/2DPlatformingKit/Widgets/Player_Widgets/HUD.HUD_C|GetCastbar (Variables|/Game/2DPlatformingKit/Blueprints/Inventory/Blueprints/Inventory_Master.Inventory_Master_C|GetHUD (Variables|/Game/2DPlatformingKit/Blueprints/Player/Player_Character.Player_Character_C|GetInventory%20Ref (Variables|Misc|GetPlayer%20Ref)))) "Visible")
      (Widget|SetVisibility (Variables|/Game/2DPlatformingKit/Widgets/Player_Widgets/HUD.HUD_C|GetSpellName (Variables|/Game/2DPlatformingKit/Blueprints/Inventory/Blueprints/Inventory_Master.Inventory_Master_C|GetHUD (Variables|/Game/2DPlatformingKit/Blueprints/Player/Player_Character.Player_Character_C|GetInventory%20Ref (Variables|Misc|GetPlayer%20Ref)))) "Visible")
      (Timeline|Cast%20Time%20Line PlayFromStart
        (:Update
          (Progress|SetPercent (Variables|/Game/2DPlatformingKit/Widgets/Player_Widgets/HUD.HUD_C|GetCastbar (Variables|/Game/2DPlatformingKit/Blueprints/Inventory/Blueprints/Inventory_Master.Inventory_Master_C|GetHUD (Variables|/Game/2DPlatformingKit/Blueprints/Player/Player_Character.Player_Character_C|GetInventory%20Ref (Variables|Misc|GetPlayer%20Ref)))) (/ (Components|Timeline|GetPlaybackPosition (Variables|Default|GetCast%20Time%20Line)) (Utilities|Struct|BreakS_ItemInfo (Variables|Default|GetItem%20Info))))
          (Rendering|Components|TextRender|SetText (Variables|/Game/2DPlatformingKit/Widgets/Player_Widgets/HUD.HUD_C|GetSpellName (Variables|/Game/2DPlatformingKit/Blueprints/Inventory/Blueprints/Inventory_Master.Inventory_Master_C|GetHUD (Variables|/Game/2DPlatformingKit/Blueprints/Player/Player_Character.Player_Character_C|GetInventory%20Ref (Variables|Misc|GetPlayer%20Ref)))) (Utilities|Text|FormatText "Casting - {SpellName}" (Utilities|Struct|BreakS_ItemInfo (Variables|Default|GetItem%20Info)))))
        (:Finished
          (Variables|SpellBool's|SetIs%20Cast%20Done? true)
          (Widget|SetVisibility (Variables|/Game/2DPlatformingKit/Widgets/Player_Widgets/HUD.HUD_C|GetCastBarOverlay (Variables|/Game/2DPlatformingKit/Blueprints/Inventory/Blueprints/Inventory_Master.Inventory_Master_C|GetHUD (Variables|/Game/2DPlatformingKit/Blueprints/Player/Player_Character.Player_Character_C|GetInventory%20Ref (Variables|Misc|GetPlayer%20Ref)))) "Hidden")
          (Widget|SetVisibility (Variables|/Game/2DPlatformingKit/Widgets/Player_Widgets/HUD.HUD_C|GetCastbar (Variables|/Game/2DPlatformingKit/Blueprints/Inventory/Blueprints/Inventory_Master.Inventory_Master_C|GetHUD (Variables|/Game/2DPlatformingKit/Blueprints/Player/Player_Character.Player_Character_C|GetInventory%20Ref (Variables|Misc|GetPlayer%20Ref)))) "Hidden")
          (Widget|SetVisibility (Variables|/Game/2DPlatformingKit/Widgets/Player_Widgets/HUD.HUD_C|GetSpellName (Variables|/Game/2DPlatformingKit/Blueprints/Inventory/Blueprints/Inventory_Master.Inventory_Master_C|GetHUD (Variables|/Game/2DPlatformingKit/Blueprints/Player/Player_Character.Player_Character_C|GetInventory%20Ref (Variables|Misc|GetPlayer%20Ref)))) "Visible")
          (CallFunction|OnCastCompleted)
          (goto _label Reset))))))

(event EventBeginPlay
  ;[1 1 1] Get Player Ref
  (bind _asplayer_character (Utilities|Casting|CastToPlayer_Character (Game|GetPlayerCharacter 0)))
  (Variables|Misc|SetPlayer%20Ref _asplayer_character))

(fn ConstructionScript
  (|CallParentFunction))