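; RageUpgrade is an inventory item that, when used, raises the player's current and maximum Rage.
; It caches the Player_Character reference on BeginPlay.
; ItemUsed passes the current values plus the configured increments to the player's UpgradeRage, then removes one item from the inventory without spawning a drop.
; The actor destroys itself only if that removal returns true, though the upgrade is applied regardless.
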(event EventBeginPlay
  (bind _asplayer_character (Utilities|Casting|CastToPlayer_Character (Game|GetPlayerCharacter 0)))
  (Variables|Default|SetPlayer%20Ref _asplayer_character))

(event EventItemUsed
  (bind _player_ref (Variables|Default|GetPlayer%20Ref))
  (Default|UpgradeRage (Variables|Default|GetPlayer%20Ref) (+ (Variables|/Game/2DPlatformingKit/Blueprints/Player/Player_Character.Player_Character_C|GetCurrent%20Rage _player_ref) (Variables|Default|GetRage%20to%20Add)) (+ (Variables|/Game/2DPlatformingKit/Blueprints/Player/Player_Character.Player_Character_C|GetMax%20Rage _player_ref) (Variables|Default|GetMax%20Rage%20to%20Add)))
  (bind _success (Default|RemoveItematIndex (Variables|Default|GetInventory) (Variables|Default|GetIndex) 1 false))
  (if _success
    (Actor|DestroyActor)))

(fn ConstructionScript
  (|CallParentFunction))