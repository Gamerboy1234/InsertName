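; SpellAdder is a usable item that teaches the player a configured spell in the 2D platforming kit.
; On BeginPlay it caches the Player_Character reference.
; When used, it checks the player's spell array for SpellToAdd, then either adds the spell and passes it to AssignNewSpells, or shows an already-known message.
; A Success flag records whether the spell was learned.
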(event EventBeginPlay
  (bind _asplayer_character (Utilities|Casting|CastToPlayer_Character (Game|GetPlayerCharacter 0)))
  (Variables|Default|SetPlayer%20Ref _asplayer_character))

(event EventItemUsed
  (if (not (CallFunction|AlreadyKnowSpell? (Variables|Default|GetSpell%20to%20Add)))
    (Utilities|Array|Add (Variables|/Game/2DPlatformingKit/Blueprints/Player/Player_Character.Player_Character_C|GetSpell%20Arrary (Variables|Default|GetPlayer%20Ref)) (Variables|Default|GetSpell%20to%20Add))
    (Default|AssignNewSpells (Variables|Default|GetPlayer%20Ref) (Utilities|Array|MakeArray (Variables|Default|GetSpell%20to%20Add)))
    (Variables|Default|SetSuccess? true)
    (else
      (Utilities|UIScreenText "Already know this spell")
      (Variables|Default|SetSuccess? false))))

(fn ConstructionScript
  (|CallParentFunction))

(fn AlreadyKnowSpell?
  (params (Spell :type Master%20Spell%20Class%20Reference))
  (if (> (Utilities|Array|FindItem (Variables|/Game/2DPlatformingKit/Blueprints/Player/Player_Character.Player_Character_C|GetSpell%20Arrary (Variables|Default|GetPlayer%20Ref)) Spell) -1)
    (return true)
    (else
      (return false))))