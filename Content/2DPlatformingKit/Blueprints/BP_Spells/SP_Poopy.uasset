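; SP_Poopy is a player spell that drops a damaging POOP actor from behind the caster.
; Casting completes immediately, since OnSpellCast calls OnCastCompleted directly.
; Completion starts the cooldown, clears the casting flag, spawns POOP at the player's BackAim transform with fixed damage and an extremely large despawn delay, then ends the player's cast.
; BeginPlay, Tick and construction only call the parent.
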(event EventBeginPlay
  (|CallParentFunction))

(event EventOnCastCompleted
  (CallFunction|CoolDown)
  (Variables|Default|SetCurrently%20Casting false)
  (Game|SpawnActorfromClass "/Game/2DPlatformingKit/Blueprints/Player/POOP.POOP_C" (Transformation|GetWorldTransform (Variables|/Game/2DPlatformingKit/Blueprints/Player/Player_Character.Player_Character_C|GetBack%20Aim (Variables|Default|GetPlayer%20Ref))) "Undefined" 0 1e+01 4.87002067341987e+18 0.0 0.0 0.0 0.0 0.0 0.75 0)
  (Default|EndCast (Variables|Default|GetPlayer%20Ref) self))

(event EventTick
  (params (DeltaSeconds :type Float%20%28single-precision%29))
  (|CallParentFunction DeltaSeconds))

(event EventOnSpellCast
  (CallFunction|OnCastCompleted))

(fn ConstructionScript
  (|CallParentFunction))