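; Ranged Paper2D enemy for the 2D platformer that turns toward the player and throws spears, under a folder marked TOBEDELETED.
; Tick drives flipbook switching and either delayed spear spawning with HP bar updates or line-trace searches for dropped spears.
; Damage is full or halved depending on spear count and aggro, and shows floating text.
; Looping-timer damage over time can be cashed in by a Warden player through DamageCheck.
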(event Custom|Damage
  (params (Incoming%20Damage :type Float%20%28single-precision%29))
  ;[1 1 1] Damage Code
  (if (and (< (Variables|Default|GetSpearAmmount) (Variables|Default|GetmaxSpearAmount)) (Variables|Default|Getaggro))
    (Variables|HPValues|SetCurrent%20HP (- (Variables|HPValues|GetCurrent%20HP) (Variables|DamageInfo|GetIncoming%20Damage)))
    (bind _returnvalue (UserInterface|CreateWidget "/Game/2DPlatformingKit/Widgets/Player_Widgets/Floating_Text.Floating_Text_C" 0 (Variables|DamageInfo|GetIncoming%20Damage) self :!label _label))
    (UserInterface|Viewport|AddtoViewport _returnvalue 0)
    (Variables|DamageInfo|SetTaken%20Damge true)
    (if (< (Variables|HPValues|GetCurrent%20HP) 1.0)
      (Variables|Default|Setdead true)
      (Variables|DamageInfo|SetTaken%20Damge false)
      (Actor|DestroyActor))
    (elif (> Incoming%20Damage 0.0)
      (bind _output_get (Variables|DamageInfo|SetIncoming%20Damage Incoming%20Damage))
      (Variables|DamageInfo|SetIncoming%20Damage (/ _output_get 2.0))
      (Variables|HPValues|SetCurrent%20HP (- (Variables|HPValues|GetCurrent%20HP) (Variables|DamageInfo|GetIncoming%20Damage)))
      (goto _label)
      (else
        (bind _returnvalue_2 (UserInterface|CreateWidget "/Game/2DPlatformingKit/Widgets/Player_Widgets/Floating_Text.Floating_Text_C" 0 0.0 self))
        (UserInterface|Viewport|AddtoViewport _returnvalue_2 0)))))

(event Custom|Damage%20Over%20Time
  ;[1 1 1] Damage Over time
  (if (not (Variables|Default|Getdead))
    (CallFunction|Damage (Variables|DamageInfo|GetDamage%20Amount))
    (bind _result (Math|Float|DecrementFloat (Variables|DamageInfo|GetTick's%20Left))
      (:%20%20
        (if (<= _result 0.0)
          (Utilities|Time|ClearandInvalidateTimerbyHandle (Variables|DamageInfo|GetEvent%20Timer))
          (Variables|Default|SetTaken%20Damage%20over%20Time? false)
          (Utilities|IsValid (Variables|DamageInfo|GetDamage%20Over%20Time%20Actor)
            (:Is%20Valid
              (Actor|DestroyActor (Variables|DamageInfo|GetDamage%20Over%20Time%20Actor)))))))
    (else
      (Utilities|Time|ClearandInvalidateTimerbyHandle (Variables|DamageInfo|GetEvent%20Timer))
      (Variables|Default|SetTaken%20Damage%20over%20Time? false)
      (Utilities|IsValid (Variables|DamageInfo|GetDamage%20Over%20Time%20Actor)
        (:Is%20Valid
          (Actor|DestroyActor (Variables|DamageInfo|GetDamage%20Over%20Time%20Actor)))))))

(event Custom|Start%20Damage%20Over%20Time
  (params (Ticks :type Float%20%28single-precision%29) (Damage :type Float%20%28single-precision%29) (Attached%20Fire :type Actor%20Object%20Reference) (Occurrences :type Float%20%28single-precision%29))
  ;[1 1 1] Damage Over time
  (Variables|Default|SetTaken%20Damage%20over%20Time? true)
  (Variables|DamageInfo|SetDamage%20Amount Damage)
  (Variables|DamageInfo|SetTick's%20Left Ticks)
  (Variables|DamageInfo|SetDamage%20Over%20Time%20Actor Attached%20Fire)
  (bind _returnvalue (Utilities|Time|SetTimerbyEvent (delegate Custom|Damage%20Over%20Time) Occurrences true))
  (Variables|DamageInfo|SetEvent%20Timer _returnvalue))

(event Custom|Add%20Spears
  ;[1 1 1] Add to Spear Count
  (Math|Integer|IncrementInt (Variables|Default|GetSpearAmmount)))

(event EventBeginPlay
  ;[1 1 1] Damage Code
  (Rendering|SetVisibility (Variables|Default|GetHPBar) false false)
  (bind _asplayer_character (Utilities|Casting|CastToPlayer_Character (Game|GetPlayerCharacter 0)))
  (Variables|Default|SetPlayer%20Ref _asplayer_character))

(event EventTick
  (params (DeltaSeconds :type Float%20%28single-precision%29))
  (bind _s_bullet_damage (Variables|DamageInfo|GetS%20Bullet%20Damage))
  (bind _hpbar (Variables|Default|GetHPBar))
  (bind (_startingspeed _maxspeed _gravity _despawndelay) (Utilities|Struct|BreakS_BulletInfo _s_bullet_damage))
  (Utilities|FlowControl|Sequence
    (:then_0
      ;[1 1 1] Animation Switching
      (CallFunction|AnimationStateMachine))
    (:then_1
      ;[1 1 1] Attack Code
      (if (Variables|Default|Getfinished1)
        (CallFunction|FindDroppedSpear)
        (elif (and (< (Variables|Default|GetSpearAmmount) (Variables|Default|GetmaxSpearAmount)) (Variables|Default|Getaggro))
          (Variables|Default|SetisFiring false)
          (else
            (CallFunction|RotatetoPlayer)
            (Utilities|FlowControl|Delay (Variables|Default|GetFireRate))
            (Math|Integer|DecrementInt (Variables|Default|GetSpearAmmount)
              (:%20%20
                (Variables|Default|SetisFiring true)
                (Game|SpawnActorfromClass "/Game/2DPlatformingKit/Blueprints/Player/E_Spear.E_Spear_C" (Transformation|GetWorldTransform (Variables|Default|GetArrow)) "Undefined" 0 _gravity _maxspeed _startingspeed _despawndelay (Variables|DamageInfo|GetSpear%20Damage) 0)
                ;[1 1 1] HP Bar Code
                (if (Variables|DamageInfo|GetTaken%20Damge)
                  (Rendering|SetVisibility _hpbar true false)
                  (Utilities|FlowControl|Delay 3.0)
                  (Rendering|SetVisibility (Variables|Default|GetHPBar) false false)
                  (Variables|DamageInfo|SetTaken%20Damge false)
                  (else
                    (Rendering|SetVisibility _hpbar false false)))
                (bind _asenemy_hpbar (Utilities|Casting|CastToEnemy_HPBar (UserInterface|GetUserWidgetObject (Variables|Default|GetHPBar))))
                (Progress|SetPercent (Variables|/Game/2DPlatformingKit/Widgets/Enemy_Widgets/Enemy_HPBar.Enemy_HPBar_C|GetHPBar _asenemy_hpbar) (/ (Variables|HPValues|GetCurrent%20HP) (Variables|HPValues|GetMax%20HP)))))))))))

(fn ConstructionScript)

(fn FindDroppedSpear
  (bind _returnvalue (Game|GetPlayerCharacter 0))
  (bind _line_1 (Variables|Default|GetLine%201))
  (bind _line_2 (Variables|Default|GetLine%202))
  (bind _returnvalue_2 (Transformation|GetWorldLocation _line_1))
  (bind _returnvalue_3 (Transformation|GetWorldLocation _line_2))
  (bind _array (Utilities|Array|MakeArray _returnvalue))
  (Utilities|FlowControl|Sequence
    (:then_0
      (bind _outhit (Collision|LineTraceForObjects _returnvalue_2 (+ _returnvalue_2 "1000.000000,0.000000,0.000000") (Utilities|Array|MakeArray "ObjectTypeQuery9") false _array "ForDuration"))
      (bind _outactors (Actor|GetAllActorsOfClass "/Game/2DPlatformingKit/Blueprints/Player/DroppedSpear_BP.DroppedSpear_BP_C"))
      (bind _array_element (Utilities|Array|ForEachLoopwithBreak _outactors :!label _label)
        (:LoopBody
          (if (== (.HitActor (Collision|BreakHitResult _outhit)) _array_element)
            (goto _label Break)))
        (:Completed
          (bind _output_get (LocalVariables|SetDropped%20Spear (.HitActor (Collision|BreakHitResult _outhit))))
          (Utilities|IsValid _output_get
            (:Is%20Valid
              (Variables|Default|SetSpearLocation (Transformation|GetActorLocation _output_get))
              (Variables|Default|SetSpearFound true)
              (Variables|Default|SetisRight true)
              (Variables|Default|SetisLeft false))))))
    (:then_1
      (bind _outhit_2 (Collision|LineTraceForObjects _returnvalue_3 (+ _returnvalue_3 "-1000.000000,0.000000,0.000000") (Utilities|Array|MakeArray "ObjectTypeQuery9") false _array "ForDuration"))
      (bind _outactors_2 (Actor|GetAllActorsOfClass "/Game/2DPlatformingKit/Blueprints/Player/DroppedSpear_BP.DroppedSpear_BP_C"))
      (bind _array_element_2 (Utilities|Array|ForEachLoopwithBreak _outactors_2 :!label _label_2)
        (:LoopBody
          (if (== (.HitActor (Collision|BreakHitResult _outhit_2)) _array_element_2)
            (goto _label_2 Break)))
        (:Completed
          (bind _output_get_2 (LocalVariables|SetDropped%20Spear (.HitActor (Collision|BreakHitResult _outhit_2))))
          (Utilities|IsValid _output_get_2
            (:Is%20Valid
              (Variables|Default|SetSpearLocation (Transformation|GetActorLocation _output_get_2))
              (Variables|Default|SetSpearFound true)
              (Variables|Default|SetisRight false)
              (Variables|Default|SetisLeft true))))))))

(fn RotatetoPlayer
  (if (> (.x (Transformation|GetActorLocation)) (.x (Transformation|GetActorLocation (Variables|Default|GetPlayer%20Ref))))
    (Transformation|SetActorRotation "0,180.000000, 0")
    (elif (< (.x (Transformation|GetActorLocation)) (.x (Transformation|GetActorLocation (Variables|Default|GetPlayer%20Ref))))
      (Transformation|SetActorRotation "0, 0, 0"))))

(fn AnimationStateMachine
  (if (Variables|Default|Getaggro)
    (if (Variables|Default|Getfinished1)
      (Sprite|SetFlipbook (Variables|Default|GetPaperFlipbook) (Variables|Animations|GetPicking%20Up%20Spear%20Animation))
      (else
        (Sprite|SetFlipbook (Variables|Default|GetPaperFlipbook) (Variables|Animations|GetAttacking%20Animation))))
    (else
      (Sprite|SetFlipbook (Variables|Default|GetPaperFlipbook) (Variables|Animations|GetIdle%20Animation)))))

(fn DamageCheck
  (params (Damage :type Float%20%28single-precision%29))
  (bind _tick_s_left (Variables|DamageInfo|GetTick's%20Left))
  (LocalVariables|SetLocal%20Damage Damage)
  (if (and (Variables|Default|GetTaken%20Damage%20over%20Time?) (Variables|/Game/2DPlatformingKit/Blueprints/Player/Player_Character.Player_Character_C|GetIs%20Warden? (Variables|Default|GetPlayer%20Ref)))
    (Utilities|Time|ClearandInvalidateTimerbyHandle (Variables|DamageInfo|GetEvent%20Timer))
    (Variables|Default|SetTaken%20Damage%20over%20Time? false)
    (Utilities|IsValid (Variables|DamageInfo|GetDamage%20Over%20Time%20Actor)
      (:Is%20Valid
        (Actor|DestroyActor (Variables|DamageInfo|GetDamage%20Over%20Time%20Actor)))
      (:Is%20Not%20Valid
        _))
    (Development|PrintString (Utilities|String|ToString(Text) (Utilities|Text|FormatText "Ticks Left: {ticks}" _tick_s_left)))
    (Development|PrintString (Utilities|String|ToString(Text) (Utilities|Text|FormatText "Damage: {ticks}" (Class|DamageIncreass|IncreaseDamage _tick_s_left (LocalVariables|GetLocal%20Damage)))))
    (CallFunction|Damage (- (Variables|HPValues|GetCurrent%20HP) (Class|DamageIncreass|IncreaseDamage _tick_s_left (LocalVariables|GetLocal%20Damage))))
    (return true)
    (else
      (return false))))