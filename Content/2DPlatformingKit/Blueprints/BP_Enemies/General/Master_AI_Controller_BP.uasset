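; Master AI controller for the 2D platforming kit's enemies, exposing action events that act on the controlled pawn.
; On BeginPlay it casts the possessed pawn to Master_Enemy and caches it as AIRef.
; ShootGun and ThrowSpear cast that reference to Shooter_E or SpearThrower before forwarding the call, while Jump calls AIJump on the base enemy directly.
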(event Custom|Shoot%20Gun
  (bind _asshooter_e (Utilities|Casting|CastToShooter_E (Variables|Default|GetAI%20Ref)))
  (Default|ShootGun _asshooter_e))

(event Custom|Throw%20Spear
  (bind _asspear_thrower (Utilities|Casting|CastToSpearThrower (Variables|Default|GetAI%20Ref)))
  (Default|ThrowSpear _asspear_thrower))

(event Custom|Jump
  (Class|MasterEnemy|AIJump (Variables|Default|GetAI%20Ref)))

(event EventBeginPlay
  (bind _asmaster_enemy (Utilities|Casting|CastToMaster_Enemy (Pawn|GetControlledPawn)))
  (Variables|Default|SetAI%20Ref _asmaster_enemy))

(fn ConstructionScript)