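; Base enemy AI character for the 2D platforming kit, holding shared movement settings and per-enemy state.
; The construction script applies gravity, acceleration and walk speed to CharacterMovement and caches the default gravity scale.
; Events let a controller trigger jumps and restore default gravity, while GravityCheck replaces gravity when it drops below a threshold.
; Getters and setters expose combat, chase, stun and status-effect state, and ApplyBuff is an empty stub.
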(event Custom|AI%20Jump
  ;[1 1 1] Call in controller to make AI Jump
  (Character|Jump))

(event Custom|Reset%20Gravity
  (Variables|/Script/Engine.CharacterMovementComponent|SetGravityScale (Variables|Character|GetCharacterMovement) (GetterFunctions|GetDefaultGravityScale))
  (Variables|Movement|SetGravity%20Scale (GetterFunctions|GetDefaultGravityScale)))

(fn ConstructionScript
  ;[1 1 1] Set Movment Vars
  (Variables|/Script/Engine.CharacterMovementComponent|SetGravityScale (Variables|Character|GetCharacterMovement) (Variables|Movement|GetGravity%20Scale))
  (Variables|/Script/Engine.CharacterMovementComponent|SetMaxAcceleration (Variables|Character|GetCharacterMovement) (Variables|Movement|GetMax%20Acceleration))
  (Variables|/Script/Engine.CharacterMovementComponent|SetMaxWalkSpeed (Variables|Character|GetCharacterMovement) (Variables|Movement|GetMax%20Walk%20Speed))
  (SetterFunctions|SetDefaultGravityScale (Variables|Movement|GetGravity%20Scale)))

(fn GravityCheck
  (params (New%20Gravity%20Scale :type Float%20%28single-precision%29))
  (LocalVariables|SetLocal%20Gravity New%20Gravity%20Scale)
  (if (< (Variables|/Script/Engine.CharacterMovementComponent|GetGravityScale (Variables|Character|GetCharacterMovement)) 0.5)
    (Variables|/Script/Engine.CharacterMovementComponent|SetGravityScale (Variables|Character|GetCharacterMovement) (LocalVariables|GetLocal%20Gravity))
    (Variables|Movement|SetGravity%20Scale (LocalVariables|GetLocal%20Gravity))))

(fn ApplyBuff)

(fn GetID
  (return (Variables|Private|GetID)))

(fn GetDefaultSpriteColor
  (return (Variables|Private|GetDefault%20Sprite%20Color)))

(fn GetIsStunned
  (return (Variables|Private|GetIs%20Stunned?)))

(fn GetStunDuration
  (return (Variables|Private|GetStun%20Duration)))

(fn GetWarlustAlreadyApplied?
  (return (Variables|Private|GetWarlust%20Already%20Applied?)))

(fn GetWarlustEffect
  (return (Variables|Private|GetWarlust%20Effect)))

(fn GetHomeLocation
  (return (Variables|Private|GetHome%20Location)))

(fn GetIsJumping?
  (return (Variables|Private|GetIs%20Jumping?)))

(fn GetIsonFire?
  (return (Variables|Private|GetIs%20on%20Fire?)))

(fn GetDidEnemyTouchMagnet?
  (return (Variables|Private|GetDid%20Enemy%20Touch%20Magnet?)))

(fn GetDefaultSpeed
  (return (Variables|Private|GetDefault%20Speed)))

(fn GetDefaultMaxAcceleration
  (return (Variables|Private|GetDefault%20Max%20Acceleration)))

(fn GetCurrentAttachedLeech
  (return (Variables|Private|GetCurrent%20Attached%20Leech)))

(fn GetChasingPlayer?
  (return (Variables|Private|GetChasing%20Player?)))

(fn GetChasingPlayerTimer
  (return (Variables|Private|GetChase%20Timer)))

(fn GetIsPlayeronEnemy?
  (return (Variables|Private|GetIs%20Player%20On%20Enemy?)))

(fn GetDefaultGravityScale
  (return (Variables|Private|GetDefault%20Gravity%20Scale)))

(fn GetHitActor
  (return (Variables|Private|GetHit%20Actor)))

(fn GetWasKnockedBack?
  (return (Variables|Private|GetWas%20knocked%20backed?)))

(fn SetID
  (params (ID :type Integer))
  (Variables|Private|SetID ID))

(fn SetDefaultSpriteColor
  (params (Default%20Sprite%20Color :type Linear%20Color%20Structure))
  (Variables|Private|SetDefault%20Sprite%20Color Default%20Sprite%20Color))

(fn SetIsStunned?
  (params (Is%20Stunned? :type Boolean))
  (Variables|Private|SetIs%20Stunned? Is%20Stunned?))

(fn GetPlayerRef
  (return (Variables|Private|GetPlayer%20Ref)))

(fn SetStunDuration
  (params (Stun%20Duration :type Float%20%28single-precision%29))
  (Variables|Private|SetStun%20Duration Stun%20Duration))

(fn SetWarlustAlreadyApplied?
  (params (Warlust%20Already%20Applied? :type Boolean))
  (Variables|Private|SetWarlust%20Already%20Applied? Warlust%20Already%20Applied?))

(fn SetWarlustEffect
  (params (Warlust%20Effect :type Warlust%20Effect%20BP%20Object%20Reference))
  (Variables|Private|SetWarlust%20Effect Warlust%20Effect))

(fn GetTakenDamage?
  (return (Variables|Private|GetTaken%20Damage?)))

(fn GetHitPlayerOnce?
  (return (Variables|Private|GetHit%20Player%20Once?)))

(fn GetIsDead?
  (return (Variables|Private|GetIs%20Dead?)))

(fn SetHomeLocation
  (params (Home%20Location :type Vector))
  (Variables|Private|SetHome%20Location Home%20Location))

(fn SetIsJumping?
  (params (Is%20Jumping? :type Boolean))
  (Variables|Private|SetIs%20Jumping? Is%20Jumping?))

(fn SetIsonFire?
  (params (Is%20On%20Fire? :type Boolean))
  (Variables|Private|SetIs%20on%20Fire? Is%20On%20Fire?))

(fn SetDidEnemyTouchMagnet?
  (params (Did%20Enemy%20Touch%20Magnet? :type Boolean))
  (Variables|Private|SetDid%20Enemy%20Touch%20Magnet? Did%20Enemy%20Touch%20Magnet?))

(fn SetDefaultSpeed
  (params (Default%20Speed :type Float%20%28single-precision%29))
  (Variables|Private|SetDefault%20Speed Default%20Speed))

(fn SetDefaultMaxAcceleration
  (params (Default%20Max%20Acceleration :type Float%20%28single-precision%29))
  (Variables|Private|SetDefault%20Max%20Acceleration Default%20Max%20Acceleration))

(fn SetCurrentAttachedLeech
  (params (Current%20Attached%20Leech :type Beetle%20Leech%20DB%20E%20Object%20Reference))
  (Variables|Private|SetCurrent%20Attached%20Leech Current%20Attached%20Leech))

(fn SetChasingPlayer?
  (params (Chasing%20Player? :type Boolean))
  (Variables|Private|SetChasing%20Player? Chasing%20Player?))

(fn SetChasingPlayerTimer
  (params (Chase%20Timer :type Timer%20Handle%20Structure))
  (Variables|Private|SetChase%20Timer Chase%20Timer))

(fn SetIsPlayeronEnemy?
  (params (Player%20On%20Enemy? :type Boolean))
  (Variables|Private|SetIs%20Player%20On%20Enemy? Player%20On%20Enemy?))

(fn SetDefaultGravityScale
  (params (Default%20Gravity%20Scale :type Float%20%28single-precision%29))
  (Variables|Private|SetDefault%20Gravity%20Scale Default%20Gravity%20Scale))

(fn SetHitActor
  (params (Hit%20Actor :type Actor%20Object%20Reference))
  (Variables|Private|SetHit%20Actor Hit%20Actor))

(fn SetWasKnockedBack?
  (params (Was%20knocked%20backed? :type Boolean))
  (Variables|Private|SetWas%20knocked%20backed? Was%20knocked%20backed?))

(fn SetHitPlayerOnce?
  (params (Hit%20Player%20Once? :type Boolean))
  (Variables|Private|SetHit%20Player%20Once? Hit%20Player%20Once?))

(fn SetTakenDamage?
  (params (Taken%20Damage? :type Boolean))
  (Variables|Private|SetTaken%20Damage? Taken%20Damage?))

(fn SetPlayerRef
  (params (Player%20Ref :type Player%20Character%20Object%20Reference))
  (Variables|Private|SetPlayer%20Ref Player%20Ref))

(fn SetIsDead?
  (params (Is%20Dead? :type Boolean))
  (Variables|Private|SetIs%20Dead? Is%20Dead?))

(fn GetOverlapedPlayer?
  (return (Variables|Private|GetOverlaped%20Player?)))

(fn SetOverlapedPlayer
  (params (Overlaped%20Player? :type Boolean))
  (Variables|Private|SetOverlaped%20Player? Overlaped%20Player?))