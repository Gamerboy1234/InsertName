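; BP_PowerUp is a 2D pickup that grants the player a selected power-up for a set duration.
; On collision overlap with player character 0, it sends GrantPowerUpMessage with the power-up and duration, then plays a pickup sound at the flipbook's location.
; After a brief delay it disables collision, destroys the flipbook sprite and sets a short lifespan so the actor removes itself.
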(event OnComponentBeginOverlap(Collision)
  (params (OverlappedComponent :type Primitive%20Component%20Object%20Reference) (OtherActor :type Actor%20Object%20Reference) (OtherComp :type Primitive%20Component%20Object%20Reference) (OtherBodyIndex :type Integer) (bFromSweep :type Boolean) (SweepResult :type Hit%20Result%20Structure%20%28by%20ref%29))
  (bind _returnvalue (Game|GetPlayerCharacter 0))
  ;[1 1 1] Grant power-up when overlapping with player then destroy the object.
  (if (== OtherActor _returnvalue)
    (Class|InteractionHandler|GrantPowerUp(Message) _returnvalue (Variables|Default|GetPowerUpSelection) (Variables|Default|GetPowerUpDuration))
    (Audio|PlaySoundatLocation (Variables|Default|GetPickupSFX) (Transformation|GetWorldLocation (Variables|Default|GetPaperFlipbook)) "0, 0, 0" 1.0 1.0 0.0 0 0 0)
    (Utilities|FlowControl|Delay 0.1)
    (Collision|SetCollisionEnabled (Variables|Default|GetCollision) "NoCollision")
    (Components|DestroyComponent (Variables|Default|GetPaperFlipbook))
    (Actor|SetLifeSpan 2.0)))

(event EventActorBeginOverlap
  (params (OtherActor :type Actor%20Object%20Reference)))

(event EventTick
  (params (DeltaSeconds :type Float%20%28single-precision%29)))

(fn ConstructionScript)