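; Enemy ID tracker for the 2D platforming kit that generates random numeric IDs and records them in an IDs list.
; GenNumber adds a random number through AddIDToList before its Contains check, so it normally removes that number and rolls another.
; The second number is stored and returned without a duplicate check, so uniqueness is not guaranteed.
; The random call's Min and Max values appear swapped.
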(fn ConstructionScript)

(fn AddIDtoList
  (params (ID :type Integer))
  (Utilities|Array|Add (Variables|Default|GetID's) ID))

(fn GenNumber
  (bind _output_get (LocalVariables|SetLocal%20Number (Class|RandomNumberNoRepeat|RandomNumber 1 100000)))
  (CallFunction|AddIDtoList _output_get)
  (if (Utilities|Array|ContainsItem (Variables|Default|GetID's) (LocalVariables|GetLocal%20Number))
    (bind _returnvalue (Utilities|Array|RemoveItem (Variables|Default|GetID's) (LocalVariables|GetLocal%20Number)))
    (if _returnvalue
      (bind _output_get_2 (LocalVariables|SetLocal%20Number (Class|RandomNumberNoRepeat|RandomNumber 1 100000)))
      (CallFunction|AddIDtoList _output_get_2)
      (return (LocalVariables|GetLocal%20Number)))
    (else
      (return (LocalVariables|GetLocal%20Number)))))