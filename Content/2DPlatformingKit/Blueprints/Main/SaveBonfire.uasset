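; SaveBonfire is a checkpoint actor in the 2D platforming kit that saves the game when the player overlaps its box.
; The box's collision stays off for one second after BeginPlay to avoid spurious triggers.
; On overlap it shows a text label for a second, caches the player reference and writes a freshly created SaveGamePlayer to its default slot, printing the result.
; No player data is copied into the save object here.
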(event OnComponentBeginOverlap(Box)
  (params (OverlappedComponent :type Primitive%20Component%20Object%20Reference) (OtherActor :type Actor%20Object%20Reference) (OtherComp :type Primitive%20Component%20Object%20Reference) (OtherBodyIndex :type Integer) (bFromSweep :type Boolean) (SweepResult :type Hit%20Result%20Structure%20%28by%20ref%29))
  (bind _returnvalue (Game|GetPlayerCharacter 0))
  ;[1 1 1] Save the game when overlapping the bonfire collision box.
  (if (== OtherActor _returnvalue)
    (Rendering|SetVisibility (Variables|Components|GetTextRender) true false)
    (bind _asplayer_character (Utilities|Casting|CastToPlayer_Character _returnvalue))
    (Variables|Default|SetPlayerReference _asplayer_character)
    (bind _returnvalue_2 (SaveGame|CreateSaveGameObject "/Game/2DPlatformingKit/Blueprints/Main/SaveGamePlayer.SaveGamePlayer_C"))
    (bind _output_get (Variables|Default|SetSaveGameInstance _returnvalue_2))
    (bind _returnvalue_3 (SaveGame|SaveGametoSlot _output_get (Variables|/Game/2DPlatformingKit/Blueprints/Main/SaveGamePlayer.SaveGamePlayer_C|GetSlotName _output_get) (Variables|/Game/2DPlatformingKit/Blueprints/Main/SaveGamePlayer.SaveGamePlayer_C|GetUserIndex _output_get)))
    (if _returnvalue_3
      (Development|PrintString "Saved Info")
      (else
        (Development|PrintString "Something went wrong...")))
    (Utilities|FlowControl|Delay 1.0)
    (Rendering|SetVisibility (Variables|Components|GetTextRender) false false)))

(event EventBeginPlay
  ;[1 1 1] Disable collision Initially to avoid any weird issues
  (Collision|SetCollisionEnabled (Variables|Components|GetBox) "NoCollision")
  (Utilities|FlowControl|Delay 1.0)
  (Collision|SetCollisionEnabled (Variables|Components|GetBox) "QueryAndPhysics"))

(event Collision|EventActorBeginOverlap
  (params (OtherActor :type Actor%20Object%20Reference)))

(event EventTick
  (params (DeltaSeconds :type Float%20%28single-precision%29)))

(fn ConstructionScript)