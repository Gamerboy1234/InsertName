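; Wall actor for a 2D platformer that puts the player character into a wall-jump state on contact.
; On BeginPlay it copies its WallJumpVelocity onto player 0's Player_Character, so the value is set globally rather than on each contact.
; Trigger overlap sets IsWalljumping and StillOnWall and updates the animation state, while leaving clears only StillOnWall.
; The construction script applies the configurable ActorsSprite.
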(event OnComponentBeginOverlap(Trigger)
  (params (OverlappedComponent :type Primitive%20Component%20Object%20Reference) (OtherActor :type Actor%20Object%20Reference) (OtherComp :type Primitive%20Component%20Object%20Reference) (OtherBodyIndex :type Integer) (bFromSweep :type Boolean) (SweepResult :type Hit%20Result%20Structure%20%28by%20ref%29))
  (bind _asplayer_character (Utilities|Casting|CastToPlayer_Character OtherActor))
  (Variables|/Game/2DPlatformingKit/Blueprints/Player/Player_Character.Player_Character_C|SetIs%20Walljumping? _asplayer_character true)
  (Variables|/Game/2DPlatformingKit/Blueprints/Player/Player_Character.Player_Character_C|SetplayerAnimState _asplayer_character "NewEnumerator34")
  (Default|UpdateAnimation _asplayer_character)
  (Variables|/Game/2DPlatformingKit/Blueprints/Player/Player_Character.Player_Character_C|SetStill%20on%20Wall? _asplayer_character true))

(event OnComponentEndOverlap(Trigger)
  (params (OverlappedComponent :type Primitive%20Component%20Object%20Reference) (OtherActor :type Actor%20Object%20Reference) (OtherComp :type Primitive%20Component%20Object%20Reference) (OtherBodyIndex :type Integer))
  (bind _asplayer_character (Utilities|Casting|CastToPlayer_Character OtherActor))
  (Variables|/Game/2DPlatformingKit/Blueprints/Player/Player_Character.Player_Character_C|SetStill%20on%20Wall? _asplayer_character false))

(event EventBeginPlay
  (bind _asplayer_character (Utilities|Casting|CastToPlayer_Character (Game|GetPlayerCharacter 0)))
  (bind _output_get (Variables|Default|SetPlayer%20Rerf _asplayer_character))
  (Variables|/Game/2DPlatformingKit/Blueprints/Player/Player_Character.Player_Character_C|SetwallJumpVelocity _output_get (Variables|Default|GetWall%20Jump%20Velocity)))

(fn ConstructionScript
  (Rendering|Components|Sprite|SetSprite (Variables|Default|Getsprite) (Variables|Default|GetActor's%20Sprite)))