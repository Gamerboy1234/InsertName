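; Moveable platform Blueprint for a 2D platforming kit that travels between a start and an end location.
; The construction script builds two relative InterpToMovement control points from those locations and uses Speed as the movement duration.
; With StartWithPlate set, movement stops at BeginPlay, and the StartMovement event restarts it when called.
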(event EventBeginPlay
  (if (Variables|Default|GetbStartWithPlate)
    (Components|Movement|StopMovementImmediately (Variables|Default|GetInterpToMovement))))

(event EventStartMovement
  (Class|InterptoMovementComponent|RestartMovement (Variables|Default|GetInterpToMovement) 1.0))

(fn ConstructionScript
  (bind _interptomovement (Variables|Default|GetInterpToMovement))
  (Variables|/Script/Engine.InterpToMovementComponent|SetControlPoints _interptomovement (Utilities|Array|MakeArray (Utilities|Struct|MakeInterpControlPoint (Variables|PlatformSettings|GetStart%20Location) true) (Utilities|Struct|MakeInterpControlPoint (Variables|PlatformSettings|GetEnd%20Location) true)))
  (Variables|/Script/Engine.InterpToMovementComponent|SetDuration _interptomovement (Variables|PlatformSettings|GetSpeed)))