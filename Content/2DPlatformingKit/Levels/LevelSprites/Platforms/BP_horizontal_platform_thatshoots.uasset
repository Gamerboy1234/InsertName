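; Blueprint for a moving 2D platform, named as a horizontal shooting platform, that animates its position around where it was placed.
; On BeginPlay it stores its location and waits a configurable Startplatform delay before setting a Start flag.
; Tick then plays a timeline whose vector track is added to the stored location to move the actor without sweep.
; The graph contains no shooting logic.
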(event EventTick
  (params (DeltaSeconds :type Float%20%28single-precision%29))
  (if (Variables|Default|Getstart)
    (Utilities|FlowControl|Sequence
      (:then_0
        (bind _newtrack_3 (Timeline|Timeline_0 Play)
          (:Update
            (Transformation|SetActorLocation (+ _newtrack_3 (Variables|Default|Getlocationofplatform)) false false)))))))

(event EventBeginPlay
  ;[1 1 1] Comment
  (Variables|Default|Setlocationofplatform (Transformation|GetActorLocation))
  (Utilities|FlowControl|Delay (Variables|Default|GetStartplatform))
  (Variables|Default|Setstart true))

(fn ConstructionScript)