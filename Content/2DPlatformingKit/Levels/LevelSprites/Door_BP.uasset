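; Door actor for a 2D platformer that carries the player through with a scripted camera pan when they overlap its collision.
; The player's DirectionInt picks a left or right timeline, which adds vector offsets to the player's location.
; Meanwhile input is disabled as MoveComponentTo eases the CameraBoom to CameraMoveLocation and back, pausing briefly between moves only when heading right.
; The construction script positions the collision from a transform variable.
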(event OnComponentBeginOverlap(ActorCollsion)
  (params (OverlappedComponent :type Primitive%20Component%20Object%20Reference) (OtherActor :type Actor%20Object%20Reference) (OtherComp :type Primitive%20Component%20Object%20Reference) (OtherBodyIndex :type Integer) (bFromSweep :type Boolean) (SweepResult :type Hit%20Result%20Structure%20%28by%20ref%29))
  (bind _asplayer_character (Utilities|Casting|CastToPlayer_Character OtherActor))
  (Variables|Default|SetPlayer%20Ref _asplayer_character)
  (|MoveCameraandPlayer))

(fn ConstructionScript
  (Transformation|SetRelativeTransform (Variables|Default|GetActor%20Collsion) (Variables|Location|GetActor%20Collsion%20Transform) false false)
  (Variables|Location|SetCamera%20Move%20Location (Variables|Location|GetCamera%20Move%20Location)))